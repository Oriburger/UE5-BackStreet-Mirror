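; Main character Blueprint, back-view variant by its name, whose own graphs hold only debug and test helpers.
; Two print functions show debuffs, action state, stats, HP and inventory counts on screen; the ammo readout is disabled and hardcoded to zero.
; Tick and the misspelled AttakRushTest event are empty, leaving the debug prints and the rush impulse test disconnected.
; The construction script is empty.
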(event `self.ReceiveTick`
  (params (DeltaSeconds :type "Float (single-precision)"))
  ;[0.9571 0 1 1 50] Tick / Debug
)

(event `AttakRushTest`
  (params (Direction :type "Vector Structure"))
  ;[0.9571 0 1 1 50] Tick / Debug
)

(fn `Print Inventory Info`
  (bind _returnvalue (`self.GetInventoryRef`))
  (`/Engine/EditorBlueprintResources/StandardMacros.IsValid` _returnvalue
    (:`Is Valid`
      (`KismetSystemLibrary.PrintString` (`KismetStringLibrary.Concat_StrStr` "Inventory Idx : " (`KismetStringLibrary.Conv_IntToString` (`WeaponInventoryBase.GetCurrentIdx` _returnvalue)) "   /   " "Weapon Count  :  " (`KismetStringLibrary.Conv_IntToString` (`WeaponInventoryBase.GetCurrentWeaponCount` _returnvalue)) "  /  Capacity" (`KismetStringLibrary.Conv_IntToString` (`WeaponInventoryBase.GetCurrentCapacity` _returnvalue))) true false (struct :`G` 0.66 :`B` 1.0 :`A` 1.0) 0.01))))

(fn `PrintCharacterInfo`
  (locals (Temp :type String))
  (bind _returnvalue (`self.GetWeaponActorRef`))
  (bind (_characterdebuffstate _bcanattack _turndirection _characteractionstate _charactercurrhp) (break `CharacterStateStruct` (`self.CharacterState`)))
  (bind (_characterid _bisinvincibility _binfinite _charactermaxhp _characteratkmultiplier _characteratkspeed _charactermovespeed _characterdefense) (break `CharacterStatStruct` (`self.CharacterStat`)))
  (`|ExecutionSequence`
    (:`then_0`
      (for _index (range 9)
        (bind _returnvalue_2 (cast `ECharacterDebuffType` (`KismetMathLibrary.Conv_IntToByte` _index)))
        (set `local.Temp` (`KismetStringLibrary.Concat_StrStr` (`local.Temp`) (`KismetStringLibrary.Concat_StrStr` (`|GetEnumeratorNameAsString` _returnvalue_2) " : " (`KismetStringLibrary.Conv_BoolToString` (`self.GetDebuffIsActive` _returnvalue_2)) " / "))))
      (`KismetSystemLibrary.PrintString` (`local.Temp`) true false (struct :`R` 0.480775 :`G` 1.0 :`B` 0.463542 :`A` 1.0) 0.003)
      (set `local.Temp` ""))
    (:`then_2`
      (`KismetSystemLibrary.PrintString` (`KismetStringLibrary.Concat_StrStr` "ActionState :  " (`|GetEnumeratorNameAsString` _characteractionstate) "  /  Can Atk : " (`KismetStringLibrary.Conv_BoolToString` _bcanattack)) true false (struct :`R` 1.0 :`G` 0.955652 :`A` 1.0) 0.003))
    (:`then_3`
      (`KismetSystemLibrary.PrintString` (`KismetStringLibrary.Concat_StrStr` "Speed : " (`KismetStringLibrary.Conv_DoubleToString` (`CharacterMovementComponent.MaxWalkSpeed` (`self.CharacterMovement`))) ", " (`KismetStringLibrary.Conv_DoubleToString` _charactermovespeed) "  /  Atk Speed : " (`KismetStringLibrary.Conv_DoubleToString` _characteratkspeed)) true false (struct :`G` 0.900125 :`B` 1.0 :`A` 1.0) 0.003))
    (:`then_4`
      (`KismetSystemLibrary.PrintString` (`KismetStringLibrary.Concat_StrStr` "DEF : " (`KismetStringLibrary.Conv_DoubleToString` _characterdefense) "/ ATK : " (`KismetStringLibrary.Conv_DoubleToString` _characteratkmultiplier)) true false (struct :`G` 0.363636 :`B` 1.0 :`A` 1.0) 0.003))
    (:`then_5`
      (`KismetSystemLibrary.PrintString` (`KismetStringLibrary.Concat_StrStr` "HP : " (`KismetStringLibrary.Conv_DoubleToString` _charactercurrhp) "/" (`KismetStringLibrary.Conv_DoubleToString` _charactermaxhp)) true false (struct :`R` 1.0 :`G` 0.227609 :`B` 0.223958 :`A` 1.0) 0.003))
    (:`then_6`
      (`/Engine/EditorBlueprintResources/StandardMacros.IsValid` _returnvalue
        (:`Is Valid`
          (if (and (`KismetSystemLibrary.IsValid` _returnvalue) false)
            (`KismetSystemLibrary.PrintString` (`KismetStringLibrary.Concat_StrStr` "Ammo : " (`KismetStringLibrary.Conv_IntToString` 0) "/" (`KismetStringLibrary.Conv_IntToString` 0)) true false (struct :`R` 1.0 :`G` 0.6475 :`B` 0.645833 :`A` 1.0) 0.003)))))))

(fn `UserConstructionScript`)