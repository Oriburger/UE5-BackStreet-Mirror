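; Player main character Blueprint, layering debug tools and test input over inherited combat, inventory and skill functions.
; Construction initializes assets from the character ID, and Tick prints character, weapon, inventory and current target info on screen.
; Up and Down keys step clamped global time dilation, right mouse release calls TrySkill with no type, and middle mouse fires a temporary IndieGo bottle-bat skill.
; Gauge-fill and cursor-rotation calls sit unwired.
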(event EventTick
  (params (DeltaSeconds :type Float%20%28single-precision%29))
  ;[0.9571 0 1 1 50] Tick / Debug
  (CallFunction|PrintCharacterInfo)
  (CallFunction|PrintInventoryInfo (Class|CharacterBase|GetWeaponInventoryRef))
  (Development|PrintString (Utilities|GetDisplayName (Class|TargetingManagerComponent|GetTargetedCharacter (Variables|Default|GetTargetingManagerComponent))) true false "(R=1.000000,G=0.863371,B=0.171760,A=1.000000)" (+ (Utilities|Time|GetWorldDeltaSeconds) 0.01)))

(event Input|KeyboardEvents|DebugKeyG
  (params (Key :type Key%20Structure :default "None") (ActionValue :type Input%20Action%20Value%20Structure))
  ;[0.9571 0 1 1 50] Tick / Debug
)

(event Input|MouseEvents|RightMouseButton
  (params (Key :type Key%20Structure :default "None"))
  ;[1 1 1 1 50] BP_ImplementableEvent
  (:Released
    (Class|MainCharacterBase|TrySkill "E_None")))

(event Input|MouseEvents|LeftMouseButton
  (params (Key :type Key%20Structure :default "None"))
  ;[1 1 1] IndieGo용 임시 코드(유리병 방망이 스킬)
)

(event Input|KeyboardEvents|Down
  (params (Key :type Key%20Structure :default "None"))
  (:Pressed
    (Variables|Default|SetTime%20Dilation (+ (Variables|Default|GetTime%20Dilation) -0.2))
    (Variables|Default|SetTime%20Dilation (Math|Float|Clamp(Float) (Variables|Default|GetTime%20Dilation)))
    (Utilities|Time|SetGlobalTimeDilation (Variables|Default|GetTime%20Dilation))))

(event Input|KeyboardEvents|Up
  (params (Key :type Key%20Structure :default "None"))
  (:Pressed
    (Variables|Default|SetTime%20Dilation (+ (Variables|Default|GetTime%20Dilation) 0.2))
    (Variables|Default|SetTime%20Dilation (Math|Float|Clamp(Float) (Variables|Default|GetTime%20Dilation)))
    (Utilities|Time|SetGlobalTimeDilation (Variables|Default|GetTime%20Dilation))))

(event Input|MouseEvents|MiddleMouseButton
  (params (Key :type Key%20Structure :default "None"))
  (:Pressed
    (Class|MainCharacterBase|TrySkill "E_Character" 5001)))

(fn ConstructionScript
  (Class|MainCharacterBase|InitAsset (.CharacterID (Utilities|Struct|BreakCharacterStatStruct (Variables|Default|GetCharacterStat)))))

(fn PrintCharacterInfo
  (bind _returnvalue (Class|CharacterBase|GetCharacterState))
  (bind _returnvalue_2 (Class|CharacterBase|GetCharacterState))
  (bind _returnvalue_3 (Class|CharacterBase|GetCurrentWeaponRef))
  (bind _returnvalue_4 (Utilities|Time|GetWorldDeltaSeconds))
  (bind (_characterdebuffstate _bcanattack _bissprinting _characteractionstate) (Utilities|Struct|BreakCharacterStateStruct _returnvalue))
  (bind (_bissprinting_2 _totalhp _totalattack _totaldefense _totalmovespeed _totalattackspeed _currenthp) (Utilities|Struct|BreakCharacterStateStruct _returnvalue_2))
  (bind _returnvalue_5 (Class|WeaponBase|GetWeaponStat _returnvalue_3))
  (bind (_weaponid _weaponname _description _weapontype _weaponimage _weaponatkspeedrate _weapondamage _bcriticalapply _criticaldamagerate _bfixdamageapply _fixeddamageamount _binfinite _bhasfinalimpact _maxdurability _weaponweight) (Utilities|Struct|BreakWeaponStatStruct _returnvalue_5))
  (Utilities|FlowControl|Sequence
    (:then_0
      (Development|PrintString (Utilities|String|Append "CharacterID : " (Utilities|String|ToString(Integer) (Utilities|Struct|BreakCharacterStatStruct (Class|CharacterBase|GetCharacterStat))) " / CharacterHP : " (Utilities|String|Append "(" (Utilities|String|ToString(Float) _totalhp) " / " (Utilities|String|ToString(Float) _currenthp) ")") " / Atk Multiplier : " (Utilities|String|ToString(Float) _totalattack) " / Atk Speed : " (Utilities|String|ToString(Float) _totalattackspeed) " / Move Speed : " (Utilities|String|ToString(Float) _totalmovespeed) " / Defense : " (Utilities|String|ToString(Float) _totaldefense)) true false "(R=1.000000,G=0.757566,B=0.086535,A=1.000000)" _returnvalue_4))
    (:then_1
      (Development|PrintString (Utilities|String|Append "Debuff State : " (Utilities|String|ToString(Integer) (- _characterdebuffstate 1024)) " / Can Attack : " (Utilities|String|ToString(Boolean) _bcanattack) " / Action State : " (Utilities|String|EnumtoString _characteractionstate)) true false "(R=1.000000,G=0.351057,B=0.000000,A=1.000000)" _returnvalue_4))
    (:then_2
      (Utilities|IsValid _returnvalue_3
        (:Is%20Valid
          (Development|PrintString (Utilities|String|Append "WeaponName : " (Utilities|String|ToString(Name) _weaponname) " / WeaponType : " (Utilities|String|EnumtoString _weapontype) " / WeaponWeight : " (Utilities|String|ToString(Byte) _weaponweight) " / Atk Speed Rate : " (Utilities|String|ToString(Float) _weaponatkspeedrate) " / Damage : " (Utilities|String|ToString(Float) _weapondamage) "/ Combo Count : " (Utilities|String|ToString(Integer) (.ComboCount (Utilities|Struct|BreakWeaponStateStruct (Class|WeaponBase|GetWeaponState _returnvalue_3))))) true false "(R=0.771003,G=0.000000,B=1.000000,A=1.000000)" _returnvalue_4)
          (if (not (Actor|ActorHasTag _returnvalue_3 "Ranged"))
            (if (Actor|ActorHasTag _returnvalue_3 "Ranged")
              _)))))))

(fn PrintInventoryInfo
  (params (InputPin :type Weapon%20Inventory%20Base%20Object%20Reference))
  (Utilities|IsValid InputPin
    (:Is%20Valid
      (Development|PrintString (Utilities|String|Append "Inventory Idx : " (Utilities|String|ToString(Integer) (Class|WeaponInventoryBase|GetCurrentIdx InputPin)) "   /   " "Weapon Count  :  " (Utilities|String|ToString(Integer) (Class|WeaponInventoryBase|GetCurrentWeaponCount InputPin)) "  /  Capacity" (Utilities|String|ToString(Integer) (Class|WeaponInventoryBase|GetCurrentCapacity InputPin))) true false "(R=0.000000,G=0.660000,B=1.000000,A=1.000000)" 0.01))))

(fn GetMouseCursorLocation
  (bind _asmain_character_controller (Utilities|Casting|CastToMainCharacterController (Game|GetPlayerController 0))
    (:then
      (return (Class|MainCharacterController|GetCursorDeprojectionWorldLocation _asmain_character_controller)))
    (:CastFailed
      (return "0, 0, 0"))))

(fn SetCharacterSkillGaugeFull
  (Utilities|Struct|SetmembersinCharacterStateStruct (Variables|Default|GetCharacterState) 1e+01))