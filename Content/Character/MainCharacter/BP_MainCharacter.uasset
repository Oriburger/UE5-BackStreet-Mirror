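; Main player character Blueprint that handles skill input and on-screen debug readouts.
; Construction calls InitAsset with the CharacterID to set up the character.
; Three hardcoded skill inputs map the weapon's skill type slots through SkillManagerComponent's equipped map into TrySkill.
; Tick prints character stat types each frame; weapon, skill and inventory printers, plus cheats for healing and stage moves, are left disconnected.
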(event `self.ReceiveTick`
  (params (DeltaSeconds :type "Float (single-precision)"))
  ;[0.9571 0 1 1 50] Tick / Debug
  (`self.PrintCharacterInfo`))

(event `EnhancedInput|/Game/Character/MainCharacter/Input/Action/IA_Skill0`
  (params (ActionValue :type Boolean) (ElapsedSeconds :type "Float (double-precision)") (TriggeredSeconds :type "Float (double-precision)") (InputAction :type "InputAction Object Reference" :default "/Game/Character/MainCharacter/Input/Action/IA_Skill0.IA_Skill0"))
  (bind _weaponcomponent (`self.WeaponComponent`))
  (bind _value (`BlueprintMapLibrary.Map_Find` (`PlayerSkillManagerComponent.GetEquipedSkillMap` (`self.SkillManagerComponent`)) (`|GetArrayItem` (`.SkillTypeList` (break `WeaponStatStruct` (`WeaponComponentBase.GetWeaponStat` _weaponcomponent))))))
  ;[1 1 1 1 34] 스킬 키바인딩 (하드코딩 BIC이후 수정 예정)
  (:`Triggered`
    (`/Engine/EditorBlueprintResources/StandardMacros.IsValid` _weaponcomponent
      (:`Is Valid`
        (if (!= _value 0)
          (`self.TrySkill` _value))))))

(event `EnhancedInput|/Game/Character/MainCharacter/Input/Action/IA_Skill1`
  (params (ActionValue :type Boolean) (ElapsedSeconds :type "Float (double-precision)") (TriggeredSeconds :type "Float (double-precision)") (InputAction :type "InputAction Object Reference" :default "/Game/Character/MainCharacter/Input/Action/IA_Skill1.IA_Skill1"))
  (bind _weaponcomponent (`self.WeaponComponent`))
  (bind _value (`BlueprintMapLibrary.Map_Find` (`PlayerSkillManagerComponent.GetEquipedSkillMap` (`self.SkillManagerComponent`)) (`|GetArrayItem` (`.SkillTypeList` (break `WeaponStatStruct` (`WeaponComponentBase.GetWeaponStat` _weaponcomponent))) 1)))
  ;[1 1 1 1 34] 스킬 키바인딩 (하드코딩 BIC이후 수정 예정)
  (:`Triggered`
    (`/Engine/EditorBlueprintResources/StandardMacros.IsValid` _weaponcomponent
      (:`Is Valid`
        (if (!= _value 0)
          (`self.TrySkill` _value))))))

(event `Key|J`
  (params (Key :type "Key Structure"))
  ;[1 0.4045 0.3047 1 50] Work In Progress
  ;;[1 1 1] Cheat
)

(event `EnhancedInput|/Game/Character/MainCharacter/Input/Action/IA_Skill2`
  (params (ActionValue :type Boolean) (ElapsedSeconds :type "Float (double-precision)") (TriggeredSeconds :type "Float (double-precision)") (InputAction :type "InputAction Object Reference" :default "/Game/Character/MainCharacter/Input/Action/IA_Skill2.IA_Skill2"))
  (bind _weaponcomponent (`self.WeaponComponent`))
  (bind _value (`BlueprintMapLibrary.Map_Find` (`PlayerSkillManagerComponent.GetEquipedSkillMap` (`self.SkillManagerComponent`)) (`|GetArrayItem` (`.SkillTypeList` (break `WeaponStatStruct` (`WeaponComponentBase.GetWeaponStat` _weaponcomponent))) 2)))
  ;[1 1 1 1 34] 스킬 키바인딩 (하드코딩 BIC이후 수정 예정)
  (:`Triggered`
    (`/Engine/EditorBlueprintResources/StandardMacros.IsValid` _weaponcomponent
      (:`Is Valid`
        (if (!= _value 0)
          (`self.TrySkill` _value))))))

(event `Key|H`
  (params (Key :type "Key Structure"))
  ;[1 0.4045 0.3047 1 50] Work In Progress
  ;;[1 1 1] Cheat
)

(event `Key|P`
  (params (Key :type "Key Structure"))
  ;[0.9217 0.3325 1] Debug(Move to Chpater1 BossStage)
)

(fn `PrintCharacterInfo`
  (locals (Temp :type String))
  (bind (_characterid _binfinite _bisinvincibility _statgrouplist) (break `CharacterGameplayInfo` (`self.CharacterGameplayInfo`)))
  (for (_ _array_index) _statgrouplist
    (bind _returnvalue (- (`KismetArrayLibrary.Array_Length` _statgrouplist) 1 _array_index))
    (bind (_defaultvalue _biscontainprobability _probabilityvalue) (break `StatValueGroup` (`|GetArrayItem` _statgrouplist _returnvalue)))
    (`KismetSystemLibrary.PrintString` (`KismetStringLibrary.Concat_StrStr` (`|GetEnumeratorNameAsString` (cast `ECharacterStatType` (`KismetMathLibrary.Conv_IntToByte` _returnvalue))) "" (`KismetMathLibrary.SelectString` (`KismetStringLibrary.Concat_StrStr` " / Probability : " (`KismetStringLibrary.Conv_DoubleToString` _probabilityvalue)) "" _biscontainprobability)) true false (struct :`G` 0.66 :`B` 1.0 :`A` 1.0) (`GameplayStatics.GetWorldDeltaSeconds`)))
  (`KismetSystemLibrary.PrintString` "[--- Character Stat Info ---] \n" true false (struct :`G` 0.66 :`B` 1.0 :`A` 1.0) (`GameplayStatics.GetWorldDeltaSeconds`)))

(fn `PrintInventoryInfo`
  (locals (Arr_TypeList :type "Array of ECraftingItemType Enum"))
  (bind _iteminventory (`self.ItemInventory`))
  (for _array_element (`local.Arr_TypeList`)
    (`KismetSystemLibrary.PrintString` (`KismetStringLibrary.Concat_StrStr` "[" (`KismetStringLibrary.Conv_NameToString` (`.ItemName` (break `ItemInfoDataStruct` (`ItemInventoryComponent.GetItemData` _iteminventory (`ItemInventoryComponent.ConvertCraftingItemTypeToItemID` _iteminventory _array_element))))) "]" ":" (`KismetStringLibrary.Conv_ByteToString` (`BlueprintMapLibrary.Map_Find` (`ItemInventoryComponent.GetAllCraftingItemAmount` _iteminventory) _array_element))) true false (struct :`R` 1.0 :`G` 0.757566 :`B` 0.086535 :`A` 1.0) (`GameplayStatics.GetWorldDeltaSeconds`))))

(fn `PrintSkillInfo`
  (bind _weaponcomponent (`self.WeaponComponent`))
  (bind _skillmanagercomponent (`self.SkillManagerComponent`))
  (if (!= (`WeaponComponentBase.WeaponID` _weaponcomponent) 0)
    (for _array_element (`.SkillTypeList` (break `WeaponStatStruct` (`WeaponComponentBase.GetWeaponStat` _weaponcomponent)))
      (bind _value (`BlueprintMapLibrary.Map_Find` (`PlayerSkillManagerComponent.GetEquipedSkillMap` _skillmanagercomponent) _array_element))
      (if (!= _value 0)
        (`KismetSystemLibrary.PrintString` (`KismetStringLibrary.Concat_StrStr` "[" (`KismetStringLibrary.Conv_NameToString` (`.SkillName` (break `SkillStatStruct` (`SkillManagerComponentBase.GetOwnSkillStat` _skillmanagercomponent _value)))) "]" ":" (`KismetStringLibrary.Conv_ByteToString` 0)) true false (struct :`R` 1.0 :`G` 0.757566 :`B` 0.086535 :`A` 1.0))))))

(fn `PrintWeaponInfo`
  (bind _returnvalue (`GameplayStatics.GetWorldDeltaSeconds`))
  (bind _weaponcomponent (`self.WeaponComponent`))
  (bind ((`WeaponName` _weaponname) (`WeaponType` _weapontype)) (break `WeaponStatStruct` (`WeaponComponentBase.GetWeaponStat` _weaponcomponent)))
  (bind ((`RangedWeaponState` _rangedweaponstate) (`UpgradedStatMap` _upgradedstatmap)) (break `WeaponStateStruct` (`WeaponComponentBase.GetWeaponState` _weaponcomponent)))
  (`|ExecutionSequence`
    (:`then_0`
      (`KismetSystemLibrary.PrintString` (`KismetStringLibrary.Concat_StrStr` "무기 이름 :  " (`KismetStringLibrary.Conv_NameToString` _weaponname) "/ 종류 : " (`|GetEnumeratorNameAsString` _weapontype) (`KismetMathLibrary.SelectString` (`KismetStringLibrary.Concat_StrStr` " /  탄환 수 : " "(" (`KismetStringLibrary.Conv_IntToString` (`.CurrentAmmoCount` (break `RangedWeaponStateStruct` _rangedweaponstate))) ")") "" (`|EnumEquality` _weapontype "E_Shoot"))) true false (struct :`G` 0.66 :`B` 1.0 :`A` 1.0) _returnvalue))
    (:`then_1`
      (`KismetSystemLibrary.PrintString` (`KismetStringLibrary.Concat_StrStr` "공격력 :  " (`KismetStringLibrary.Conv_ByteToString` (`BlueprintMapLibrary.Map_Find` _upgradedstatmap "E_Attack")) "/ 공격 속도 : " (`KismetStringLibrary.Conv_ByteToString` (`BlueprintMapLibrary.Map_Find` _upgradedstatmap "E_AttackSpeed")) "/ 파이널 임팩트 : " (`KismetStringLibrary.Conv_ByteToString` (`BlueprintMapLibrary.Map_Find` _upgradedstatmap "E_FinalAttack"))) true false (struct :`G` 0.66 :`B` 1.0 :`A` 1.0) _returnvalue))))

(fn `UserConstructionScript`
  (`self.InitAsset` (`.CharacterID` (break `CharacterGameplayInfo` (`self.CharacterGameplayInfo`)))))