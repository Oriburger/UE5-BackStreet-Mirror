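; BP_EnemyCharacter_TypeA_Melee_Test is a test Blueprint for a melee Type A enemy character with a floating HP bar.
; Its InitFloatingHpWidget event casts the floating bar's widget to WB_EnemyHPBar and passes the enemy as its owner reference.
; The AnyDamage event and GetAttackRange are empty, and a delayed debug print of damage and current HP is left disconnected.
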(event `self.ReceiveAnyDamage`
  (params (Damage :type "Float (single-precision)") (DamageType :type "DamageType Object Reference") (InstigatedBy :type "Controller Object Reference") (DamageCauser :type "Actor Object Reference"))
  ;[1 1 1] Debug
)

(event `self.InitFloatingHpWidget`
  (bind _returnvalue (`WidgetComponent.GetWidget` (`self.FloatingHpBar`)))
  ;[1 1 1] BP_ImplementableEvent
  (`/Engine/EditorBlueprintResources/StandardMacros.IsValid` _returnvalue
    (:`Is Valid`
      (bind _aswb_enemy_hpbar (cast `/Game/UI/InGame/Blueprint/WB_EnemyHPBar` _returnvalue))
      (`/Game/UI/InGame/Blueprint/WB_EnemyHPBar.SetOwnerRef` _aswb_enemy_hpbar self))))

(fn `GetAttackRange`)

(fn `UserConstructionScript`)