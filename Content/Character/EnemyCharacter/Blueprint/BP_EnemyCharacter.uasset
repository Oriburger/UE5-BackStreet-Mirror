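; Enemy character Blueprint that sets up its assets and stats from a character ID in the construction script and handles the enemy's on-screen widgets and visual effects.
; Targeting events toggle the targeting-support widget using the player's targeting manager state.
; A floating health bar gets an ID-based height and is shown when a debuff is added.
; BeginPlay plays an appear Niagara effect with timeline-driven scaling, and a Hologram event animates a material parameter collection.
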(event `self.InitTargetingSupportingWidget`
  (bind _returnvalue (`GameplayStatics.GetPlayerCharacter` 0))
  (bind _returnvalue_2 (`WidgetComponent.GetWidget` (`self.TargetingSupportWidget`)))
  ;[1 1 1] 타게팅 UI
  (`KismetSystemLibrary.Delay` 0.4)
  (`/Engine/EditorBlueprintResources/StandardMacros.IsValid` _returnvalue
    (:`Is Valid`
      (bind _asbp_main_character (cast `/Game/Character/MainCharacter/BP_MainCharacter` _returnvalue))
      (`/Engine/EditorBlueprintResources/StandardMacros.IsValid` _returnvalue_2
        (:`Is Valid`
          (bind _aswb_targeting_support (cast `/Game/Character/EnemyCharacter/Blueprint/Widget/WB_TargetingSupport` _returnvalue_2))
          (set `self.TargetingSupportWidgetRef` _aswb_targeting_support))))))

(event `self.ReceiveBeginPlay`
  (`self.SpawnEffect`))

(event `self.OnTargetUpdated`
  (params (Target :type "Pawn Object Reference"))
  (bind _targetingsupportwidgetref (`self.TargetingSupportWidgetRef`))
  (bind _returnvalue (== Target self))
  ;[1 1 1] 타게팅 UI
  (bind _targetingmanagercomponent (`CharacterBase.TargetingManagerComponent` (stale `self.InitTargetingSupportingWidget` _asbp_main_character)))
  (if (not (`TargetingManagerComponent.GetIsTargetingActivated` _targetingmanagercomponent))
    (`/Game/Character/EnemyCharacter/Blueprint/Widget/WB_TargetingSupport.SwitchMode` _targetingsupportwidgetref _returnvalue false)
    (else
      (bind _returnvalue_2 (== (`TargetingManagerComponent.GetTargetedCharacter` _targetingmanagercomponent) self))
      (`/Game/Character/EnemyCharacter/Blueprint/Widget/WB_TargetingSupport.SwitchMode` _targetingsupportwidgetref (or _returnvalue _returnvalue_2) _returnvalue_2))))

(event `self.OnTargetingActivated`
  (params (bIsActivated :type Boolean) (Target :type "Pawn Object Reference"))
  ;[1 1 1] 타게팅 UI
  (`/Game/Character/EnemyCharacter/Blueprint/Widget/WB_TargetingSupport.SwitchMode` (`self.TargetingSupportWidgetRef`) (== Target self) bIsActivated))

(event `self.InitFloatingHpWidget`
  (bind _floatinghpbar (`self.FloatingHpBar`))
  (bind _returnvalue (`WidgetComponent.GetWidget` (`self.FloatingHpBar`)))
  (bind _returnvalue_2 (== (`self.CharacterID`) 1200))
  (bind _returnvalue_3 (`KismetMathLibrary.SelectFloat` 200.0 85.0 _returnvalue_2))
  ;[1 1 1] BP_ImplementableEvent
  (`/Engine/EditorBlueprintResources/StandardMacros.IsValid` _returnvalue
    (:`Is Valid`
      (bind _aswb_enemy_floating_healthbar (cast `/Game/Character/EnemyCharacter/Blueprint/Widget/WB_EnemyFloatingHealthbar` _returnvalue))
      (`/Game/Character/EnemyCharacter/Blueprint/Widget/WB_EnemyFloatingHealthbar.SetOwnerManually` _aswb_enemy_floating_healthbar self)
      (if _returnvalue_2
        (`SceneComponent.K2_SetRelativeLocation` _floatinghpbar (`KismetMathLibrary.MakeVector` 0.0 0.0 _returnvalue_3) false true)
        (else
          (`SceneComponent.K2_SetRelativeLocation` _floatinghpbar (`KismetMathLibrary.MakeVector` 0.0 0.0 _returnvalue_3) false true))))))

(event `SpawnEffect`
  ;[1 1 1] BP_ImplementableEvent
  (`NiagaraFunctionLibrary.SpawnSystemAttached` "/Game/Character/Particle/NS_Appear.NS_Appear" (`self.Mesh`) "root" (0.0 0.0 -80.0) (struct) "KeepRelativeOffset" true)
  (bind (_direction `_새_트랙_0`) (`Timeline|타임라인`)
    (:`Update`
      (`self.K2_SetActorTransform` (`KismetMathLibrary.MakeTransform` (`self.K2_GetActorLocation`) (`self.K2_GetActorRotation`) (`KismetMathLibrary.Conv_DoubleToVector` `_새_트랙_0`))))))

(event `self.ReceiveTick`
  (params (DeltaSeconds :type "Float (single-precision)"))
  ;[1 1 1] Debug
)

(event `self.DebuffManagerComponent.OnDebuffAdded`
  (params (DebuffType :type "ECharacterDebuffType Enum" :default "E_None"))
  (if (`|EnumInequality` DebuffType "E_None")
    (`SceneComponent.SetVisibility` (`self.FloatingHpBar`) true false)))

(event `Hologram`
  (bind (_direction _newtrack_0) (`Timeline|Hologram_Timeline` :!via `PlayFromStart`)
    (:`Update`
      (`KismetMaterialLibrary.SetScalarParameterValue` "/Game/VFX/Material/Material_Function/MPC_Hologram.MPC_Hologram" "Progress" _newtrack_0))
    (:`Finished`
      (`KismetMaterialLibrary.SetScalarParameterValue` "/Game/VFX/Material/Material_Function/MPC_Hologram.MPC_Hologram" "Progress" 1.0))))

(fn `UserConstructionScript`
  (bind _characterid (break `CharacterAssetSoftInfo` (`self.AssetSoftPtrInfo`)))
  (`self.InitAsset` _characterid)
  (`self.InitEnemyCharacter` _characterid))