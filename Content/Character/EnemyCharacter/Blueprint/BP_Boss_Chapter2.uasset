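; Enemy character Blueprint for the Chapter 2 boss, which tracks trash objects from the level as its weapons.
; On BeginPlay it initializes every BP_TrashSpawnPoint with itself as owner and an index, then collects each spawner's TrashRef into TrashWeaponArray.
; Add and remove functions maintain that array, with removal swapping the item to the end before deleting it.
; The construction script initializes asset and enemy data from a hard-coded ID.
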(event `self.InitFloatingHpWidget`
  (`parent.InitFloatingHpWidget`))

(event `self.ReceiveBeginPlay`
  (`parent.ReceiveBeginPlay`)
  (bind _outactors (`GameplayStatics.GetAllActorsOfClass` "/Game/System/SkillManager/Blueprint/Actor/BP_TrashSpawnPoint.BP_TrashSpawnPoint_C"))
  (bind _output_get (set `self.TrashSpawnerArray` _outactors))
  (for (_array_element _array_index) _output_get
    (`/Engine/EditorBlueprintResources/StandardMacros.IsValid` _array_element
      (:`Is Valid`
        (`/Game/System/SkillManager/Blueprint/Actor/BP_TrashSpawnPoint.Initialize` _array_element self _array_index))))
  (for _array_element_2 _output_get
    (`KismetArrayLibrary.Array_Add` (`self.TrashWeaponArray`) (`/Game/System/SkillManager/Blueprint/Actor/BP_TrashSpawnPoint.Trash Ref` _array_element_2))))

(fn `Add Trash Weapon`
  (params (NewItem :type "/Game/System/SkillManager/Blueprint/Actor/BP_TrashWeapon Object Reference (by ref)"))
  (`KismetArrayLibrary.Array_Add` (`self.TrashWeaponArray`) NewItem))

(fn `Remove Trash Weapon`
  (params (`Trash Ref` :type "/Game/System/SkillManager/Blueprint/Actor/BP_TrashWeapon Object Reference"))
  (bind _trashweaponarray (`self.TrashWeaponArray`))
  (bind _returnvalue (- (`KismetArrayLibrary.Array_Length` _trashweaponarray) 1))
  (`KismetArrayLibrary.Array_Swap` _trashweaponarray (`KismetArrayLibrary.Array_Find` _trashweaponarray `Trash Ref`) _returnvalue)
  (`KismetArrayLibrary.Array_Remove` _trashweaponarray _returnvalue))

(fn `UserConstructionScript`
  (`self.InitAsset` 2200)
  (`self.InitEnemyCharacter` 2200))