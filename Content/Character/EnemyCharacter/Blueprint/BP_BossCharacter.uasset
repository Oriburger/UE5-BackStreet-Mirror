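; BP_BossCharacter is the boss enemy character, set up in its construction script through InitAsset and InitEnemyCharacter with a shared ID.
; On BeginPlay it waits a tick, gathers every BP_Pillar in the level and initializes each valid one with itself as the boss reference.
; Initialize clears that pillar list and repeats the search and linking after a fixed delay.
; The floating HP widget setup defers to the parent.
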(event `self.ReceiveBeginPlay`
  (`parent.ReceiveBeginPlay`)
  (`KismetSystemLibrary.DelayUntilNextTick` :!label _label)
  (bind _outactors (`GameplayStatics.GetAllActorsOfClass` "/Game/System/SkillManager/Blueprint/Actor/BP_Pillar.BP_Pillar_C"))
  (bind _output_get (set `self.pillar Array` _outactors))
  (for _array_element _output_get
    (`/Engine/EditorBlueprintResources/StandardMacros.IsValid` _array_element
      (:`Is Valid`
        (`/Game/System/SkillManager/Blueprint/Actor/BP_Pillar.InitializePillar` _array_element self)))))

(event `Initialize`
  (`KismetArrayLibrary.Array_Clear` (`self.pillar Array`))
  (`KismetSystemLibrary.Delay` 6.0)
  (goto _label))

(event `self.InitFloatingHpWidget`
  (`parent.InitFloatingHpWidget`))

(fn `UserConstructionScript`
  (`self.InitAsset` 1200)
  (`self.InitEnemyCharacter` 1200))