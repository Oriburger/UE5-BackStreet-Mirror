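; Boss enemy Blueprint that extends a parent enemy class and links itself to the pillars in the level.
; One tick after BeginPlay it gathers every BP_Pillar actor and initializes each valid one with itself as the boss reference.
; The construction script calls InitAsset with a fixed number, and the floating HP widget setup defers to the parent.
; A debug helper prints inventory index, weapon count and capacity on screen.
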(event `self.ReceiveBeginPlay`
  (`parent.ReceiveBeginPlay`)
  (`KismetSystemLibrary.DelayUntilNextTick`)
  (bind _outactors (`GameplayStatics.GetAllActorsOfClass` "/Game/System/SkillManager/Blueprint/Actor/BP_Pillar.BP_Pillar_C"))
  (bind _output_get (set `self.pillar Array` _outactors))
  (for _array_element _output_get
    (`/Engine/EditorBlueprintResources/StandardMacros.IsValid` _array_element
      (:`Is Valid`
        (`/Game/System/SkillManager/Blueprint/Actor/BP_Pillar.InitializePillar` _array_element self)))))

(event `self.InitFloatingHpWidget`
  (`parent.InitFloatingHpWidget`))

(fn `Print Inventory Info`
  (params (InputPin :type "WeaponInventoryBase Object Reference"))
  (`/Engine/EditorBlueprintResources/StandardMacros.IsValid` InputPin
    (:`Is Valid`
      (`KismetSystemLibrary.PrintString` (`KismetStringLibrary.Concat_StrStr` "Inventory Idx : " (`KismetStringLibrary.Conv_IntToString` (`WeaponInventoryBase.GetCurrentIdx` InputPin)) "   /   " "Weapon Count  :  " (`KismetStringLibrary.Conv_IntToString` (`WeaponInventoryBase.GetCurrentWeaponCount` InputPin)) "  /  Capacity" (`KismetStringLibrary.Conv_IntToString` (`WeaponInventoryBase.GetCurrentCapacity` InputPin))) true false (struct :`G` 0.66 :`B` 1.0 :`A` 1.0) 0.01))))

(fn `UserConstructionScript`
  (`parent.UserConstructionScript`)
  (`self.InitAsset` 1200))