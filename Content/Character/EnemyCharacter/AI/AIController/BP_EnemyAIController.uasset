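; Enemy AI controller that feeds perception results into the blackboard so the AI can target the player.
; On each valid target perception update it calls UpdateTargetPerception, then stores the player character as TargetCharacter if the stimulus is sight of the player.
; The sight branch does not check whether sensing succeeded and never clears the target.
; Activation of the perception component resets ReadyToAttack to false.
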(event `self.AIPerceptionComponent.OnTargetPerceptionUpdated`
  (params (Actor :type "Actor Object Reference") (Stimulus :type "AIStimulus Structure"))
  (bind _returnvalue (`GameplayStatics.GetPlayerCharacter` 0))
  (`/Engine/EditorBlueprintResources/StandardMacros.IsValid` Actor
    (:`Is Valid`
      (`self.UpdateTargetPerception` Actor Stimulus)
      (bind _returnvalue_2 (`AIPerceptionSystem.GetSenseClassForStimulus` Stimulus))
      (if (== _returnvalue_2 "/Script/AIModule.AISense_Sight")
        (if (== Actor _returnvalue)
          (`BlackboardComponent.SetValueAsObject` (`AIBlueprintHelperLibrary.GetBlackboard` null) "TargetCharacter" _returnvalue))))))

(event `self.AIPerceptionComponent.OnComponentActivated`
  (params (Component :type "ActorComponent Object Reference") (bReset :type Boolean))
  (`BlackboardComponent.SetValueAsBool` (`AIBlueprintHelperLibrary.GetBlackboard` null) "ReadyToAttack" false))

(fn `UserConstructionScript`)