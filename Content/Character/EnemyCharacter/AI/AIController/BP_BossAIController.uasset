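; AI controller for the boss enemy, feeding its Blackboard and hooking the boss up to the HUD health bar.
; On BeginPlay it sets the player as TargetCharacter, and a looping timer restores that key whenever it becomes invalid.
; Perception updates go to UpdateTargetPerception, and the first valid one assigns the boss as owner of the HUD boss HP bar.
; Tick mirrors the pawn's action state into the Blackboard.
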(event `self.AIPerceptionComponent.OnTargetPerceptionUpdated`
  (params (Actor :type "Actor Object Reference") (Stimulus :type "AIStimulus Structure"))
  (`/Engine/EditorBlueprintResources/StandardMacros.IsValid` Actor
    (:`Is Valid`
      (`self.UpdateTargetPerception` Actor Stimulus)
      (`/Engine/EditorBlueprintResources/StandardMacros.DoOnce` false
        (:`Completed`
          (bind _asbp_boss_character (cast `/Game/Character/EnemyCharacter/Blueprint/BP_BossCharacter` (`self.K2_GetPawn`)))
          (bind _aswb_main_hud (cast `/Game/UI/InGame/Blueprint/MainHUD/WB_MainHUD` (`/Game/UI/Global/BPFL_CommonWidget.Get Main HUD Ref`)))
          (`/Game/UI/InGame/Blueprint/MainHUD/Component/WB_Comp_BossHPBar.SetOwnerManually` (`/Game/UI/InGame/Blueprint/MainHUD/WB_MainHUD.WB_BossHPBar` _aswb_main_hud) _asbp_boss_character))))))

(event `self.ReceiveBeginPlay`
  (bind _returnvalue (`AIBlueprintHelperLibrary.GetBlackboard` null))
  (`/Engine/EditorBlueprintResources/StandardMacros.IsValid` _returnvalue
    (:`Is Valid`
      (`BlackboardComponent.SetValueAsObject` _returnvalue "TargetCharacter" (`GameplayStatics.GetPlayerCharacter` 0))
      (bind _returnvalue_2 (`KismetSystemLibrary.K2_SetTimerDelegate` (delegate `UpdateTarget`) 0.1 true))
      (set `self.TargetSetTimerHandler` _returnvalue_2))))

(event `UpdateTarget`
  (bind _returnvalue (`GameplayStatics.GetPlayerCharacter` 0))
  (bind _blackboard (`self.Blackboard`))
  (`/Engine/EditorBlueprintResources/StandardMacros.IsValid` _returnvalue
    (:`Is Valid`
      (`/Engine/EditorBlueprintResources/StandardMacros.IsValid` _blackboard
        (:`Is Valid`
          (`/Engine/EditorBlueprintResources/StandardMacros.IsValid` (`BlackboardComponent.GetValueAsObject` _blackboard "TargetCharacter")
            (:`Is Not Valid`
              (`BlackboardComponent.SetValueAsObject` _blackboard "TargetCharacter" _returnvalue))))))))

(event `self.ReceiveTick`
  (params (DeltaSeconds :type "Float (single-precision)"))
  (bind _returnvalue (`self.K2_GetPawn`))
  (`/Engine/EditorBlueprintResources/StandardMacros.IsValid` _returnvalue
    (:`Is Valid`
      (bind _ascharacter_base (cast `CharacterBase` _returnvalue))
      (`BlackboardComponent.SetValueAsEnum` (`AIBlueprintHelperLibrary.GetBlackboard` null) "ActionState" (`.CharacterActionState` (break `CharacterGameplayInfo` (`CharacterBase.GetCharacterGameplayInfoRef` _ascharacter_base)))))))

(fn `UserConstructionScript`)