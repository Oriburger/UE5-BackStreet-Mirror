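; BP_Debug_ItemSpawner is a debug actor in the development map folder that spawns the item matching its ItemID on interaction.
; Construction script looks up the ID in the D_ItemData table and shows the item's name on its ItemName text.
; When InteractiveCollision begins an interaction, it spawns the item class at SpawnPoint, waits briefly, initializes it through BP_ItemBase's InitItem, then activates a particle effect.
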(event `self.InteractiveCollision.OnInteractionBegin`
  (bind _returnvalue (`/Game/UI/Global/BPFL_CommonWidget.GetItemInfo` (`self.ItemID`)))
  (bind _returnvalue_2 (`|SpawnActorFromClass` (`.ItemClass` (break `ItemInfoDataStruct` _returnvalue)) (`SceneComponent.K2_GetComponentToWorld` (`self.SpawnPoint`)) "Undefined" "MultiplyWithRoot" null null))
  (`KismetSystemLibrary.Delay` 0.2)
  (bind _asbp_item_base (cast `/Game/Item/Blueprint/BP_ItemBase` _returnvalue_2))
  (`ItemBase.InitItem` _asbp_item_base (`self.ItemID`) _returnvalue)
  (`ActorComponent.Activate` (`self.ParticleSystem`) true))

(fn `UserConstructionScript`
  (bind _returnvalue (`|GetDataTableRow` "/Game/Item/Data/D_ItemData.D_ItemData" (`KismetStringLibrary.Conv_StringToName` (`KismetStringLibrary.Conv_IntToString` (`self.ItemID`))))
    (:`then`
      (`TextRenderComponent.K2_SetText` (`self.ItemName`) (`.ItemNameText` (break `ItemInfoDataStruct` _returnvalue))))))