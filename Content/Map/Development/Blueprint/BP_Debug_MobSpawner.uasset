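; Debug interactable that spawns an enemy of a configurable class and ID when the player interacts with it.
; Interaction availability toggles the ChildActor component's visibility, and the construction script writes the EnemyID onto the ItemName text.
; On interaction it spawns at SpawnPoint, initializes the enemy by ID, requests a default controller and activates a particle effect.
; A DoOnce with a short delay forms a cooldown, during which Cube3 is hidden.
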(event `self.InteractiveCollision.OnInteractionAvailableStateUpdate`
  (params (bNewState :type Boolean))
  (`SceneComponent.SetVisibility` (`self.ChildActor`) bNewState false))

(event `self.InteractiveCollision.OnInteractionBegin`
  (bind _enemyid (`self.EnemyID`))
  (`/Engine/EditorBlueprintResources/StandardMacros.IsValid` (`/Game/UI/Global/BPFL_CommonWidget.GetMainCharacterRef`)
    (:`Is Valid`
      (`/Engine/EditorBlueprintResources/StandardMacros.DoOnce` false :!label _label
        (:`Completed`
          (bind _returnvalue (`|SpawnActorFromClass` (`self.CustomClass Override`) (`SceneComponent.K2_GetComponentToWorld` (`self.Spawn Point`)) "Undefined" "MultiplyWithRoot" null null))
          (`EnemyCharacterBase.InitEnemyCharacter` _returnvalue _enemyid)
          (`EnemyCharacterBase.InitAsset` _returnvalue _enemyid)
          (`Pawn.SpawnDefaultController` (`Actor.Instigator` _returnvalue))
          (`ActorComponent.Activate` (`self.ParticleSystem`) true)
          (`SceneComponent.SetVisibility` (`self.Cube3`) false false)
          (`KismetSystemLibrary.Delay` 1.0)
          (`SceneComponent.SetVisibility` (`self.Cube3`) true false)
          (goto _label :!via `Reset`))))))

(fn `UserConstructionScript`
  (`TextRenderComponent.K2_SetText` (`self.ItemName`) (`KismetTextLibrary.Conv_StringToText` (`KismetStringLibrary.Conv_IntToString` (`self.EnemyID`)))))