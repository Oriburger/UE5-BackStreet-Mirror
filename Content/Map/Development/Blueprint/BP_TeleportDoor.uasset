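; BP_TeleportDoor is an interactive door that teleports the player to a linked OtherPoint actor on interaction.
; If the target is another teleport door, the player takes its Arrow's transform; otherwise they land above the actor with its rotation.
; A DoOnce reset after a short delay throttles repeat use.
; The InteractiveCollision's availability state shows or hides a child actor.
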(event `self.InteractiveCollision.OnInteractionBegin`
  (bind _returnvalue (`GameplayStatics.GetPlayerCharacter` 0))
  (bind _otherpoint (`self.OtherPoint`))
  (`/Engine/EditorBlueprintResources/StandardMacros.IsValid` _otherpoint
    (:`Is Valid`
      (`/Engine/EditorBlueprintResources/StandardMacros.DoOnce` false :!label _label
        (:`Completed`
          (bind _asbp_teleport_door (cast `/Game/Map/Development/Blueprint/BP_TeleportDoor` _otherpoint)
            (:`then`
              (bind _arrow (`/Game/Map/Development/Blueprint/BP_TeleportDoor.Arrow` _asbp_teleport_door))
              (`self.K2_SetActorLocationAndRotation` _returnvalue (`SceneComponent.K2_GetComponentLocation` _arrow) (`SceneComponent.K2_GetComponentRotation` _arrow) false true))
            (:`CastFailed`
              (`self.K2_SetActorLocationAndRotation` _returnvalue (+ (`self.K2_GetActorLocation` _otherpoint) (0.0 0.0 200.0)) (`self.K2_GetActorRotation` _otherpoint) false true)))
          (`KismetSystemLibrary.Delay` 1.0)
          (goto _label :!via `Reset`))))))

(event `self.InteractiveCollision.OnInteractionAvailableStateUpdate`
  (params (bNewState :type Boolean))
  (`self.SetActorHiddenInGame` (`ChildActorComponent.ChildActor` (`self.ChildActor`)) (not bNewState)))

(fn `UserConstructionScript`)