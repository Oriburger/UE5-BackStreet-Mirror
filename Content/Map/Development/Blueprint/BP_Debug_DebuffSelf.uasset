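; BP_Debug_DebuffSelf is a debug interactable that applies a configurable debuff to the main character.
; Its InteractiveCollision toggles a ChildActor's visibility with interaction availability and, on interaction, builds the debuff from its variables.
; Each use activates a particle effect and hides Cube3 for a one-second cooldown gated by a DoOnce.
; The construction script sets the ItemName text to the selected debuff type.
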(event `self.InteractiveCollision.OnInteractionAvailableStateUpdate`
  (params (bNewState :type Boolean))
  (`SceneComponent.SetVisibility` (`self.ChildActor`) bNewState false))

(event `self.InteractiveCollision.OnInteractionBegin`
  (bind _returnvalue__ (`/Game/UI/Global/BPFL_CommonWidget.GetMainCharacterRef`))
  (`/Engine/EditorBlueprintResources/StandardMacros.IsValid` _returnvalue__
    (:`Is Valid`
      (`/Engine/EditorBlueprintResources/StandardMacros.DoOnce` false :!label _label
        (:`Completed`
          (`CharacterBase.TryAddNewDebuff` _returnvalue__ (make `DebuffInfoStruct` (`self.Type`) (`self.Total Time`) (`self.Variable`) (`self.Is Percentage`)) self)
          (`ActorComponent.Activate` (`self.ParticleSystem`) true)
          (`SceneComponent.SetVisibility` (`self.Cube3`) false false)
          (`KismetSystemLibrary.Delay` 1.0)
          (`SceneComponent.SetVisibility` (`self.Cube3`) true false)
          (goto _label :!via `Reset`))))))

(fn `UserConstructionScript`
  (`TextRenderComponent.K2_SetText` (`self.ItemName`) (`KismetTextLibrary.Conv_StringToText` (`|GetEnumeratorNameAsString` (`self.Type`)))))