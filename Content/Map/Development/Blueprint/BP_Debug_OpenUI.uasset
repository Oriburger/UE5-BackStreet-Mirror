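; Debug interactable actor that opens a configurable UI widget, labeled in the level with that widget class's name by the construction script.
; An interaction collision toggles a child actor as the key guide and, on interaction with a valid main character, creates the widget and adds a media sound component.
; A DoOnce blocks repeat opens until ResetState, apparently bound to widget removal, destroys the sound component and resets the gate.
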(event `self.InteractiveCollision.OnInteractionAvailableStateUpdate`
  (params (bNewState :type Boolean))
  ;[1 1 1] 키 가이드
  (`SceneComponent.SetVisibility` (`self.ChildActor`) bNewState false))

(event `self.InteractiveCollision.OnInteractionBegin`
  ;[1 0.3966 0.2564] 위젯 및 미디어 컴포넌트 생성
  (`/Engine/EditorBlueprintResources/StandardMacros.IsValid` (`/Game/UI/Global/BPFL_CommonWidget.GetMainCharacterRef`)
    (:`Is Valid`
      (`/Engine/EditorBlueprintResources/StandardMacros.DoOnce` false :!label _label
        (:`Completed`
          (bind _widgetref (`/Game/EasyGameUI/Core/BFL_EasyFunctionUtilities.SafeCreateWidget` (`self.Widget Class`)))
          (bind _aswb_cui_activatable_base (cast `/Game/UI/Global/WB_CUI_ActivatableBase` _widgetref))
          (bind _returnvalue (`AddComponent|NODE_AddMediaSoundComponent-1`))
          (add `/Game/UI/Global/WB_CUI_ActivatableBase.OnWidgetRemoved` _aswb_cui_activatable_base (`|CreateDelegate` :!event `ResetState`))
          (set `self.MediaSoundComponentRef` _returnvalue))))))

(event `ResetState`
  (bind _mediasoundcomponentref (`self.MediaSoundComponentRef`))
  ;[1 0.3966 0.2564] 위젯 및 미디어 컴포넌트 생성
  ;;[1 0 0 0.491] 위젯 제거 이후, 상태 초기화
  (`SynthComponent.Stop` _mediasoundcomponentref)
  (`ActorComponent.K2_DestroyComponent` _mediasoundcomponentref)
  (goto _label :!via `Reset`))

(fn `UserConstructionScript`
  (`TextRenderComponent.K2_SetText` (`self.ItemName`) (`KismetTextLibrary.Conv_StringToText` (`KismetSystemLibrary.GetClassDisplayName` (`self.Widget Class`)))))