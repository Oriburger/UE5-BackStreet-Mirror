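; BP_Test_UI is a test actor that opens a UI when its InteractiveCollision begins an interaction, chosen by an EUICommand enum.
; The info option lazily creates and reuses WB_UI_Info, nearly freezes global time dilation and switches to UI-only input with a cursor.
; The crafting option re-adds WB_UI_MainCrafting to the combat UI main stack and initializes it with the CraftingManagerComponent.
; The weapon select option is an empty stub.
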(event `self.ReceiveTick`
  (params (DeltaSeconds :type "Float (single-precision)")))

(event `self.InteractiveCollision.OnInteractionBegin`
  (switch `/Game/Map/Blueprint/EUICommand` (`self.EUICommand`)
    (:`NewEnumerator0`
      (`self.OpenInfoUI`))
    (:`NewEnumerator1`
      (`self.OpenWeaponSelectUI`))
    (:`NewEnumerator3`
      (`self.OpenCraftingUI`))))

(fn `OpenCraftingUI`
  (bind _returnvalue (`/Game/UI/Global/BPFL_CommonWidget.Get Combat UI Main Stack`))
  (bind _craftingmanagercomponent (`self.CraftingManagerComponent`))
  (bind _maincraftingwidgetref (`self.MainCraftingWidgetRef`))
  (bind _maincraftingwidgetref_2 (`self.MainCraftingWidgetRef`))
  (`/Engine/EditorBlueprintResources/StandardMacros.IsValid` _maincraftingwidgetref_2
    (:`Is Valid`
      (`Widget.RemoveFromParent` _maincraftingwidgetref_2)
      (set `self.MainCraftingWidgetRef` null))
    (:`Is Not Valid`
      _))
  (`/Engine/EditorBlueprintResources/StandardMacros.IsValid` _returnvalue
    (:`Is Valid`
      (`|ExecutionSequence`
        (:`then_0`
          (bind _returnvalue_2 (`CommonActivatableWidgetContainerBase.BP_AddWidget` _returnvalue "/Game/UI/InGame/Blueprint/04_CraftingUI/WB_UI_MainCrafting.WB_UI_MainCrafting_C"))
          (set `self.MainCraftingWidgetRef` _returnvalue_2))
        (:`then_1`
          (`/Engine/EditorBlueprintResources/StandardMacros.IsValid` _craftingmanagercomponent
            (:`Is Valid`
              (`/Game/UI/InGame/Blueprint/04_CraftingUI/WB_UI_MainCrafting.Initialize` _maincraftingwidgetref _craftingmanagercomponent)
              (`CommonActivatableWidget.ActivateWidget` _maincraftingwidgetref))
            (:`Is Not Valid`
              (`KismetSystemLibrary.PrintString` "BP_TestUI : Crafting Manager Is Not Valid"))))))))

(fn `OpenInfoUI`
  (bind _returnvalue (`GameplayStatics.GetPlayerController` 0))
  (bind _wb_ui_info (`self.WB_UI_Info`))
  (`/Engine/EditorBlueprintResources/StandardMacros.IsValid` (`self.WB_UI_Info`)
    (:`Is Valid`
      (`GameplayStatics.SetGlobalTimeDilation` 0.001 :!label _label)
      (`WidgetBlueprintLibrary.SetInputMode_UIOnlyEx` _returnvalue _wb_ui_info)
      (`UserWidget.AddToViewport` _wb_ui_info 0)
      (set `PlayerController.bShowMouseCursor` true _returnvalue))
    (:`Is Not Valid`
      (`|ExecutionSequence`
        (:`then_0`
          (bind _returnvalue_2 (`|CreateWidget` "/Game/UI/New/InfoMenu/WB_UI_Info.WB_UI_Info_C" (`GameplayStatics.GetPlayerController` 0)))
          (set `self.WB_UI_Info` _returnvalue_2))
        (:`then_1`
          (goto _label))))))

(fn `OpenWeaponSelectUI`)

(fn `UserConstructionScript`)