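; BP_CraftBox is a map object that opens the main crafting UI.
; EnterUI creates and initializes WB_UI_MainCrafting, nearly freezes time through global time dilation, switches input to UI-only and shows the cursor.
; The construction script makes its text render component visible, while BeginPlay calls the parent and has an empty Tutorial tag branch.
; A disconnected copy of the opening sequence targets the skill-select widget and never runs.
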(event `self.ReceiveBeginPlay`
  (`parent.ReceiveBeginPlay`)
  (if (`self.ActorHasTag` "Tutorial")
    _))

(event `self.EnterUI`
  (params (Causer :type "Actor Object Reference"))
  (bind _returnvalue (`GameplayStatics.GetPlayerController` 0))
  ;[1 1 1] Press F 팝업 문구 제거
  (bind _returnvalue_2 (`|CreateWidget` "/Game/UI/InGame/Blueprint/08_CraftingUI/WB_UI_MainCrafting.WB_UI_MainCrafting_C" (`GameplayStatics.GetPlayerController` 0)))
  (`GameplayStatics.SetGlobalTimeDilation` 0.001)
  (`WidgetBlueprintLibrary.SetInputMode_UIOnlyEx` _returnvalue _returnvalue_2)
  (`/Game/UI/InGame/Blueprint/08_CraftingUI/WB_UI_MainCrafting.Initialize` _returnvalue_2)
  (`UserWidget.AddToViewport` _returnvalue_2 0)
  (set `PlayerController.bShowMouseCursor` true _returnvalue))

(fn `UserConstructionScript`
  (`SceneComponent.SetVisibility` (`self.TextRenderComp`) true false))