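; Component that gives its owner an on-screen direction indicator widget, with the component itself set as the widget's target.
; On request it creates a single WB_DirectionIndicator_ with its icon image and adds it to the viewport.
; It can play a normal or fast highlight animation on the widget, looping indefinitely at a given speed.
; The widget is removed and cleared on an explicit destroy call or on EndPlay.
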(event `CreateDirectionIndicator`
  ;[1 1 1] 위젯 생성
  (`self.Direction Indicator Widget`
    (:`then`)
    (:`else`
      (`|ExecutionSequence`
        (:`then_0`
          (bind _returnvalue (`|CreateWidget` "/Game/UI/InGame/Blueprint/CombatUI/Component/WB_DirectionIndicator_.WB_DirectionIndicator__C" (`GameplayStatics.GetPlayerController` 0) null (`self.Icon Image`)))
          (set `/Game/UI/InGame/Blueprint/CombatUI/Component/WB_DirectionIndicator_.Targeted Component` self _returnvalue)
          (`UserWidget.AddToViewport` _returnvalue 0)
          (set `self.Direction Indicator Widget` _returnvalue))))))

(event `self.ReceiveEndPlay`
  (params (EndPlayReason :type "EEndPlayReason Enum" :default "Destroyed"))
  (bind _direction_indicator_widget (`self.Direction Indicator Widget` :!label _label)
    (:`then`
      (`Widget.RemoveFromParent` _direction_indicator_widget)
      (set `self.Direction Indicator Widget` null))
    (:`else`)))

(event `PlayHighlightAnimation`
  (params (bIsFastAnimation :type Boolean) (PlaybackSpeed :type "Float (single-precision)"))
  (bind _direction_indicator_widget (`self.Direction Indicator Widget`)
    (:`then`
      (bind _aswb_direction_indicator_ (cast `/Game/UI/InGame/Blueprint/CombatUI/Component/WB_DirectionIndicator_` _direction_indicator_widget))
      (`UserWidget.PlayAnimation` _direction_indicator_widget (select `bool` bIsFastAnimation :`false` (`/Game/UI/InGame/Blueprint/CombatUI/Component/WB_DirectionIndicator_.Highlighting` _aswb_direction_indicator_) :`true` (`/Game/UI/InGame/Blueprint/CombatUI/Component/WB_DirectionIndicator_.Highlighting_Fast` _aswb_direction_indicator_)) 0.0 0 "Forward" PlaybackSpeed false))
    (:`else`)))

(event `DestroyDirectionalIndicator`
  (goto _label))