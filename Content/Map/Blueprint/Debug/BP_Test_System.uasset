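; Debug interactable that runs one configurable test command on the player character, with the command name shown on its text render.
; On interaction it switches on the command enum to add skills, grant crafting items, upgrade weapon stats or apply a debuff.
; Each command calls the matching component or function on the MainCharacterBase cached at BeginPlay.
; The skill upgrade command is an empty stub.
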(event `self.ReceiveBeginPlay`
  (bind _asmain_character_base (cast `MainCharacterBase` (`GameplayStatics.GetPlayerCharacter` 0)))
  (set `self.Main Character Ref` _asmain_character_base))

(event `self.InteractiveCollision.OnInteractionBegin`
  (switch `/Game/Map/Blueprint/Data/ESystemCommand` (`self.ESystemCommand`)
    (:`NewEnumerator3`
      (for _array_element (`self.SkillID_AS`)
        (`self.AddSkill` _array_element)))
    (:`NewEnumerator4`
      (`self.UpgradeSkill`))
    (:`NewEnumerator1`
      (`self.GetCraftingItem`))
    (:`NewEnumerator2`
      (`self.UpgradeWeapon`))
    (:`NewEnumerator5`
      (`self.AddDebuff` (`self.Type`) (`self.Total Time`) (`self.Variable`) (`self.Is Percentage`)))))

(fn `AddDebuff`
  (params (Type :type "ECharacterDebuffType Enum" :default "E_None") (`Total Time` :type "Float (single-precision)") (Variable :type "Float (single-precision)") (`Is Percentage` :type Boolean))
  (bind _main_character_ref (`self.Main Character Ref`))
  (`CharacterBase.TryAddNewDebuff` _main_character_ref (make `DebuffInfoStruct` Type `Total Time` Variable `Is Percentage`) _main_character_ref))

(fn `AddSkill`
  (params (NewSkillID :type Integer))
  (locals (CharacterStat :type " Structure"))
  (bind _returnvalue (`SkillManagerComponentBase.TryAddSkill` (`MainCharacterBase.SkillManagerComponent` (`self.Main Character Ref`)) NewSkillID))
  (`KismetSystemLibrary.PrintString` (`KismetStringLibrary.Conv_BoolToString` _returnvalue)))

(fn `GetCraftingItem`
  (for _array_element (`self.ItemID`)
    (`ItemInventoryComponent.AddItem` (`MainCharacterBase.ItemInventory` (`self.Main Character Ref`)) _array_element 1)))

(fn `UpgradeSkill`
  (locals (CharacterStat :type " Structure")))

(fn `UpgradeWeapon`
  (locals (NewLevelList :type "Array of Byte"))
  (bind _new_level_map (`self.New Level Map`))
  (bind _keys (`BlueprintMapLibrary.Map_Keys` _new_level_map))
  (for _array_element _keys
    (`KismetArrayLibrary.Array_Add` (`local.NewLevelList`) (`BlueprintMapLibrary.Map_Find` _new_level_map _array_element)))
  (bind _returnvalue (`WeaponComponentBase.UpgradeStat` (`CharacterBase.WeaponComponent` (`self.Main Character Ref`)) (`local.NewLevelList`)))
  (if _returnvalue
    (`KismetSystemLibrary.PrintString` "Hello")))

(fn `UserConstructionScript`
  (`TextRenderComponent.K2_SetText` (`self.TextRender`) (`KismetTextLibrary.Conv_StringToText` (`|GetEnumeratorNameAsString` (`self.ESystemCommand`)))))