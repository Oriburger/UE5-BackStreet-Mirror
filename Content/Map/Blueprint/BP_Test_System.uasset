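; Test actor that grants skills, skill upgrades or crafting items to the main character through an interaction.
; On interaction begin, ESystemCommand selects adding listed skills, raising one skill's level via SkillManagerComponent, or adding listed items to the inventory.
; Both skill commands set InfiniteSkillMaterial from IsCraftingMatInfinite beforehand, then write its inverse rather than the saved value.
; AddSkill writes that inverse inside its loop, after each skill.
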(event `self.ReceiveBeginPlay`
  (bind _asbp_main_character (cast `/Game/Character/MainCharacter/BP_MainCharacter` (`GameplayStatics.GetPlayerCharacter` 0)))
  (set `self.Main Character Ref` _asbp_main_character))

(event `self.InteractiveCollision.OnInteractionBegin`
  (switch `/Game/Map/Blueprint/ESystemCommand` (`self.ESystemCommand`)
    (:`NewEnumerator3`
      (`self.AddSkill`))
    (:`NewEnumerator4`
      (`self.UpgradeSkill`))
    (:`NewEnumerator1`
      (`self.GetCraftingItem`))))

(fn `AddSkill`
  (locals (CharacterStat :type "CharacterStatStruct Structure"))
  (bind _main_character_ref (`self.Main Character Ref`))
  (bind _output_get (set `local.CharacterStat` (`CharacterBase.GetCharacterStat` _main_character_ref)))
  (bind _structout (setmembers `CharacterStatStruct` :`StructRef` _output_get :`bInfiniteSkillMaterial` (`self.IsCraftingMatInfinite`)))
  (`CharacterBase.UpdateCharacterStat` _main_character_ref _structout)
  (for _array_element (`self.SkillID_AS`)
    (bind _returnvalue (`PlayerSkillManagerComponent.AddSkill` (`MainCharacterBase.SkillManagerComponent` (`self.Main Character Ref`)) _array_element))
    (if (not _returnvalue)
      (`KismetSystemLibrary.PrintString` "Failed"))
    (bind _structout_2 (setmembers `CharacterStatStruct` :`StructRef` (`local.CharacterStat`) :`bInfiniteSkillMaterial` (not (`self.IsCraftingMatInfinite`))))
    (`CharacterBase.UpdateCharacterStat` (`self.Main Character Ref`) _structout_2)))

(fn `GetCraftingItem`
  (for _array_element (`self.ItemID`)
    (`ItemInventoryComponent.AddItem` (`MainCharacterBase.ItemInventory` (`self.Main Character Ref`)) _array_element 1)))

(fn `UpgradeSkill`
  (locals (CharacterStat :type "CharacterStatStruct Structure"))
  (bind _skillid_us (`self.SkillID_US`))
  (bind _main_character_ref (`self.Main Character Ref`))
  (bind _returnvalue (`CharacterBase.GetCharacterStat` _main_character_ref))
  (bind _skillmanagercomponent (`MainCharacterBase.SkillManagerComponent` (`self.Main Character Ref`)))
  (bind _output_get (set `local.CharacterStat` _returnvalue))
  (bind _structout (setmembers `CharacterStatStruct` :`StructRef` _output_get :`bInfiniteSkillMaterial` (`self.IsCraftingMatInfinite`)))
  (`CharacterBase.UpdateCharacterStat` _main_character_ref _structout)
  (`PlayerSkillManagerComponent.UpgradeSkill` _skillmanagercomponent _skillid_us (+ (`.SkillLevel` (break `SkillLevelStateStruct` (`.SkillLevelStateStruct` (break `SkillStateStruct` (`SkillManagerComponentBase.GetOwnSkillState` _skillmanagercomponent _skillid_us))))) (`self.SkillAdder_US`)))
  (bind _structout_2 (setmembers `CharacterStatStruct` :`StructRef` _returnvalue :`bInfiniteSkillMaterial` (not (`self.IsCraftingMatInfinite`))))
  (`CharacterBase.UpdateCharacterStat` (`self.Main Character Ref`) _structout_2))

(fn `UserConstructionScript`)