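; BP_BattleZoneTransitionGate is a battle zone gate that opens once all tracked actors from its related spawn points are destroyed.
; After the chapter's stage manager reports stage load done, it waits briefly, collects matching-class actors from those spawn points into a set and binds to their destruction.
; Each destruction shrinks the set, and an empty set triggers the parent's open logic once.
; With no spawn points or matching actors, the gate destroys itself.
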(event `self.ReceiveTick`
  (params (DeltaSeconds :type "Float (single-precision)")))

(event `self.ReceiveBeginPlay`
  (bind _returnvalue (`/Game/UI/Global/BPFL_CommonWidget.GetChapterManagerRef`))
  ;[1 1 1] Begin Play
  (`parent.ReceiveBeginPlay`)
  (`/Engine/EditorBlueprintResources/StandardMacros.IsValid` _returnvalue
    (:`Is Valid`
      (add `StageManagerComponent.OnStageLoadDone` (`NewChapterManagerBase.StageManagerComponent` _returnvalue) (delegate `OnStageLoadDone`)))))

(event `OnStageLoadDone`
  (bind _relatedspawnpoint (`self.RelatedSpawnPoint`))
  ;[1 1 1] Begin Play
  ;;[1 0.2927 0.8091] 스테이지 로드 직후
  (`KismetSystemLibrary.Delay` 0.75)
  (if (`KismetArrayLibrary.Array_IsNotEmpty` _relatedspawnpoint)
    (for _array_element _relatedspawnpoint
      (for _array_element_2 (`/Game/Map/Blueprint/BP_SpawnPoint.RelatedActorList` _array_element)
        (`/Engine/EditorBlueprintResources/StandardMacros.IsValid` _array_element_2
          (:`Is Valid`
            (if (`GameplayStatics.ObjectIsA` _array_element_2 (`self.RelatedActorClass`))
              (`BlueprintSetLibrary.Set_Add` (`self.RelatedActorSet`) _array_element_2)
              (add `self.OnDestroyed` _array_element_2 (delegate `OnRelatedActorDestroyed`)))))))
    (else
      (`self.K2_DestroyActor`)))
  (if (`BlueprintSetLibrary.Set_IsEmpty` (`self.RelatedActorSet`))
    (`self.K2_DestroyActor`)))

(event `OnRelatedActorDestroyed` :!signature `self.OnDestroyed`
  (params (DestroyedActor :type "Actor Object Reference"))
  (bind _relatedactorset (`self.RelatedActorSet`))
  ;[1 0.6823 0.5233] Disappear Trigger : 관련 액터 전부 소멸 시
  (`BlueprintSetLibrary.Set_Remove` _relatedactorset DestroyedActor)
  (if (`BlueprintSetLibrary.Set_IsEmpty` _relatedactorset)
    (`/Engine/EditorBlueprintResources/StandardMacros.DoOnce` false
      (:`Completed`
        (`self.OpenGate`)))))

(event `self.InitDynamicMaterial`
  ;[1 1 1] Override
  (`parent.InitDynamicMaterial`))

(event `self.OpenGate`
  ;[1 1 1] Override
  (`parent.OpenGate`))

(fn `UserConstructionScript`
  (`parent.UserConstructionScript`))