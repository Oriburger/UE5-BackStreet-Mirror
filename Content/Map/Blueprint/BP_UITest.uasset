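; BP_UITest is a map actor that opens a menu screen for the player, selected by its EUICommand value.
; Overlapping its volume shows or hides the "Press F" guide text, while EnterUI checks the Player tag and opens the stat, weapon select, skill select or stat upgrade widget.
; Each opener nearly freezes time through global time dilation, switches to UI-only input and shows the cursor.
; A skill upgrade opener exists but EnterUI never calls it.
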(event `self.ReceiveBeginPlay`
  (`parent.ReceiveBeginPlay`)
  (if true
    _))

(event `self.OverlapVolume.OnComponentBeginOverlap`
  (params (OverlappedComponent :type "PrimitiveComponent Object Reference") (OtherActor :type "Actor Object Reference") (OtherComp :type "PrimitiveComponent Object Reference") (OtherBodyIndex :type Integer) (bFromSweep :type Boolean) (SweepResult :type "HitResult Structure (by ref)"))
  ;[1 1 1] Press F 팝업 문구 호출
  (`self.VisibleGuideTextRender` OtherActor))

(event `self.OverlapVolume.OnComponentEndOverlap`
  (params (OverlappedComponent :type "PrimitiveComponent Object Reference") (OtherActor :type "Actor Object Reference") (OtherComp :type "PrimitiveComponent Object Reference") (OtherBodyIndex :type Integer))
  ;[1 1 1] Press F 팝업 문구 제거
  (`self.InVisibleGuideTextRender` OtherActor))

(event `self.EnterUI`
  (params (Causer :type "Actor Object Reference"))
  ;[1 1 1] Press F 팝업 문구 제거
  (if (`self.ActorHasTag` Causer "Player")
    (switch `/Game/Map/Blueprint/EUICommand` (`self.EUICommand`)
      (:`NewEnumerator0`
        ;;[1 0.4431 0.513] Stat
        (`self.OpenStatUI`))
      (:`NewEnumerator1`
        ;;[0.5794 0.4828 1] WeaponSelect
        (`self.OpenWeaponSelectUI`))
      (:`NewEnumerator3`
        (`self.OpenSkillSelectUI`))
      (:`NewEnumerator5`
        (`self.OpenStatUPgradeUI`)))))

(fn `OpenSkillSelectUI`
  (locals (WB_UI_SkillSelect :type "/Game/UI/InGame/Blueprint/04_CraftingUI/WB_UISkillSelect Object Reference"))
  (bind _returnvalue (`GameplayStatics.GetPlayerController` 0))
  (bind _returnvalue_2 (`|CreateWidget` "/Game/UI/InGame/Blueprint/04_CraftingUI/WB_UISkillSelect.WB_UISkillSelect_C" (`GameplayStatics.GetPlayerController` 0)))
  (bind _output_get (set `local.WB_UI_SkillSelect` _returnvalue_2))
  (`GameplayStatics.SetGlobalTimeDilation` 0.001)
  (`WidgetBlueprintLibrary.SetInputMode_UIOnlyEx` _returnvalue _output_get)
  (`/Game/UI/InGame/Blueprint/04_CraftingUI/WB_UISkillSelect.Initialize` _output_get)
  (`UserWidget.AddToViewport` _output_get 0)
  (set `PlayerController.bShowMouseCursor` true _returnvalue))

(fn `OpenSkillUpgradeUI`
  (locals (WB_UI_SkillUpgrade :type "/Game/UI/InGame/Blueprint/04_CraftingUI/WB_UISkillUpgrade Object Reference"))
  (bind _returnvalue (`GameplayStatics.GetPlayerController` 0))
  (bind _returnvalue_2 (`|CreateWidget` "/Game/UI/InGame/Blueprint/04_CraftingUI/WB_UISkillUpgrade.WB_UISkillUpgrade_C" (`GameplayStatics.GetPlayerController` 0)))
  (bind _output_get (set `local.WB_UI_SkillUpgrade` _returnvalue_2))
  (`GameplayStatics.SetGlobalTimeDilation` 0.001)
  (`WidgetBlueprintLibrary.SetInputMode_UIOnlyEx` _returnvalue _output_get)
  (`/Game/UI/InGame/Blueprint/04_CraftingUI/WB_UISkillUpgrade.Initialize` :`self` _output_get)
  (`UserWidget.AddToViewport` _output_get 0)
  (set `PlayerController.bShowMouseCursor` true _returnvalue))

(fn `OpenStatUI`
  (locals (StatUI :type "/Game/UI/InGame/Blueprint/03_StatUI/WB_StatUI Object Reference"))
  (bind _returnvalue (`GameplayStatics.GetPlayerController` 0))
  (bind _returnvalue_2 (`|CreateWidget` "/Game/UI/InGame/Blueprint/03_StatUI/WB_StatUI.WB_StatUI_C" (`GameplayStatics.GetPlayerController` 0)))
  (bind _output_get (set `local.StatUI` _returnvalue_2))
  (`GameplayStatics.SetGlobalTimeDilation` 0.001)
  (`WidgetBlueprintLibrary.SetInputMode_UIOnlyEx` _returnvalue _output_get)
  (`/Game/UI/InGame/Blueprint/03_StatUI/WB_StatUI.Initialize` _output_get null)
  (`UserWidget.AddToViewport` _output_get 0)
  (set `PlayerController.bShowMouseCursor` true _returnvalue))

(fn `OpenStatUPgradeUI`
  (locals (WB_UI_StatUpgrade :type "/Game/UI/InGame/Blueprint/04_CraftingUI/WB_UIStatUpgrade Object Reference"))
  (bind _returnvalue (`GameplayStatics.GetPlayerController` 0))
  (bind _returnvalue_2 (`|CreateWidget` "/Game/UI/InGame/Blueprint/04_CraftingUI/WB_UIStatUpgrade.WB_UIStatUpgrade_C" (`GameplayStatics.GetPlayerController` 0)))
  (bind _output_get (set `local.WB_UI_StatUpgrade` _returnvalue_2))
  (`GameplayStatics.SetGlobalTimeDilation` 0.001)
  (`WidgetBlueprintLibrary.SetInputMode_UIOnlyEx` _returnvalue null)
  (`/Game/UI/InGame/Blueprint/04_CraftingUI/WB_UIStatUpgrade.Initialize` _output_get)
  (`UserWidget.AddToViewport` _output_get 0)
  (set `PlayerController.bShowMouseCursor` true _returnvalue))

(fn `OpenWeaponSelectUI`
  (locals (MainWeaponSelectUI :type "/Game/UI/InGame/Blueprint/02_WeaponSelectUI/WB_UIMainWeaponSelect Object Reference"))
  (bind _returnvalue (`GameplayStatics.GetPlayerController` 0))
  (bind _returnvalue_2 (`|CreateWidget` "/Game/UI/InGame/Blueprint/02_WeaponSelectUI/WB_UIMainWeaponSelect.WB_UIMainWeaponSelect_C" (`GameplayStatics.GetPlayerController` 0)))
  (bind _output_get (set `local.MainWeaponSelectUI` _returnvalue_2))
  (`GameplayStatics.SetGlobalTimeDilation` 0.001)
  (`WidgetBlueprintLibrary.SetInputMode_UIOnlyEx` _returnvalue _output_get)
  (`/Game/UI/InGame/Blueprint/02_WeaponSelectUI/WB_UIMainWeaponSelect.Initialize` _output_get)
  (`UserWidget.AddToViewport` _output_get 0)
  (set `PlayerController.bShowMouseCursor` true _returnvalue))

(fn `UserConstructionScript`
  (`SceneComponent.SetVisibility` (`self.TextRenderComp`) true false))