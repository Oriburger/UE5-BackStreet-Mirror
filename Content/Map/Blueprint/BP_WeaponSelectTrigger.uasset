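; BP_WeaponSelectTrigger is a one-shot map trigger that opens the main weapon selection screen for the player.
; When an actor tagged Player stops overlapping its Box, it creates and initializes WB_UIMainWeaponSelect, then destroys itself.
; While opening the menu, it slows global time to a near standstill, switches input to UI only and shows the mouse cursor.
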(event `self.Box.OnComponentEndOverlap`
  (params (OverlappedComponent :type "PrimitiveComponent Object Reference") (OtherActor :type "Actor Object Reference") (OtherComp :type "PrimitiveComponent Object Reference") (OtherBodyIndex :type Integer))
  (`/Engine/EditorBlueprintResources/StandardMacros.IsValid` OtherActor
    (:`Is Valid`
      (if (`self.ActorHasTag` OtherActor "Player")
        (`/Engine/EditorBlueprintResources/StandardMacros.DoOnce` false
          (:`Completed`
            (`self.OpenWeaponSelectUI`)
            (`self.K2_DestroyActor`)))))))

(fn `OpenWeaponSelectUI`
  (locals (MainWeaponSelectUI :type "/Game/UI/InGame/Blueprint/02_WeaponSelectUI/WB_UIMainWeaponSelect Object Reference"))
  (bind _returnvalue (`GameplayStatics.GetPlayerController` 0))
  (bind _returnvalue_2 (`|CreateWidget` "/Game/UI/InGame/Blueprint/02_WeaponSelectUI/WB_UIMainWeaponSelect.WB_UIMainWeaponSelect_C" (`GameplayStatics.GetPlayerController` 0)))
  (bind _output_get (set `local.MainWeaponSelectUI` _returnvalue_2))
  (`GameplayStatics.SetGlobalTimeDilation` 0.001)
  (`WidgetBlueprintLibrary.SetInputMode_UIOnlyEx` _returnvalue _output_get)
  (`/Game/UI/InGame/Blueprint/02_WeaponSelectUI/WB_UIMainWeaponSelect.Initialize` _output_get)
  (`UserWidget.AddToViewport` _output_get 0)
  (set `PlayerController.bShowMouseCursor` true _returnvalue))

(fn `UserConstructionScript`)