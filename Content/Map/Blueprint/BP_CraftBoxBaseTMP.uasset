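; Craft box base Blueprint that opens a skill selection screen when its EnterUI event fires.
; EnterUI creates and initializes WB_UISkillSelect, adds it to the viewport, switches to UI-only input with a visible cursor, and slows global time to near zero as a pseudo-pause.
; The construction script makes its text render component visible.
; BeginPlay calls the parent and checks a Tutorial tag without acting on it.
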(event `self.ReceiveBeginPlay`
  (`parent.ReceiveBeginPlay`)
  (if (`self.ActorHasTag` "Tutorial")
    _))

(event `self.EnterUI`
  (params (Causer :type "Actor Object Reference"))
  (bind _returnvalue (`GameplayStatics.GetPlayerController` 0))
  ;[1 1 1] Press F 팝업 문구 제거
  (bind _returnvalue_2 (`|CreateWidget` "/Game/UI/InGame/Blueprint/04_CraftingUI/WB_UISkillSelect.WB_UISkillSelect_C" (`GameplayStatics.GetPlayerController` 0)))
  (bind _output_get (set `self.WB_UI_SkillSelect` _returnvalue_2))
  (`GameplayStatics.SetGlobalTimeDilation` 0.001)
  (`WidgetBlueprintLibrary.SetInputMode_UIOnlyEx` _returnvalue _output_get)
  (`/Game/UI/InGame/Blueprint/04_CraftingUI/WB_UISkillSelect.Initialize` _output_get)
  (`UserWidget.AddToViewport` _output_get 0)
  (set `PlayerController.bShowMouseCursor` true _returnvalue))

(fn `UserConstructionScript`
  (`SceneComponent.SetVisibility` (`self.TextRenderComp`) true false))