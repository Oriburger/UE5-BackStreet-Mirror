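; BP_SystemTest is an interactable debug actor for exercising the player's skill, inventory and weapon systems.
; Overlapping its volume toggles a "Press F" guide text, and EnterUI switches on ESystemCommand to run one test.
; The tests add and upgrade a skill, grant crafting items, or set upgraded weapon stats on the player character.
; Results are printed on screen, with the skill test cross-checking the manager's equipped, skill and inventory maps.
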(event `self.ReceiveBeginPlay`
  (`parent.ReceiveBeginPlay`))

(event `self.OverlapVolume.OnComponentBeginOverlap`
  (params (OverlappedComponent :type "PrimitiveComponent Object Reference") (OtherActor :type "Actor Object Reference") (OtherComp :type "PrimitiveComponent Object Reference") (OtherBodyIndex :type Integer) (bFromSweep :type Boolean) (SweepResult :type "HitResult Structure (by ref)"))
  ;[1 1 1] Press F 팝업 문구 호출
  (`self.VisibleGuideTextRender` OtherActor))

(event `self.OverlapVolume.OnComponentEndOverlap`
  (params (OverlappedComponent :type "PrimitiveComponent Object Reference") (OtherActor :type "Actor Object Reference") (OtherComp :type "PrimitiveComponent Object Reference") (OtherBodyIndex :type Integer))
  ;[1 1 1] Press F 팝업 문구 제거
  (`self.InVisibleGuideTextRender` OtherActor))

(event `self.EnterUI`
  (params (Causer :type "Actor Object Reference"))
  ;[1 1 1] Press F 팝업 문구 제거
  (switch `/Game/Map/Blueprint/ESystemCommand` (`self.ESystemCommand`)
    (:`NewEnumerator3`
      ;;[0.07532 0.7789 1] Skill Level 추가
      (`self.AddSkillLevel`))
    (:`NewEnumerator1`
      ;;[0.7985 0.4973 1] Item 추가
      (`self.AddCraftingItem`))
    (:`NewEnumerator2`
      ;;[0.8536 1 0.6873] WeaponStat추가
      (`self.AddWeaponStat`))))

(fn `AddCraftingItem`
  (bind _asbp_main_character (cast `/Game/Character/MainCharacter/BP_MainCharacter` (`GameplayStatics.GetPlayerCharacter` 0)))
  (bind _iteminventory (`MainCharacterBase.ItemInventory` _asbp_main_character))
  (`ItemInventoryComponent.AddItem` _iteminventory 1 6)
  (`ItemInventoryComponent.AddItem` _iteminventory 2 7)
  (`ItemInventoryComponent.AddItem` _iteminventory 3 5)
  (for _index (range 1 4)
    (bind _itemdata (`ItemInventoryComponent.GetItemData` _iteminventory _index))
    (bind ((`ItemName` _itemname) (`ItemAmount` _itemamount)) (break `ItemDataStruct` _itemdata))
    (`KismetSystemLibrary.PrintString` (`KismetStringLibrary.Concat_StrStr` "Name : " (`KismetStringLibrary.Conv_NameToString` _itemname) "Amount : " (`KismetStringLibrary.Conv_ByteToString` _itemamount)))))

(fn `AddSkillLevel`
  (bind _skillid_getskill_ (`self.SkillID(GetSkill)`))
  (bind _asmain_character_base (cast `MainCharacterBase` (`GameplayStatics.GetPlayerCharacter` 0)))
  (bind _skillmanagercomponent (`CharacterBase.SkillManagerComponent` _asmain_character_base))
  (`SkillManagerComponent.AddSkill` _skillmanagercomponent _skillid_getskill_)
  (`SkillManagerComponent.UpgradeSkill` _skillmanagercomponent _skillid_getskill_ 1)
  (bind ((`SkillType` _skilltype)) (break `SkillWeaponStruct` (`.SkillWeaponStruct` (break `SkillStatStruct` (`SkillManagerComponent.GetSkillInfo` _skillmanagercomponent _skillid_getskill_)))))
  (bind (_value _returnvalue) (`BlueprintMapLibrary.Map_Find` (`SkillManagerComponent.EquipedSkillMap` _skillmanagercomponent) _skilltype))
  ;[1 1 1] EquipedSkillMap확인
  (if _returnvalue
    (if (== _value _skillid_getskill_)
      (`KismetSystemLibrary.PrintString` "EquipedSkillMap(o)")
      ;[1 1 1] SkillMap확인
      (if (`SkillManagerComponent.IsSkillValid` _skillmanagercomponent _value)
        (`KismetSystemLibrary.PrintString` "SkillMap(o)")
        (bind (_value_2 _returnvalue_2) (`BlueprintMapLibrary.Map_Find` (`SkillManagerComponent.GetSkillInventoryMap` _skillmanagercomponent) _skilltype))
        ;[1 1 1] SkillInventoryMap(확인)
        (if _returnvalue_2
          (for _array_element (`.SkillBaseList` (break `SkillListContainer` _value_2))
            (if (== (`.SkillID` (break `SkillStatStruct` (`SkillBase.SkillStat` _array_element))) (`self.SkillID(GetSkill)`))
              (`KismetSystemLibrary.PrintString` "SkillInventoryMap(o)")
              (else
                (`KismetSystemLibrary.PrintString` "SkillInventoryMap(x)"))))
          (else
            (`KismetSystemLibrary.PrintString` "NoType")))
        (else
          (`KismetSystemLibrary.PrintString` "SkillMap(x)")))
      (else
        (`KismetSystemLibrary.PrintString` "EquipedSkillMap(x)")))
    (else
      (`KismetSystemLibrary.PrintString` "NoType"))))

(fn `AddWeaponStat`
  (locals (UpgradeStatList :type "Array of Byte"))
  (bind _upgradestatlist (`local.UpgradeStatList`))
  (bind _asbp_main_character (cast `/Game/Character/MainCharacter/BP_MainCharacter` (`GameplayStatics.GetPlayerCharacter` 0)))
  (bind _output_get (set `self.WeaponState` (struct)))
  (`KismetArrayLibrary.Array_Add` _upgradestatlist 1)
  (`KismetArrayLibrary.Array_Add` _upgradestatlist 2)
  (`KismetArrayLibrary.Array_Add` _upgradestatlist 3)
  (bind _structout (setmembers `WeaponStateStruct` :`StructRef` _output_get :`UpgradedStatList` _upgradestatlist))
  (`WeaponComponentBase.SetWeaponState` (`CharacterBase.WeaponComponent` _asbp_main_character) _structout)
  (bind ((`UpgradedStatList` _upgradedstatlist)) (break `WeaponStateStruct` _structout))
  (`KismetSystemLibrary.PrintString` (`KismetStringLibrary.Concat_StrStr` " \nAttack  ;" (`KismetStringLibrary.Conv_ByteToString` (`|GetArrayItem` _upgradedstatlist)) " \nSpeed : " (`KismetStringLibrary.Conv_ByteToString` (`|GetArrayItem` _upgradedstatlist 1)) " \nFinalImpact :" (`KismetStringLibrary.Conv_ByteToString` (`|GetArrayItem` _upgradedstatlist 2)))))

(fn `UserConstructionScript`
  (`SceneComponent.SetVisibility` (`self.TextRenderComp`) true false))