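; BP_SpawnPoint is a map marker for a spawn location that keeps a list of actors spawned at it.
; On BeginPlay it subscribes to the chapter manager's StageManagerComponent spawn event and adds actors appearing within a small tolerance of its position.
; A handler removes destroyed actors, but its binding is never executed.
; The construction script matches actor tags to set the text label and arrow color.
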(event `self.ReceiveBeginPlay`
  (bind _returnvalue (`/Game/UI/Global/BPFL_CommonWidget.GetChapterManagerRef`))
  ;[1 1 1] Begin Play
  (`/Engine/EditorBlueprintResources/StandardMacros.IsValid` _returnvalue
    (:`Is Valid`
      (add `StageManagerComponent.OnActorSpawned` (`NewChapterManagerBase.StageManagerComponent` _returnvalue) (delegate `OnActorSpawned`)))
    (:`Is Not Valid`
      (`KismetSystemLibrary.PrintString` "Error : Cannot find chapter manager" true true (struct :`R` 1.0 :`B` 0.006496 :`A` 1.0)))))

(event `OnActorSpawned`
  (params (SpawnLocation :type "Vector Structure") (NewActor :type "Actor Object Reference"))
  ;[1 1 1] 관련 액터 관리
  (if (== SpawnLocation (`self.K2_GetActorLocation`) :`ErrorTolerance` 76.0)
    (`/Engine/EditorBlueprintResources/StandardMacros.IsValid` NewActor
      (:`Is Valid`
        (`KismetArrayLibrary.Array_AddUnique` (`self.RelatedActorList`) NewActor)))))

(event `OnActorDestroyed`
  (params (DestroyedActor :type "Actor Object Reference"))
  ;[1 1 1] 관련 액터 관리
  (`KismetArrayLibrary.Array_RemoveItem` (`self.RelatedActorList`) DestroyedActor))

(fn `UserConstructionScript`
  (for (_array_element _array_index) (`self.Tag`)
    (if (`self.ActorHasTag` _array_element)
      (`TextRenderComponent.K2_SetText` (`self.TextRender`) (`KismetTextLibrary.Conv_NameToText` _array_element))
      (set `ArrowComponent.ArrowColor` (`|GetArrayItem` (`self.Color`) _array_index) (`self.Arrow`)))))