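; Road border actor for the Chapter01 map that lays spline mesh segments along an editable spline.
; The Construction Script adds one SplineMeshComponent per pair of neighboring spline points, using their local locations and tangents as start and end, then attaches it to DefaultSceneRoot.
; The event graph holds only empty placeholder events, so the actor has no runtime logic.
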(fn `UserConstructionScript`
  (bind _spline (`self.Spline`))
  (bind _spline_2 (`self.Spline`))
  (`/Engine/EditorBlueprintResources/StandardMacros.IsValid` _spline
    (:`Is Valid`
      (for _index (range (+ (- (`SplineComponent.GetNumberOfSplinePoints` _spline) 2) 1))
        (bind _returnvalue (`AddComponent|NODE_AddSplineMeshComponent-0`))
        (`/Engine/EditorBlueprintResources/StandardMacros.IsValid` _returnvalue
          (:`Is Valid`
            (bind (_location _tangent) (`SplineComponent.GetLocationAndTangentAtSplinePoint` _spline_2 _index "Local"))
            (bind (_location_2 _tangent_2) (`SplineComponent.GetLocationAndTangentAtSplinePoint` _spline_2 (+ _index 1) "Local"))
            (`SplineMeshComponent.SetStartAndEnd` _returnvalue _location _tangent _location_2 _tangent_2 true)
            (`SceneComponent.K2_AttachToComponent` _returnvalue (`self.DefaultSceneRoot`) "None" "KeepRelative" "KeepRelative" "KeepRelative" true)))))))