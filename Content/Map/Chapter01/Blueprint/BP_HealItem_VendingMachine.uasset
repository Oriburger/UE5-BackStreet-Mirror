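; Vending machine interactable that dispenses a physics-simulated heal pack once, in exchange for a required amount of inventory item 1.
; The interaction collision toggles a child actor's visibility by availability and triggers the inventory check.
; Success removes the items, spawns the pack and animates a dynamic light material, then disables interaction by teleporting the collision far below (marked temporary).
; Insufficient items plays an error sound and light timeline.
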(event `self.ReceiveBeginPlay`
  (bind _vendingmachine (`self.VendingMachine`))
  (bind _returnvalue (`PrimitiveComponent.CreateDynamicMaterialInstance` _vendingmachine 1 "/Game/Map/Chapter01/Material/M_Light_Inst.M_Light_Inst" "None"))
  (`PrimitiveComponent.SetMaterial` _vendingmachine 1 _returnvalue)
  (set `self.LightDynamicMaterial` _returnvalue)
  (`SceneComponent.SetVisibility` (`self.ChildActor`) false true))

(event `self.InteractiveCollision.OnInteractionAvailableStateUpdate`
  (params (bNewState :type Boolean))
  (`SceneComponent.SetVisibility` (`self.ChildActor`) bNewState true))

(event `self.InteractiveCollision.OnInteractionBegin`
  (bind _returnvalue__ (`/Game/UI/Global/BPFL_CommonWidget.GetMainCharacterRef`))
  (bind _requiredmaterialcount (`self.RequiredMaterialCount`))
  (bind _iteminventory (`MainCharacterBase.ItemInventory` _returnvalue__))
  (if (`self.bCanInteract`)
    (`/Engine/EditorBlueprintResources/StandardMacros.IsValid` _returnvalue__
      (:`Is Valid`
        (if (>= (`ItemInventoryComponent.GetItemAmount` _iteminventory 1) _requiredmaterialcount)
          (`/Engine/EditorBlueprintResources/StandardMacros.DoOnce` false
            (:`Completed`
              (`ItemInventoryComponent.RemoveItem` _iteminventory 1 (`KismetMathLibrary.Conv_IntToByte` _requiredmaterialcount))
              (`self.SpawnItem`)
              (bind (_direction `_새_트랙_0`) (`Timeline|타임라인` :!via `PlayFromStart`)
                (:`Update`
                  (`MaterialInstanceDynamic.SetVectorParameterValue` (`self.LightDynamicMaterial`) "LightColor" `_새_트랙_0`)
                  ;[1 1 1] Temp Logic
                  (set `self.bCanInteract` false)
                  (`SceneComponent.K2_SetRelativeLocation` (`self.InteractiveCollision`) (0.0 0.0 -50000.0) false true)))))
          (else
            (`GameplayStatics.PlaySound2D` "/Game/Sound/VendingMachine/SC_VendingMahcineError.SC_VendingMahcineError" 1.0 1.0 0.0 null null)
            (bind (_direction_2 `_새_트랙_0_2`) (`Timeline|ErrorVendingMachine` :!via `PlayFromStart`)
              (:`Update`
                (`MaterialInstanceDynamic.SetVectorParameterValue` (`self.LightDynamicMaterial`) "LightColor" `_새_트랙_0_2`)))))))))

(event `SpawnItem`
  (bind _returnvalue (`|SpawnActorFromClass` "/Game/Item/Blueprint/Item/BP_HealPackItem.BP_HealPackItem_C" (`SceneComponent.K2_GetComponentToWorld` (`self.SpawnPoint`)) "Undefined" "MultiplyWithRoot" null -1.0 true null))
  (`PrimitiveComponent.SetSimulatePhysics` (`ItemBase.MeshComponent` _returnvalue) true))

(fn `UserConstructionScript`)