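; Actor component that makes its owner saveable in the EasySaveGame system.
; It registers the owner with the game instance on BeginPlay and can report its destruction on EndPlay.
; SaveOrLoadVariables converts optional transform, custom variables via the LoadingOrSavingVariables dispatcher, and, for some save types, component settings to and from a JSON string.
; RequestLoadVariables lets eligible actors pull their data from BP_EasySaveGameOperationsManager once the world is initialized and idle.
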(event `RetriggerRegistration`
  (message `/Game/EasyGameUI/EasySaveGameUI/Core/BPI_EasySaveGameInterface.Register For Save Game` (`GameplayStatics.GetGameInstance`) (`self.OwnerActorRef`) (make `/Game/EasyGameUI/EasySaveGameUI/Datas/S_ActorSaveInfos` false (`|ConvertAsset` self) (`self.ActorClass`) (`self.ActorSaveType`) (`self.RespawnOrFindOnlyInSameLevel?`) (`self.ActorUniqueID`)) :!label _label))

(event `self.ReceiveBeginPlay`
  (bind _returnvalue (`self.GetOwner`))
  (set `self.OwnerActorRef` (`|ConvertAsset` _returnvalue))
  (set `self.ActorClass` (`|ConvertAsset` (`GameplayStatics.GetObjectClass` _returnvalue)))
  (goto _label))

(event `self.ReceiveEndPlay`
  (params (EndPlayReason :type "EEndPlayReason Enum" :default "Destroyed"))
  (bind _returnvalue (`GameplayStatics.GetGameInstance`))
  (bind _respawnorfindonlyinsamelevel_ (`self.RespawnOrFindOnlyInSameLevel?`))
  (bind _owneractorref (`self.OwnerActorRef`))
  (bind _actorclass (`self.ActorClass`))
  (bind _actorsavetype (`self.ActorSaveType`))
  (bind _output (`|ConvertAsset` self))
  (if (and (`|EnumEquality` EndPlayReason "Destroyed") (`self.RegisterDestruction?`))
    (if (and (`KismetStringLibrary.IsEmpty` (`self.ActorUniqueID`)) (`|EnumEquality` (`self.ActorSaveType`) "NewEnumerator3"))
      (message `/Game/EasyGameUI/EasySaveGameUI/Core/BPI_EasySaveGameInterface.Register For Save Game` _returnvalue _owneractorref (make `/Game/EasyGameUI/EasySaveGameUI/Datas/S_ActorSaveInfos` true _output _actorclass _actorsavetype _respawnorfindonlyinsamelevel_ (`KismetGuidLibrary.Conv_GuidToString` (`KismetGuidLibrary.NewGuid`))))
      (else
        (message `/Game/EasyGameUI/EasySaveGameUI/Core/BPI_EasySaveGameInterface.Register For Save Game` _returnvalue _owneractorref (make `/Game/EasyGameUI/EasySaveGameUI/Datas/S_ActorSaveInfos` true _output _actorclass _actorsavetype _respawnorfindonlyinsamelevel_ (`self.ActorUniqueID`)))))))

(fn `RequestLoadVariables`
  (if (and (`|EnumEquality` (`self.ActorSaveType`) "NewEnumerator0") (not (`self.RegisterDestruction?`)))
    (bind _returnvalue (`GameplayStatics.GetActorOfClass` "/Game/EasyGameUI/EasySaveGameUI/Core/BP_EasySaveGameOperationsManager.BP_EasySaveGameOperationsManager_C"))
    (if (and (`/Game/EasyGameUI/EasySaveGameUI/Core/BP_EasySaveGameOperationsManager.WorldInitialized?` _returnvalue) (not (`/Game/EasyGameUI/EasySaveGameUI/Core/BP_EasySaveGameOperationsManager.IsSavingOrLoading?` _returnvalue)))
      (`self.SaveOrLoadVariables` "NewEnumerator1" (`BlueprintMapLibrary.Map_Find` (`/Game/EasyGameUI/EasySaveGameUI/Core/BP_EasySaveGameOperationsManager.PersistentActors` _returnvalue) (`self.OwnerActorRef`))))))

(fn `SaveOrLoadVariables`
  (params (OperationType :type "/Game/EasyGameUI/EasySaveGameUI/Datas/E_SaveGameOperationType Enum" :default "NewEnumerator0") (SavedVariables :type String))
  (returns (ActorRef :type "Actor Soft Object Reference") (SavedVariablesOut :type String) (ActorUniqueID :type String))
  (bind _jsonobject (`self.JsonObject`))
  (switch `/Game/EasyGameUI/EasySaveGameUI/Datas/E_SaveGameOperationType` OperationType
    (:`NewEnumerator0`
      ;[1 0 0.243] Save Actor
      (bind _outjsonobject (`JsonBlueprintFunctionLibrary.FromString` ""))
      (set `self.JsonObject` _outjsonobject)
      (`|ExecutionSequence`
        (:`then_0`
          (if (`|EnumInequality` (`self.ActorSaveType`) "NewEnumerator0") :!label _label
            (bind _output_get (set `self.ComponentState` (`|MakeArray` (`self.RegisterDestruction?`) (`self.SaveTranform?`) (`self.HasVariablesToSave?`) (`self.RespawnOrFindOnlyInSameLevel?`))))
            (bind _loadedvalue (`/Game/EasyGameUI/Core/BML_EasyMacroUtilities.SaveOrLoadArrayVariable` (`local.OperationType`) (`self.JsonObject`) "Component State" _output_get)
              (:`Loaded`
                (set `self.RegisterDestruction?` (`|GetArrayItem` _loadedvalue))
                (set `self.SaveTranform?` (`|GetArrayItem` _loadedvalue 1))
                (set `self.HasVariablesToSave?` (`|GetArrayItem` _loadedvalue 2))
                (set `self.RespawnOrFindOnlyInSameLevel?` (`|GetArrayItem` _loadedvalue 3))
                (`self.RetriggerRegistration`)))))
        (:`then_1`
          (if (`self.HasVariablesToSave?`)
            (`self.LoadingOrSavingVariables` "NewEnumerator0" (`self.JsonObject`)))
          (if (`self.SaveTranform?`)
            (`|SetJsonField` _jsonobject "Transform" (`Actor.GetTransform` (`|ConvertAsset` (`self.OwnerActorRef`)))))
          (bind _outjsonstring (`JsonBlueprintFunctionLibrary.ToString` _jsonobject))
          (return (`self.OwnerActorRef`) _outjsonstring (`self.ActorUniqueID`)))))
    (:`NewEnumerator1`
      ;[0 1 0.1932] Load Actor
      (bind _outjsonobject_2 (`JsonBlueprintFunctionLibrary.FromString` (`local.SavedVariables`)))
      (set `self.JsonObject` _outjsonobject_2)
      (`|ExecutionSequence`
        (:`then_0`
          (goto _label))
        (:`then_1`
          (bind (_outvalue _returnvalue) (`|GetJsonField` (`self.JsonObject`) "Transform"))
          (if _returnvalue
            (`Actor.K2_SetActorTransform` (`|ConvertAsset` (`self.OwnerActorRef`)) _outvalue false false))
          (if (`self.HasVariablesToSave?`)
            (`self.LoadingOrSavingVariables` "NewEnumerator1" (`self.JsonObject`))))))))