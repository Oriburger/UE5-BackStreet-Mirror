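; BP_ESGU_ImportantSaveTrigger is a box trigger that starts a save game operation when the player character overlaps it.
; It requests an available slot for its SaveType and passes it to a GameInstance save message.
; With DisableAfterActivation, it turns off collision after firing and flags its save component as having variables to save.
; The component saves and restores the Activated flag, so a used trigger stays disabled after loading.
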(event `self.Box.OnComponentBeginOverlap`
  (params (OverlappedComponent :type "PrimitiveComponent Object Reference") (OtherActor :type "Actor Object Reference") (OtherComp :type "PrimitiveComponent Object Reference") (OtherBodyIndex :type Integer) (bFromSweep :type Boolean) (SweepResult :type "HitResult Structure (by ref)"))
  (if (and (== OtherActor (`GameplayStatics.GetPlayerCharacter` 0)) (not (`self.Activated?`)))
    (bind _saveuniquename (`/Game/EasyGameUI/EasySaveGameUI/Core/BFL_EasySaveGameFunctions.FindAvailableIndexForSaveType` (`self.SaveType`)))
    (message `/Game/EasyGameUI/EasySaveGameUI/Core/BPI_EasySaveGameInterface.StartSaveGameOperation` (`GameplayStatics.GetGameInstance`) (make `/Game/EasyGameUI/EasySaveGameUI/Datas/S_SaveOperationInfos` _saveuniquename) false)
    (if (`self.DisableAfterActivation?`)
      (set `self.Activated?` true)
      (`PrimitiveComponent.SetCollisionEnabled` (`self.Box`) "NoCollision"))))

(event `self.BP_EasySaveGameComponent.LoadingOrSavingVariables`
  (params (OperationType :type "/Game/EasyGameUI/EasySaveGameUI/Datas/E_SaveGameOperationType Enum" :default "NewEnumerator0") (JsonObject :type "JsonObjectWrapper Structure"))
  (bind _loadedvalue (`/Game/EasyGameUI/Core/BML_EasyMacroUtilities.SaveOrLoadVariable` OperationType JsonObject "Activation" (`self.Activated?`))
    (:`Loaded`
      (bind _output_get (set `self.Activated?` _loadedvalue))
      (if _output_get
        (`PrimitiveComponent.SetCollisionEnabled` (`self.Box`) "NoCollision")))))

(fn `UserConstructionScript`
  (set `/Game/EasyGameUI/EasySaveGameUI/Core/BP_EasySaveGameComponent.HasVariablesToSave?` (`self.DisableAfterActivation?`) (`self.BP_EasySaveGameComponent`)))