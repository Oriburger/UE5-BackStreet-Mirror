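; Demo actor for the Easy Save Game system that provides randomized state to save and load.
; BeginPlay randomizes its location, scale, cube rotation and material, plus a title and integer shown on a text render.
; The save component's LoadingOrSavingVariables event chains SaveOrLoadVariable calls that handle both directions through a JSON object, reapplying values on each Loaded branch.
; The construction script passes the actor's save type to the component.
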(event `self.BP_EasySaveGameComponent.LoadingOrSavingVariables`
  (params (OperationType :type "/Game/EasyGameUI/EasySaveGameUI/Datas/E_SaveGameOperationType Enum" :default "NewEnumerator0") (JsonObject :type "JsonObjectWrapper Structure"))
  (bind _cube (`self.Cube`))
  (bind _loadedvalue (`/Game/EasyGameUI/Core/BML_EasyMacroUtilities.SaveOrLoadVariable` OperationType JsonObject "Title" (`self.Title`))
    (:`Then`
      (bind _loadedvalue_2 (`/Game/EasyGameUI/Core/BML_EasyMacroUtilities.SaveOrLoadVariable` OperationType JsonObject "Int" (`self.IntegerVar`))
        (:`Then`
          (bind _loadedvalue_3 (`/Game/EasyGameUI/Core/BML_EasyMacroUtilities.SaveOrLoadVariable` OperationType JsonObject "Material" (`PrimitiveComponent.GetMaterial` (`self.Cube`) 0))
            (:`Then`
              (bind _loadedvalue_4 (`/Game/EasyGameUI/Core/BML_EasyMacroUtilities.SaveOrLoadVariable` OperationType JsonObject "Cube Rot" (`SceneComponent.RelativeRotation` _cube))
                (:`Loaded`
                  (`SceneComponent.K2_SetRelativeRotation` (`self.Cube`) _loadedvalue_4 false false))))
            (:`Loaded`
              (`PrimitiveComponent.SetMaterial` _cube 0 _loadedvalue_3))))
        (:`Loaded`
          (set `self.IntegerVar` _loadedvalue_2)
          (`TextRenderComponent.K2_SetText` (`self.TextRender`) (`|FormatText` "{Title} \n{ID}" (`self.Title`) (`KismetStringLibrary.Conv_IntToString` (`self.IntegerVar`)))))))
    (:`Loaded`
      (set `self.Title` _loadedvalue))))

(event `self.ReceiveBeginPlay`
  (bind _returnvalue (`KismetMathLibrary.RandomFloatInRange` 0.5 1.0))
  (bind _returnvalue_2 (`KismetMathLibrary.RandomFloatInRange` -50.0 50.0))
  (`self.K2_SetActorTransform` (`KismetMathLibrary.MakeTransform` (+ (`self.K2_GetActorLocation`) (`KismetMathLibrary.MakeVector` _returnvalue_2 _returnvalue_2 _returnvalue_2)) (`self.K2_GetActorRotation`) (`KismetMathLibrary.MakeVector` _returnvalue _returnvalue _returnvalue)))
  (`SceneComponent.K2_AddLocalRotation` (`self.Cube`) (`KismetMathLibrary.RandomRotator` true) false false)
  (set `self.Title` (`KismetStringLibrary.Concat_StrStr` "Item_" (`KismetStringLibrary.Conv_IntToString` (`KismetMathLibrary.RandomInteger` 9999))))
  (set `self.IntegerVar` (`KismetMathLibrary.RandomInteger` 99999999))
  (`TextRenderComponent.K2_SetText` (`self.TextRender`) (`|FormatText` "{Title} \n{ID}" (`self.Title`) (`KismetStringLibrary.Conv_IntToString` (`self.IntegerVar`))))
  (`PrimitiveComponent.SetMaterial` (`self.Cube`) 0 (`KismetArrayLibrary.Array_Random` (`|MakeArray` "/Game/EasyGameUI/DemoContent/Materials/M_MatMaterial.M_MatMaterial" "/Game/EasyGameUI/DemoContent/Materials/MI_MatMaterial_Green.MI_MatMaterial_Green" "/Game/EasyGameUI/DemoContent/Materials/MI_MatMaterial_Blue.MI_MatMaterial_Blue" "/Game/EasyGameUI/DemoContent/Materials/M_GlossyMaterial.M_GlossyMaterial" :!type "MaterialInterface Object Reference"))))

(fn `UserConstructionScript`
  (set `/Game/EasyGameUI/EasySaveGameUI/Core/BP_EasySaveGameComponent.ActorSaveType` (`self.ActorSaveType`) (`self.BP_EasySaveGameComponent`)))