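; World-placed actor that shows an input prompt, with key icons and text, through a widget component using WBP_EasyMultiInputPromptDisplayer.
; Construction script sets the widget space from DisplayType.
; BeginPlay configures the displayer from either an input action or key settings, taking icon size and text styling from CalculateFinalResolution.
; It then divides the component's world scale by ResolutionMultiplier, pairing with that resolution calculation for sharper rendering.
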(event `self.ReceiveBeginPlay`
  (bind _font_infos (`self.Font Infos`))
  (bind _resolutionmultiplier (`self.ResolutionMultiplier`))
  (bind _widget (`self.Widget`))
  (bind _aswbp_easy_multi_input_prompt_displayer (cast `/Game/EasyGameUI/EasyInputPrompts/Core/WBP_EasyMultiInputPromptDisplayer` (`WidgetComponent.GetWidget` (`self.Widget`))))
  (`/Game/EasyGameUI/EasyInputPrompts/Core/WBP_EasyMultiInputPromptDisplayer.SetupWidget` _aswbp_easy_multi_input_prompt_displayer (`self.Use Input Action?`) (`self.Input Action`) (`self.Input Mapping Context`) (`self.Gamepad Keys`) (`self.MNK Keys`) (* (`self.Key Image Size`) _resolutionmultiplier) (`self.Text To Display`) (`self.Text Position`) (`self.Text Padding`) (make `/Game/EasyGameUI/Datas/S_CommonTextInfo` (make `/Game/EasyGameUI/GraphicContent/Fonts/S_FontSelector` (break `/Game/EasyGameUI/GraphicContent/Fonts/S_FontSelector` (break `/Game/EasyGameUI/Datas/S_CommonTextInfo` _font_infos)) (`.Italic?_7_1AE77E7B48F1DCE50C0B58A663BD0DCA` (break `/Game/EasyGameUI/GraphicContent/Fonts/S_FontSelector` (break `/Game/EasyGameUI/Datas/S_CommonTextInfo` _font_infos))) (* (`.FontSize_8_B7A94D3A449B47D657AADAA82FE5E6C7` (break `/Game/EasyGameUI/GraphicContent/Fonts/S_FontSelector` (break `/Game/EasyGameUI/Datas/S_CommonTextInfo` _font_infos))) _resolutionmultiplier)) (`.TransformPolicy_6_8E3FCB2140778805833D3D9DE43DBAA1` (break `/Game/EasyGameUI/Datas/S_CommonTextInfo` _font_infos)) (`.TextJustification_8_A09C15E6474D13902A497EAD0351DB00` (break `/Game/EasyGameUI/Datas/S_CommonTextInfo` _font_infos))) (`self.Spacing`) (`self.Hide Key For Other Devices?`) (`self.HideTextAsWell?`) (`self.Use Styling Local Override?`) (`self.Text Color`) (`self.Icon Color`))
  (`SceneComponent.SetWorldScale3D` _widget (/ (`SceneComponent.K2_GetComponentScale` _widget) (`self.ResolutionMultiplier`))))

(fn `UserConstructionScript`
  (`WidgetComponent.SetWidgetSpace` (`self.Widget`) (`self.DisplayType`)))