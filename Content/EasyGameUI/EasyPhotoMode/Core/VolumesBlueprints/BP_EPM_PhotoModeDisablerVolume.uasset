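; Volume actor that blocks photo mode spawning for a character inside its box.
; On overlap, it finds the EGUI controller component on the actor's instigator controller, clears CanSpawnPhotoMode and caches both actor and component.
; Shortly after BeginPlay it applies the same check to characters already inside.
; When the cached actor leaves, spawning is re-enabled; only the last qualifying actor is tracked.
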(event `self.ReceiveBeginPlay`
  (`KismetSystemLibrary.Delay` 0.2)
  (for _array_element (`PrimitiveComponent.GetOverlappingActors` (`self.Box`) "/Script/Engine.Character")
    (`self.SetVariablesAndDisablePhotoMode` _array_element)))

(event `self.Box.OnComponentBeginOverlap`
  (params (OverlappedComponent :type "PrimitiveComponent Object Reference") (OtherActor :type "Actor Object Reference") (OtherComp :type "PrimitiveComponent Object Reference") (OtherBodyIndex :type Integer) (bFromSweep :type Boolean) (SweepResult :type "HitResult Structure (by ref)"))
  (`self.SetVariablesAndDisablePhotoMode` OtherActor))

(event `self.Box.OnComponentEndOverlap`
  (params (OverlappedComponent :type "PrimitiveComponent Object Reference") (OtherActor :type "Actor Object Reference") (OtherComp :type "PrimitiveComponent Object Reference") (OtherBodyIndex :type Integer))
  (if (== OtherActor (`self.OverlappedActor`))
    (set `/Game/EasyGameUI/Core/BP_EGUI_ControllerComponent.CanSpawnPhotoMode?` true (`self.OverlappedController`))))

(fn `SetVariablesAndDisablePhotoMode`
  (params (InActor :type "Actor Object Reference"))
  (bind _returnvalue (`self.GetComponentByClass` (`self.GetInstigatorController` InActor) "/Game/EasyGameUI/Core/BP_EGUI_ControllerComponent.BP_EGUI_ControllerComponent_C"))
  (`/Engine/EditorBlueprintResources/StandardMacros.IsValid` _returnvalue
    (:`Is Valid`
      (bind _output_get (set `self.OverlappedController` _returnvalue))
      (set `/Game/EasyGameUI/Core/BP_EGUI_ControllerComponent.CanSpawnPhotoMode?` false _output_get)
      (set `self.OverlappedActor` (`local.InActor`)))))

(fn `UserConstructionScript`)