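; Boss skill manager, owned by a CharacterBase, that spawns pillars, attaches them to the boss and fires them in sequence.
; BeginPlay caches the owner and every BP_PillarSpawnPoint in the level; SpawnPillar triggers those points and collects their pillars.
; AttachtoBoss attaches each pillar to the owner.
; ShootPillar derives an interval from total duration and pillar count, then a looping timer shoots one pillar per tick until the list is exhausted.
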(event `self.ReceiveBeginPlay`
  (bind _ascharacter_base (cast `CharacterBase` (`self.GetOwner`)))
  (set `self.CharacterRef` _ascharacter_base)
  (bind _outactors (`GameplayStatics.GetAllActorsOfClass` "/Game/System/SkillManager/Blueprint/Actor/BP_PillarSpawnPoint.BP_PillarSpawnPoint_C"))
  (set `self.PillarSpawnPoint` _outactors))

(event `SpawnPillar`
  (bind _pillarspawnpoint (`self.PillarSpawnPoint`))
  (for _array_element _pillarspawnpoint
    (`/Game/System/SkillManager/Blueprint/Actor/BP_PillarSpawnPoint.Spawn` _array_element))
  (for _array_element_2 _pillarspawnpoint
    (`KismetArrayLibrary.Array_Add` (`self.Pillar`) (`/Game/System/SkillManager/Blueprint/Actor/BP_PillarSpawnPoint.Pillar` _array_element_2))))

(event `Attach to Boss`
  (for _array_element (`self.Pillar`)
    (`/Game/System/SkillManager/Blueprint/Actor/BP_Pillar.Attach to boss` _array_element (`self.CharacterRef`))))

(event `ShootPillar`
  (params (TotalDulationTime :type "Float (double-precision)"))
  (bind _delaytime (`self. CalculateShootDelayTime` TotalDulationTime))
  (bind _output_get (set `self.ShootIntervalTime` _delaytime))
  (bind _returnvalue (`KismetSystemLibrary.K2_SetTimerDelegate` (delegate `ShootWithIntervalTime`) _output_get true))
  (set `self.ShootIntervalTimehandler` _returnvalue))

(event `ShootWithIntervalTime`
  (bind _pillaridx (`self.Pillaridx`))
  (if (not (< (`self.Pillaridx`) (`KismetArrayLibrary.Array_Length` (`self.Pillar`))))
    (`KismetSystemLibrary.K2_ClearAndInvalidateTimerHandle` (`self.ShootIntervalTimehandler`))
    (else
      (`/Game/System/SkillManager/Blueprint/Actor/BP_Pillar.Shoot` (`|GetArrayItem` (`self.Pillar`) _pillaridx))
      (`/Engine/EditorBlueprintResources/StandardMacros.IncrementInt` _pillaridx))))

(event `커스텀이벤트`)

(fn ` CalculateShootDelayTime`
  (params (TotalDurationTime :type "Float (double-precision)"))
  (returns (DelayTime :type "Float (double-precision)"))
  (locals (ShootDelayTime :type "Float (double-precision)"))
  (bind _returnvalue (`KismetArrayLibrary.Array_Length` (`self.Pillar`)))
  (if (> _returnvalue 2)
    (set `local.ShootDelayTime` (`KismetMathLibrary.SafeDivide` TotalDurationTime (`KismetMathLibrary.Conv_IntToDouble` (- _returnvalue 1))))
    (return (`local.ShootDelayTime`))
    (elif (== _returnvalue 2)
      (set `local.ShootDelayTime` TotalDurationTime)
      (return (`local.ShootDelayTime`))
      (elif (<= _returnvalue 1)
        (return (`local.ShootDelayTime`))))))