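; Pillar actor used as a boss skill projectile: the boss lifts it above itself, aims it and hurls it at the player.
; Attachtoboss starts looping timers that interp the spinning pillar to a random offset over the owner, then turn pillar and boss toward the player with a timeline float.
; Shoot interps it to the player's captured position, ending with camera shake and impact sound.
; Overlap deals damage and knockback only while shooting.
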(event `InitializePillar`
  (params (OwnerCharacterRef :type "CharacterBase Object Reference"))
  ;[1 1 1 1 30] InitializePillar
  (set `self.Owner Character Ref` OwnerCharacterRef)
  (set `self.SpawnLocation` (`self.K2_GetActorLocation`)))

(event `self.boxCollision.OnComponentBeginOverlap`
  (params (OverlappedComponent :type "PrimitiveComponent Object Reference") (OtherActor :type "Actor Object Reference") (OtherComp :type "PrimitiveComponent Object Reference") (OtherBodyIndex :type Integer) (bFromSweep :type Boolean) (SweepResult :type "HitResult Structure (by ref)"))
  (bind _returnvalue (`GameplayStatics.GetPlayerCharacter` 0))
  (bind _owner_character_ref (`self.Owner Character Ref`))
  ;[1 0.2292 0.2292 1 30] Overlap시 데미지 주기
  (`/Engine/EditorBlueprintResources/StandardMacros.IsValid` OverlappedComponent
    (:`Is Valid`
      (if (== OtherActor (`GameplayStatics.GetPlayerCharacter` 0))
        (if (`self.IsShoot`)
          (`PrimitiveComponent.SetCollisionEnabled` (`self.pillar`) "NoCollision")
          (bind _asmain_character_base (cast `MainCharacterBase` _returnvalue))
          (`CharacterBase.ApplyKnockBack` _owner_character_ref _asmain_character_base 5000.0)
          (`GameplayStatics.ApplyDamage` _returnvalue 250.0 null _owner_character_ref "/Script/Engine.DamageType"))))))

(event `Attach to boss`
  ;[0.5914 1 0.576 1 30] Attach to Boss 이벤트 호출시(BPS_ShootPillar에서) Set timer를 통해 보스 위로 Pillar들 interp, 플레이어(Boxman)을 향해 Rinterp과 TimeLine을 이용한 Floating 효과
  (`/Engine/EditorBlueprintResources/StandardMacros.IsValid` (`self.Owner Character Ref`)
    (:`Is Valid`
      (bind _returnvalue (`KismetSystemLibrary.K2_SetTimerDelegate` (delegate `UpdateLocation`) 0.01 true))
      (set `self.UpdateLocationTimerHandle` _returnvalue)
      (bind _returnvalue_2 (`|AddComponentByClass` :`self` self :`Class` "/Script/Engine.AudioComponent"))
      (`AudioComponent.SetSound` _returnvalue_2 "/Game/System/SkillManager/Sound/SC_BossShootSkill_Start.SC_BossShootSkill_Start")
      (`AudioComponent.Play` _returnvalue_2 0.0))))

(event `UpdateLocation`
  (bind _returnvalue (`self.K2_GetActorLocation`))
  (bind _returnvalue_2 (`KismetMathLibrary.RandomFloatInRange` 1.0 3.0))
  (bind _owner_character_ref (`self.Owner Character Ref`))
  (bind _returnvalue_3 (+ (`self.K2_GetActorLocation` (`self.Owner Character Ref`)) (`KismetMathLibrary.MakeVector` (`KismetMathLibrary.RandomFloatInRange` -200.0 200.0) (`KismetMathLibrary.RandomFloatInRange` -200.0 200.0) (`KismetMathLibrary.RandomFloatInRange` 600.0 700.0))))
  ;[0.5914 1 0.576 1 30] Attach to Boss 이벤트 호출시(BPS_ShootPillar에서) Set timer를 통해 보스 위로 Pillar들 interp, 플레이어(Boxman)을 향해 Rinterp과 TimeLine을 이용한 Floating 효과
  (if (`CharacterBase.GetIsActionActive` _owner_character_ref "E_Idle")
    (`CharacterBase.SetActionState` _owner_character_ref "E_Skill"))
  (if (== _returnvalue _returnvalue_3 :`ErrorTolerance` (`self.tolerance`))
    (`KismetSystemLibrary.K2_ClearAndInvalidateTimerHandle` (`self.UpdateLocationTimerHandle`))
    (bind _returnvalue_4 (`KismetSystemLibrary.K2_SetTimerDelegate` (delegate `UpdateRotate`) 0.01 true))
    (set `self.UpdateRotateTimeHandle` _returnvalue_4)
    (else
      (`self.K2_SetActorLocation` (`KismetMathLibrary.VInterpTo` _returnvalue _returnvalue_3 0.01 (`self.Interp Speed`)))
      (`self.K2_AddActorWorldRotation` (`KismetMathLibrary.MakeRotator` _returnvalue_2 _returnvalue_2 _returnvalue_2)))))

(event `UpdateRotate`
  (bind _owner_character_ref (`self.Owner Character Ref`))
  ;[0.5914 1 0.576 1 30] Attach to Boss 이벤트 호출시(BPS_ShootPillar에서) Set timer를 통해 보스 위로 Pillar들 interp, 플레이어(Boxman)을 향해 Rinterp과 TimeLine을 이용한 Floating 효과
  (`self.K2_SetActorRotation` (`KismetMathLibrary.RInterpTo` (`self.K2_GetActorRotation`) (`KismetMathLibrary.FindLookAtRotation` (`self.K2_GetActorLocation`) (`self.K2_GetActorLocation` (`GameplayStatics.GetPlayerCharacter` 0))) 0.01 6.0))
  (`/Engine/EditorBlueprintResources/StandardMacros.IsValid` _owner_character_ref
    (:`Is Valid`
      (`self.K2_SetActorRotation` _owner_character_ref (`KismetMathLibrary.RInterpTo` (`self.K2_GetActorRotation` _owner_character_ref) (`KismetMathLibrary.FindLookAtRotation` (`self.K2_GetActorLocation` _owner_character_ref) (`self.K2_GetActorLocation` (`GameplayStatics.GetPlayerCharacter` 0))) 0.01 6.0) false)
      (bind (_direction _floating) (`Timeline|FloatingTimeLine` :!label _label)
        (:`Update`
          (`self.K2_AddActorWorldOffset` (`KismetMathLibrary.MakeVector` 0.0 0.0 _floating)))))))

(event `Shoot`
  (bind (_returnvalue_x _returnvalue_y) (`KismetMathLibrary.BreakVector` (`self.K2_GetActorLocation` (`GameplayStatics.GetPlayerCharacter` 0))))
  (bind (_returnvalue_x_2 _returnvalue_y_2 _returnvalue_z) (`KismetMathLibrary.BreakVector` (`self.K2_GetActorLocation` (`self.Owner Character Ref`))))
  ;[0.4475 0.5927 1 1 30] Shoot 이벤트 호출 시( BPS_ShootPillar ) 플레이어를 향해 Shoot, 카메라 Shake효과, 플레이어 Overlap시 꺼줬던 Collision 다시 켜주기
  ; Is Shoot 변수를 통해 Shoot인 상태에서만 플레이어 overlap시 데미지 주고, Shoot이 아닌 맵에 배치된 상태에서는 overlap시 데미지 X
  (set `self.IsShoot` true)
  (set `self.ShootLocation` (`KismetMathLibrary.MakeVector` _returnvalue_x _returnvalue_y (- _returnvalue_z 60.0)))
  (bind _returnvalue (`KismetSystemLibrary.K2_SetTimerDelegate` (delegate `UpdateShoot`) 0.01 true))
  (`KismetSystemLibrary.K2_ClearAndInvalidateTimerHandle` (`self.UpdateRotateTimeHandle`))
  (set `self.UpdateShootTimeHandle` _returnvalue)
  (`|ExecutionSequence`
    (:`then_0`
      (goto _label :!via `Stop`))
    (:`then_1`
      (`AudioComponent.Stop` (stale `Attach to boss` _returnvalue_2))
      (`AudioComponent.SetSound` (stale `Attach to boss` _returnvalue_2) "/Game/System/SkillManager/Sound/SC_BossShootSkill_Middle2.SC_BossShootSkill_Middle2")
      (`AudioComponent.Play` (stale `Attach to boss` _returnvalue_2) 0.0))))

(event `UpdateShoot`
  (bind _returnvalue (`self.K2_GetActorLocation`))
  (bind _pillar (`self.pillar`))
  (bind _returnvalue_2 (+ (`self.ShootLocation`) (* (`self.GetActorForwardVector` (`GameplayStatics.GetPlayerCharacter` 0)) 35.0)))
  ;[0.4475 0.5927 1 1 30] Shoot 이벤트 호출 시( BPS_ShootPillar ) 플레이어를 향해 Shoot, 카메라 Shake효과, 플레이어 Overlap시 꺼줬던 Collision 다시 켜주기
  ; Is Shoot 변수를 통해 Shoot인 상태에서만 플레이어 overlap시 데미지 주고, Shoot이 아닌 맵에 배치된 상태에서는 overlap시 데미지 X
  (if (== _returnvalue _returnvalue_2 :`ErrorTolerance` 1.0)
    (`KismetSystemLibrary.K2_ClearAndInvalidateTimerHandle` (`self.UpdateShootTimeHandle`))
    (set `self.IsShoot` false)
    (bind _asbp_back_street_game_mode (cast `/Game/BP_BackStreetGameMode` (`GameplayStatics.GetGameMode`)))
    (`BackStreetGameModeBase.PlayCameraShakeEffect` _asbp_back_street_game_mode "E_Hit" (`self.K2_GetActorLocation`) 500.0)
    ;;[1 1 1] 사운드 플레이
    (`ActorComponent.K2_DestroyComponent` (stale `Attach to boss` _returnvalue_2))
    (bind _asbp_back_street_game_mode_2 (cast `/Game/BP_BackStreetGameMode` (`GameplayStatics.GetGameMode`)))
    (bind _returnvalue_3 (`BackStreetGameModeBase.GetGlobalAssetManagerBaseRef` _asbp_back_street_game_mode_2))
    (`/Engine/EditorBlueprintResources/StandardMacros.IsValid` _returnvalue_3
      (:`Is Valid`
        (`AssetManagerBase.PlaySingleSound` _returnvalue_3 self "E_Prop" 1002 "PillarHit" 2.0 1.0 0.0)
        (if (`|EnumEquality` (`PrimitiveComponent.GetCollisionEnabled` _pillar) "NoCollision")
          (`PrimitiveComponent.SetCollisionEnabled` _pillar "QueryAndPhysics"))))
    (else
      (`self.K2_SetActorLocation` (`KismetMathLibrary.VInterpTo` _returnvalue _returnvalue_2 0.01 12.0)))))

(fn `GetSoundAsset`
  (params (SoundType :type "ESoundAssetType Enum" :default "E_None") (SoundID :type Integer) (SoundName :type Name))
  (returns (Output :type "SoundCue Object Reference"))
  (bind _asbp_back_street_game_mode (cast `/Game/BP_BackStreetGameMode` (`GameplayStatics.GetGameMode`)))
  (bind _returnvalue (`BackStreetGameModeBase.GetGlobalAssetManagerBaseRef` _asbp_back_street_game_mode))
  (`/Engine/EditorBlueprintResources/StandardMacros.IsValid` _returnvalue
    (:`Is Valid`
      (bind _returnvalue_2 (`AssetManagerBase.GetSoundList` _returnvalue SoundType SoundID SoundName))
      (if (`KismetArrayLibrary.Array_IsValidIndex` _returnvalue_2)
        (return (`|GetArrayItem` _returnvalue_2))))))

(fn `UserConstructionScript`)