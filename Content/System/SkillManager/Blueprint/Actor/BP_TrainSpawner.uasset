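; BP_TrainSpawner is an actor that spawns timed waves of BP_Train actors along spline paths.
; On BeginPlay it waits briefly, then caches the level's BP_TrainSplinePath.
; SpawnTrain creates trains at the spawner's location, assigning each the path, a spline index and speed before calling Start.
; Pattern scripts staggered waves by number, with only pattern 1 defined; leftover test sequences are disconnected.
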(event `self.ReceiveBeginPlay`
  (`KismetSystemLibrary.Delay` 2.0)
  (bind _returnvalue (`GameplayStatics.GetActorOfClass` "/Game/System/SkillManager/Blueprint/Actor/BP_TrainSplinePath.BP_TrainSplinePath_C"))
  (set `self.Spline` _returnvalue))

(event `Spawn Train`
  (params (SpawnNum :type Integer) (SplineID :type "Array of Integer") (Speed :type "Float (double-precision)"))
  (for _index (range SpawnNum)
    (bind _returnvalue (`|SpawnActorFromClass` "/Game/System/SkillManager/Blueprint/Actor/BP_Train.BP_Train_C" (`KismetMathLibrary.MakeTransform` (`self.K2_GetActorLocation`)) "Undefined" "MultiplyWithRoot" null null))
    (set `/Game/System/SkillManager/Blueprint/Actor/BP_Train.SplinePath` (`self.Spline`) _returnvalue)
    (set `/Game/System/SkillManager/Blueprint/Actor/BP_Train.SplineID` (`|GetArrayItem` SplineID _index) _returnvalue)
    (set `/Game/System/SkillManager/Blueprint/Actor/BP_Train.Speed` Speed _returnvalue)
    (`/Game/System/SkillManager/Blueprint/Actor/BP_Train.Start` _returnvalue)))

(event `Pattern`
  (params (`Pattern Num` :type Integer))
  (if (== `Pattern Num` 1)
    (`self.Spawn Train` 1 (`|MakeArray` 0) 4000.0)
    (`KismetSystemLibrary.Delay` 0.1)
    (`self.Spawn Train` 1 (`|MakeArray` 1) 4000.0)
    (`KismetSystemLibrary.Delay` 1.0)
    (`self.Spawn Train` 2 (`|MakeArray` 2 3) 3500.0)))

(fn `UserConstructionScript`)