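; Pillar actor that stuns the boss when it runs into the pillar's box collision during a skill.
; On overlap with an exact BP_BossEnemy actor, it stores the boss and, if its action state is Skill, tries to add a short stun debuff.
; Debug prints mark the outcomes; the Attachtoboss event only prints, and the collision toggle nodes are unconnected.
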(event `self.BoxCollision.OnComponentBeginOverlap`
  (params (OverlappedComponent :type "PrimitiveComponent Object Reference") (OtherActor :type "Actor Object Reference") (OtherComp :type "PrimitiveComponent Object Reference") (OtherBodyIndex :type Integer) (bFromSweep :type Boolean) (SweepResult :type "HitResult Structure (by ref)"))
  (`/Engine/EditorBlueprintResources/StandardMacros.IsValid` OverlappedComponent
    (:`Is Valid`
      (if (== (`GameplayStatics.GetObjectClass` OtherActor) "/Game/Character/EnemyCharacter/Blueprint/BP_BossEnemy.BP_BossEnemy_C")
        (`/Engine/EditorBlueprintResources/StandardMacros.IsValid` OtherActor
          (:`Is Valid`
            (bind _asenemy_character_base (cast `EnemyCharacterBase` OtherActor)
              (:`then`
                (set `self.Boss` _asenemy_character_base)
                (if (`|EnumEquality` (`.CharacterActionState` (break `CharacterStateStruct` (`CharacterBase.CharacterState` _asenemy_character_base))) "E_Skill")
                  (bind _returnvalue (`CharacterBase.TryAddNewDebuff` (`self.Boss`) (make `DebuffInfoStruct` "E_Stun" 2.0) null))
                  (if _returnvalue
                    (`KismetSystemLibrary.PrintString` "Hello")
                    (else
                      (`KismetSystemLibrary.PrintString` "Hello")))
                  (else
                    (`KismetSystemLibrary.PrintString` "Not Active Skill"))))
              (:`CastFailed`
                (`KismetSystemLibrary.PrintString` "Cast Failed")))))))))

(event `Attach to boss`
  (`KismetSystemLibrary.PrintString` "attach to boss"))

(fn `UserConstructionScript`)