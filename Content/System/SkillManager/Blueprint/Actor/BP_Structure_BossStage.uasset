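; Breakable boss-stage structure that punishes a boss crashing into it during a skill, such as a charge.
; CrashBox overlap resets the boss's location-interp timer, deals damage, shakes the camera, applies a stun and plays its sound.
; A boss crash or BP_Pillar overlap briefly spawns a BP_MasterField to break the structure.
; It then swaps to dynamic chaos-pillar materials, animates opacity on a timeline and destroys itself.
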(event `self.CrashBox.OnComponentBeginOverlap`
  (params (OverlappedComponent :type "PrimitiveComponent Object Reference") (OtherActor :type "Actor Object Reference") (OtherComp :type "PrimitiveComponent Object Reference") (OtherBodyIndex :type Integer) (bFromSweep :type Boolean) (SweepResult :type "HitResult Structure (by ref)"))
  (bind (_returnvalue_x _returnvalue_y _returnvalue_z) (`KismetMathLibrary.BreakVector` (`self.K2_GetActorLocation` OtherActor)))
  (bind (_returnvalue_x_2 _returnvalue_y_2) (`KismetMathLibrary.BreakVector` (`SceneComponent.K2_GetComponentLocation` (`self.DestroyPoint`))))
  ;[1 0.8738 0.5796 1 30] Overlap시 보스인지 체크, Action State가 Skill인지 체크, 모두 True이면 Set Location with Interp함수(BPS_Charge 스킬에서 사용)의 Timer Reset, 데미지 주기 -> 카메라 shake효과 -> Stun주기
  (`/Engine/EditorBlueprintResources/StandardMacros.IsValid` OverlappedComponent
    (:`Is Valid`
      (if (== (`GameplayStatics.GetObjectClass` OtherActor) null)
        (`/Engine/EditorBlueprintResources/StandardMacros.IsValid` null
          (:`Is Valid`
            (bind _asenemy_character_base (cast `EnemyCharacterBase` OtherActor))
            (bind _output_get (set `self.boss` _asenemy_character_base))
            (if (`CharacterBase.GetIsActionActive` _asenemy_character_base "E_Skill")
              (`CharacterBase.ResetLocationInterpTimer` _output_get)
              (`GameplayStatics.ApplyDamage` _output_get 50.0 null self "/Script/Engine.DamageType")
              (bind _returnvalue (`|SpawnActorFromClass` "/Game/System/Chaos/Blueprint/BP_MasterField.BP_MasterField_C" (`KismetMathLibrary.MakeTransform` (`SceneComponent.K2_GetComponentLocation` (`self.DestroyPoint`)) (struct) (0.5 0.5 0.5)) "Undefined" "MultiplyWithRoot" null null))
              (`GeometryCollectionComponent.SetEnableDamageFromCollision` (`self.Cube`) false)
              (bind _asbp_back_street_game_mode (cast `/Game/BP_BackStreetGameMode` (`GameplayStatics.GetGameMode`)))
              (`BackStreetGameModeBase.PlayCameraShakeEffect` _asbp_back_street_game_mode "E_Hit" (`self.K2_GetActorLocation`) 750.0)
              (`CharacterBase.TryAddNewDebuff` (`self.boss`) (make `DebuffInfoStruct` "E_Stun" 4.0) null)
              ;[0.7969 0.7562 1] Play Single Sound(Boss Stun Sound) and Destroy BP_MasterField
              (bind _asbp_back_street_game_mode_2 (cast `/Game/BP_BackStreetGameMode` (`GameplayStatics.GetGameMode`)))
              (bind _returnvalue_2 (`BackStreetGameModeBase.GetGlobalAssetManagerBaseRef` _asbp_back_street_game_mode_2))
              (`/Engine/EditorBlueprintResources/StandardMacros.IsValid` _returnvalue_2
                (:`Is Valid`
                  (`AssetManagerBase.PlaySingleSound` _returnvalue_2 self "E_Prop" 1001 "BossStun" 2.0 1.0 0.0)
                  (`self.Destroy with Fade Out`)
                  (`KismetSystemLibrary.Delay` 0.2)
                  (`self.K2_DestroyActor` _returnvalue))))))
        (elif (== (`GameplayStatics.GetObjectClass` OtherActor) "/Game/System/SkillManager/Blueprint/Actor/BP_Pillar.BP_Pillar_C")
          (`/Engine/EditorBlueprintResources/StandardMacros.DoOnce` false
            (:`Completed`
              (bind _returnvalue_3 (`|SpawnActorFromClass` "/Game/System/Chaos/Blueprint/BP_MasterField.BP_MasterField_C" (`KismetMathLibrary.MakeTransform` (`KismetMathLibrary.MakeVector` _returnvalue_x_2 _returnvalue_y_2 _returnvalue_z) (struct) (0.5 0.5 0.5)) "Undefined" "MultiplyWithRoot" null null))
              (`GeometryCollectionComponent.SetEnableDamageFromCollision` (`self.Cube`) false)
              (`self.Destroy with Fade Out`)
              (`KismetSystemLibrary.Delay` 0.2)
              (`self.K2_DestroyActor` _returnvalue_3))))))))

(event `Destroy with Fade Out`
  (bind _cube (`self.cube`))
  ;[1 0.602 0.9146] Destroy with Fade Out
  (bind _returnvalue (`PrimitiveComponent.CreateDynamicMaterialInstance` _cube 0 "/Game/System/Chaos/Material/M_Pillar_Chaos.M_Pillar_Chaos" "None"))
  (`PrimitiveComponent.SetMaterial` _cube 0 _returnvalue)
  (bind _returnvalue_2 (`PrimitiveComponent.CreateDynamicMaterialInstance` _cube 1 "/Game/System/Chaos/Material/M_Pillar_Chaos.M_Pillar_Chaos" "None"))
  (`PrimitiveComponent.SetMaterial` _cube 1 _returnvalue_2)
  (`KismetSystemLibrary.Delay` 2.0)
  (bind (_direction _opacity) (`Timeline|타임라인`)
    (:`Update`
      (`MaterialInstanceDynamic.SetScalarParameterValue` _returnvalue "Opacity" _opacity)
      (`MaterialInstanceDynamic.SetScalarParameterValue` _returnvalue_2 "Opacity" _opacity)
      (if (>= _opacity 1.0)
        (`self.K2_DestroyActor`)))))

(fn `UserConstructionScript`)