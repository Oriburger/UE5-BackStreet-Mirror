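; BP_TrashSpawnPoint is a spawn point that creates and replaces BP_TrashWeapon projectiles for its owning character, used by the Chapter 2 boss.
; Initialize stores the owner and index, spawns a weapon at the point's location, links it back as Spawner, and initializes it from projectile stat and asset data tables by ProjectileID.
; SpawnTrash removes the passed weapon from the boss's list, spawns a replacement the same way, and registers it with the boss.
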(event `Initialize`
  (params (`Owner Character` :type "CharacterBase Object Reference") (TrashIndex :type Integer))
  (bind _projectile_id (`self.Projectile ID`))
  (bind _returnvalue (`KismetStringLibrary.Conv_StringToName` (`KismetStringLibrary.Conv_IntToString` _projectile_id)))
  (set `self.Owner Character` `Owner Character`)
  (set `self.TrashIndex` TrashIndex)
  (bind _returnvalue_2 (`|SpawnActorFromClass` "/Game/System/SkillManager/Blueprint/Actor/BP_TrashWeapon.BP_TrashWeapon_C" (`KismetMathLibrary.MakeTransform` (`self.K2_GetActorLocation` self)) "Undefined" "MultiplyWithRoot" null null))
  (bind _output_get (set `self.Trash Ref` _returnvalue_2))
  (set `/Game/System/SkillManager/Blueprint/Actor/BP_TrashWeapon.Projectile ID` _projectile_id _output_get)
  (set `/Game/System/SkillManager/Blueprint/Actor/BP_TrashWeapon.spawner` self _output_get)
  (bind _returnvalue_3 (`|GetDataTableRow` "/Game/Weapon/Data/D_ProjectileStatTable.D_ProjectileStatTable" _returnvalue)
    (:`then`
      (bind _returnvalue_4 (`|GetDataTableRow` "/Game/Weapon/Data/D_ProjectileAssetInfo.D_ProjectileAssetInfo" _returnvalue)
        (:`then`
          (`ProjectileBase.InitProjectile` _returnvalue_2 (`self.Owner Character`) _returnvalue_4 _returnvalue_3))))))

(event `Spawn Trash`
  (params (`Trash Ref` :type "/Game/System/SkillManager/Blueprint/Actor/BP_TrashWeapon Object Reference"))
  (bind _projectile_id (`self.Projectile ID`))
  (bind _owner_character (`self.Owner Character`))
  (bind _trash_ref (`self.Trash Ref`))
  (bind _returnvalue (`KismetStringLibrary.Conv_StringToName` (`KismetStringLibrary.Conv_IntToString` _projectile_id)))
  (bind _asbp_boss_chapter_2 (cast `/Game/Character/EnemyCharacter/Blueprint/BP_Boss_Chapter2` (`self.Owner Character`)))
  (`/Game/Character/EnemyCharacter/Blueprint/BP_Boss_Chapter2.Remove Trash Weapon` _asbp_boss_chapter_2 `Trash Ref`)
  (bind _returnvalue_2 (`|SpawnActorFromClass` "/Game/System/SkillManager/Blueprint/Actor/BP_TrashWeapon.BP_TrashWeapon_C" (`KismetMathLibrary.MakeTransform` (`self.K2_GetActorLocation` self)) "Undefined" "MultiplyWithRoot" null null))
  (bind _output_get (set `self.Trash Ref` _returnvalue_2))
  (set `/Game/System/SkillManager/Blueprint/Actor/BP_TrashWeapon.Projectile ID` _projectile_id _output_get)
  (set `/Game/System/SkillManager/Blueprint/Actor/BP_TrashWeapon.spawner` self _output_get)
  (bind _returnvalue_3 (`|GetDataTableRow` "/Game/Weapon/Data/D_ProjectileStatTable.D_ProjectileStatTable" _returnvalue)
    (:`then`
      (bind _returnvalue_4 (`|GetDataTableRow` "/Game/Weapon/Data/D_ProjectileAssetInfo.D_ProjectileAssetInfo" _returnvalue)
        (:`then`
          (`ProjectileBase.InitProjectile` _trash_ref _owner_character _returnvalue_4 _returnvalue_3)
          (bind _asbp_boss_chapter_2_2 (cast `/Game/Character/EnemyCharacter/Blueprint/BP_Boss_Chapter2` _owner_character))
          (`/Game/Character/EnemyCharacter/Blueprint/BP_Boss_Chapter2.Add Trash Weapon` _asbp_boss_chapter_2_2 _trash_ref))))))

(fn `UserConstructionScript`)