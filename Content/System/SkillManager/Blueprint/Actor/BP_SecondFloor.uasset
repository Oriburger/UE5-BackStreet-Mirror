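; BP_SecondFloor is a floor actor that starts a timeline-driven opacity fade on BeginPlay through DestroyWithFadeOut.
; It puts dynamic instances of MI_Asphalt_Chaos on both Floor material slots, then waits briefly before playing the timeline.
; Each timeline update writes Opacity to both instances and prints it for debugging.
; Despite the event name, the graph never destroys the actor.
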(event `self.ReceiveBeginPlay`
  (`self.Destroy With Fade Out`))

(event `Destroy With Fade Out`
  (bind _floor (`self.Floor`))
  (bind _returnvalue (`PrimitiveComponent.CreateDynamicMaterialInstance` _floor 0 "/Game/System/Chaos/Material/MI_Asphalt_Chaos.MI_Asphalt_Chaos" "None"))
  (`PrimitiveComponent.SetMaterial` _floor 0 _returnvalue)
  (bind _returnvalue_2 (`PrimitiveComponent.CreateDynamicMaterialInstance` _floor 1 "/Game/System/Chaos/Material/MI_Asphalt_Chaos.MI_Asphalt_Chaos" "None"))
  (`PrimitiveComponent.SetMaterial` _floor 1 _returnvalue_2)
  (`KismetSystemLibrary.Delay` 2.0)
  (bind (_direction _opacity) (`Timeline|타임라인`)
    (:`Update`
      (`MaterialInstanceDynamic.SetScalarParameterValue` _returnvalue_2 "Opacity" _opacity)
      (`MaterialInstanceDynamic.SetScalarParameterValue` _returnvalue "Opacity" _opacity)
      (`KismetSystemLibrary.PrintString` (`KismetStringLibrary.Conv_DoubleToString` _opacity)))))

(fn `UserConstructionScript`)