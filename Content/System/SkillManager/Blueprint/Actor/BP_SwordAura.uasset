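; BP_SwordAura is a homing sword-aura projectile that damages the player character on overlap.
; Each tick it advances a fixed step along the capsule's forward vector, eases its yaw toward the player and spins the Aura component; movement and turning ignore frame delta time.
; Capsule overlap with the player applies damage, and any overlap destroys the actor.
; An accumulated-time check also destroys it after a few seconds.
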(event `self.Capsule.OnComponentBeginOverlap`
  (params (OverlappedComponent :type "PrimitiveComponent Object Reference") (OtherActor :type "Actor Object Reference") (OtherComp :type "PrimitiveComponent Object Reference") (OtherBodyIndex :type Integer) (bFromSweep :type Boolean) (SweepResult :type "HitResult Structure (by ref)"))
  ;[1 1 1 1 30] Overlap시 데미지 주고 Destroy
  (`/Engine/EditorBlueprintResources/StandardMacros.IsValid` OverlappedComponent
    (:`Is Valid`
      (if (== OtherActor (`GameplayStatics.GetPlayerCharacter` 0))
        (`GameplayStatics.ApplyDamage` (`GameplayStatics.GetPlayerCharacter` 0) 100.0 null self "/Script/Engine.DamageType")
        (`self.K2_DestroyActor`)
        (else
          (`self.K2_DestroyActor`))))))

(event `self.ReceiveTick`
  (params (DeltaSeconds :type "Float (single-precision)"))
  (bind (_returnvalue_roll _returnvalue_pitch _returnvalue_yaw) (`KismetMathLibrary.BreakRotator` (`self.K2_GetActorRotation`)))
  (bind _aura (`self.Aura`))
  (bind (_returnvalue_roll_2 _returnvalue_pitch_2 _returnvalue_yaw_2) (`KismetMathLibrary.BreakRotator` (`KismetMathLibrary.FindLookAtRotation` (`self.K2_GetActorLocation`) (`self.K2_GetActorLocation` (`GameplayStatics.GetPlayerCharacter` 0)))))
  ;[0.9429 0.7035 1 1 30] Tick마다 플레이어 추적, SwordAuraTime을 매 틱마다 Delta Seconds 더해 일정 값보다 크면(일정시간이 지나면) Destroy
  (bind _output_get (set `self.SwordAuraTime` (+ (`self.SwordAuraTime`) DeltaSeconds)))
  (if (> _output_get 4.0)
    (set `self.SwordAuraTime` 0.0)
    (`self.K2_DestroyActor`)
    (else
      (`self.K2_AddActorWorldOffset` (* (`SceneComponent.GetForwardVector` (`self.Capsule`)) 6.0))
      (`self.K2_SetActorRotation` (`KismetMathLibrary.RInterpTo` (`KismetMathLibrary.MakeRotator` 0.0 0.0 _returnvalue_yaw) (`KismetMathLibrary.MakeRotator` 0.0 0.0 _returnvalue_yaw_2) 0.01 2.0))
      (`/Engine/EditorBlueprintResources/StandardMacros.IsValid` _aura
        (:`Is Valid`
          (`SceneComponent.K2_AddLocalRotation` _aura (struct :`Yaw` -30.0) false false))))))

(fn `UserConstructionScript`)