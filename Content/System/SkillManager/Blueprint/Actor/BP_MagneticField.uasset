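; BP_MagneticField is a skill actor that drags the player toward its center, then releases an expanding damage wave.
; A looping timer interpolates player location for about five seconds, faster with distance, while Niagara bursts play at spawn and two seconds later.
; Near the end, if the player is still off-center, a second timer widens the Wave horizontally.
; Wave overlap damages the player unless touching WaveCenter has already cleared CanApplyDamage.
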(event `self.ReceiveBeginPlay`
  (bind _returnvalue (`KismetSystemLibrary.K2_SetTimerDelegate` (delegate `InterpToMagneticCenter`) 0.01 true))
  (set `self.MagneticInterpTimerHandler` _returnvalue)
  (`NiagaraFunctionLibrary.SpawnSystemAtLocation` "/Game/Asset/VFX/sA_Megapack_v1/sA_Projectilevfx/Vfx/Fx/Niagara_Systems/NS_Projectile6.NS_Projectile6" (`SceneComponent.K2_GetComponentLocation` (`self.MagneticCenter`)) (struct) (2.0 2.0 2.0))
  (`KismetSystemLibrary.Delay` 2.0)
  (`NiagaraFunctionLibrary.SpawnSystemAtLocation` "/Game/Asset/VFX/sA_Megapack_v1/sA_Projectilevfx/Vfx/Fx/Niagara_Systems/NS_Projectile6.NS_Projectile6" (`SceneComponent.K2_GetComponentLocation` (`self.MagneticCenter`)) (struct) (2.0 2.0 2.0)))

(event `InterpToMagneticCenter`
  (bind _returnvalue (`GameplayStatics.GetPlayerCharacter` 0))
  (bind _returnvalue_2 (`self.K2_GetActorLocation`))
  (bind _timer (`self.Timer`))
  (bind _returnvalue_3 (`self.K2_GetActorLocation` _returnvalue))
  (set `self.Timer` (+ (`self.Timer`) 0.01))
  (if (!= _returnvalue_3 _returnvalue_2 :`ErrorTolerance` 0.9)
    (`self.K2_SetActorLocation` _returnvalue (`KismetMathLibrary.VInterpTo` _returnvalue_3 _returnvalue_2 0.01 (* (`self.GetDistanceTo` _returnvalue self) 0.001)) false false)
    (if (>= _timer 4.8)
      (if (>= _timer 5.0)
        (`KismetSystemLibrary.K2_ClearAndInvalidateTimerHandle` (`self.MagneticInterpTimerHandler`))
        (else
          (`/Engine/EditorBlueprintResources/StandardMacros.DoOnce` false
            (:`Completed`
              (`self.WaveEffectDamge`))))))))

(event `self.Wave.OnComponentBeginOverlap`
  (params (OverlappedComponent :type "PrimitiveComponent Object Reference") (OtherActor :type "Actor Object Reference") (OtherComp :type "PrimitiveComponent Object Reference") (OtherBodyIndex :type Integer) (bFromSweep :type Boolean) (SweepResult :type "HitResult Structure (by ref)"))
  (bind _returnvalue (`GameplayStatics.GetPlayerCharacter` 0))
  (`/Engine/EditorBlueprintResources/StandardMacros.IsValid` OtherActor
    (:`Is Valid`
      (if (`self.bCanApplyDamage`)
        (if (== OtherActor _returnvalue)
          (`GameplayStatics.ApplyDamage` _returnvalue 50.0 null self "/Script/Engine.DamageType"))))))

(event `WaveEffectDamge`
  (bind _returnvalue (`KismetSystemLibrary.K2_SetTimerDelegate` (delegate `WaveEffect`) 0.01 true))
  (set `self.WeveScaleTimerHandler` _returnvalue)
  (`KismetSystemLibrary.Delay` 2.0)
  (`KismetSystemLibrary.K2_ClearAndInvalidateTimerHandle` (`self.WeveScaleTimerHandler`)))

(event `WaveEffect`
  (bind _wave (`self.Wave`))
  (`SceneComponent.SetWorldScale3D` _wave (+ (`SceneComponent.K2_GetComponentScale` _wave) (0.5 0.5 0.0))))

(event `self.WaveCenter.OnComponentBeginOverlap`
  (params (OverlappedComponent :type "PrimitiveComponent Object Reference") (OtherActor :type "Actor Object Reference") (OtherComp :type "PrimitiveComponent Object Reference") (OtherBodyIndex :type Integer) (bFromSweep :type Boolean) (SweepResult :type "HitResult Structure (by ref)"))
  (`/Engine/EditorBlueprintResources/StandardMacros.IsValid` OtherActor
    (:`Is Valid`
      (if (== OtherActor (`GameplayStatics.GetPlayerCharacter` 0))
        (set `self.bCanApplyDamage` false)))))

(fn `UserConstructionScript`)