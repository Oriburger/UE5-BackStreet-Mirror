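; BP_SkillRange_Rectangle is an actor that sizes a rectangular skill range shape.
; Shortly after BeginPlay, it sets SkillRange's world scale from SkillRangeX and SkillRangeY, adding SkillFloor's X scale to the length and flattening Z to zero.
; A looping-timer setup and a relative-scale variant are left unconnected, and the SkillRangeScale event is empty, so scaling happens only once.
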(event `self.ReceiveBeginPlay`
  (bind _returnvalue_x (`KismetMathLibrary.BreakVector` (`SceneComponent.K2_GetComponentScale` (`self.SkillFloor`))))
  (`KismetSystemLibrary.Delay` 0.2)
  (`SceneComponent.SetWorldScale3D` (`self.SkillRange`) (`KismetMathLibrary.MakeVector` (+ (`self.SkillRangeX`) _returnvalue_x) (`self.SkillRangeY`))))

(event `SkillRangeScale`)

(fn `UserConstructionScript`)