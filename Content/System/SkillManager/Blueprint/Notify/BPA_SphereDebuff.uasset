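; BPA_SphereDebuff is an animation notify that debuffs a nearby player when the animation reaches it.
; It sphere-overlaps pawns around the mesh owner and stores the last MainCharacterBase tagged Player in a member reference, which is not cleared between triggers.
; If that reference is valid, it applies the configured debuff type and duration with the owner as causer, then spawns an effect at the owner.
; An optional debug sphere shows the radius.
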(fn `Received_Notify`
  (params (MeshComp :type "SkeletalMeshComponent Object Reference") (Animation :type "AnimSequenceBase Object Reference") (EventReference :type "AnimNotifyEventReference Structure (by ref)"))
  (returns (ReturnValue :type Boolean))
  (locals (mainCharRef :type "MainCharacterBase Object Reference"))
  (bind _returnvalue (`ActorComponent.GetOwner` MeshComp))
  (bind _overlap_radius (`self.Overlap Radius`))
  (bind _maincharref (`local.mainCharRef`))
  (bind _returnvalue_2 (`Actor.K2_GetActorLocation` _returnvalue))
  (if (`self.DrawDebugSphere`)
    (`KismetSystemLibrary.DrawDebugSphere` _returnvalue_2 _overlap_radius 12 (struct :`R` 1.0 :`B` 0.881596 :`A` 1.0) 1.0 2.0))
  (bind _outactors (`KismetSystemLibrary.SphereOverlapActors` _returnvalue_2 _overlap_radius (`|MakeArray` "ObjectTypeQuery3" :!type "EObjectTypeQuery Enum") "/Script/BackStreet.MainCharacterBase" (`|MakeArray` _returnvalue)))
  (for _array_element _outactors
    (`/Engine/EditorBlueprintResources/StandardMacros.IsValid` _array_element
      (:`Is Valid`
        (if (`Actor.ActorHasTag` _array_element "Player")
          (bind _asmain_character_base (cast `MainCharacterBase` _array_element))
          (set `local.mainCharRef` _asmain_character_base)))))
  (`/Engine/EditorBlueprintResources/StandardMacros.IsValid` _maincharref
    (:`Is Valid`
      (`CharacterBase.TryAddNewDebuff` _maincharref (make `DebuffInfoStruct` :`Type` (`self.DebuffType`) :`TotalTime` (`self.StunTime`)) _returnvalue)
      (`NiagaraFunctionLibrary.SpawnSystemAtLocation` (`self.Debuff FX`) _returnvalue_2 (`Actor.K2_GetActorRotation` _returnvalue) (`self.Debuff Scale`))
      (return true))
    (:`Is Not Valid`
      (return false))))