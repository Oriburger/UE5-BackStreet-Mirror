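; Save manager that persists and restores chapter progress, player inventory and achievement data through the Easy Save Game component.
; Fetch events snapshot the chapter manager and player into structs cached on the GameInstance; achievement fetching is still empty.
; Saving targets a single slot, while loading picks the newest slot and passes its level to the GameInstance.
; The component callback chains progress, inventory and achievements, applying each on load and broadcasting failure if one fails.
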(event `self.BP_EasySaveGameComponent.LoadingOrSavingVariables`
  (params (OperationType :type "/Game/EasyGameUI/EasySaveGameUI/Datas/E_SaveGameOperationType Enum" :default "NewEnumerator0") (JsonObject :type "JsonObjectWrapper Structure"))
  ;[0.9717 1 0.303] On Save / Load
  (bind _loadedvalue (`/Game/EasyGameUI/Core/BML_EasyMacroUtilities.SaveOrLoadVariable` OperationType JsonObject "ProgressData" (`self.ProgressSaveData`))
    (:`Loaded`
      (set `self.ProgressSaveData` _loadedvalue)
      (`self.LoadProgress`)
      (bind _loadedvalue_2 (`/Game/EasyGameUI/Core/BML_EasyMacroUtilities.SaveOrLoadVariable` OperationType JsonObject "InventoryData" (`self.InventorySaveData`))
        (:`Loaded`
          (set `self.InventorySaveData` _loadedvalue_2)
          (`self.LoadInventory`)
          (bind _loadedvalue_3 (`/Game/EasyGameUI/Core/BML_EasyMacroUtilities.SaveOrLoadVariable` OperationType JsonObject "AchievementData" (`self.AchievementSaveData`))
            (:`Loaded`
              (set `self.AchievementSaveData` _loadedvalue_3)
              (`self.LoadAchievement`))
            (:`FailedToLoad`
              (`self.OnLoadDone` false :!label _label))))
        (:`FailedToLoad`
          (goto _label))))
    (:`FailedToLoad`
      (goto _label))))

(event `self.Initialize`
  ;[1 1 1 1 40] BeginPlay
  (`parent.Initialize`)
  (bind _output_get (set `self.GameInstanceRef` (`/Game/UI/Global/BPFL_CommonWidget.GetGameInstanceRef`)))
  (bind (_outprogressdata _outachievementdata _outinventorydata) (`BackStreetGameInstance.GetCachedSaveGameData` _output_get))
  (set `self.ProgressSaveData` _outprogressdata)
  (set `self.AchievementSaveData` _outachievementdata)
  (set `self.InventorySaveData` _outinventorydata)
  (set `self.PlayerRef` (`/Game/UI/Global/BPFL_CommonWidget.GetMainCharacterRef`))
  (set `self.ChapterManagerRef` (`/Game/UI/Global/BPFL_CommonWidget.GetChapterManagerRef`)))

(event `self.SaveGameData`
  ;[1 0.4698 0.4128 1 40] Save / Load Game Data
  (`parent.SaveGameData`)
  (bind _saveuniquename (`/Game/EasyGameUI/EasySaveGameUI/Core/BFL_EasySaveGameFunctions.FindAvailableIndexForSaveType` (`self.MainSaveType`) 1))
  (message `/Game/EasyGameUI/EasySaveGameUI/Core/BPI_EasySaveGameInterface.StartSaveGameOperation` (`GameplayStatics.GetGameInstance`) (make `/Game/EasyGameUI/EasySaveGameUI/Datas/S_SaveOperationInfos` _saveuniquename) false))

(event `self.LoadGameData`
  ;[1 0.4698 0.4128 1 40] Save / Load Game Data
  (`parent.LoadGameData`)
  (bind (_foundslots _foundslots_) (`/Game/EasyGameUI/EasySaveGameUI/Core/BFL_EasySaveGameFunctions.GetAllSaveSlots` (`self.MainSaveType`)))
  (if _foundslots_
    (bind (_slotuniquename _slotindex _saveslot) (`/Game/EasyGameUI/EasySaveGameUI/Core/BFL_EasySaveGameFunctions.FindNewestOrOldestSaveSlotFromList` _foundslots true))
    (message `/Game/EasyGameUI/EasySaveGameUI/Core/BPI_EasySaveGameInterface.SetupGameInstanceForSaveGameOperation` (`self.GameInstanceRef`) (make `/Game/EasyGameUI/EasySaveGameUI/Datas/S_SaveOperationInfos` _slotuniquename "NewEnumerator1" "NewEnumerator2" true) (`.Level_21_695CD24945849F1ACCE62C89B973AEA9` (break `/Game/EasyGameUI/EasySaveGameUI/Datas/S_SaveGameMetadata` (`/Game/EasyGameUI/EasySaveGameUI/Core/BP_EasySaveGameObject.Metadatas` _saveslot))))))

(event `self.SaveInventory`
  ;[0.6997 1 0.5547 1 40] Save Detail Data
  (`parent.SaveInventory`)
  (`self.SaveGameData` :!label _label_2))

(event `self.SaveProgress`
  ;[0.6997 1 0.5547 1 40] Save Detail Data
  (`parent.SaveProgress`)
  (goto _label_2))

(event `OnPostLoadMap_1`
  (params (LoadedWorld :type "World Object Reference")))

(event `self.SaveAchievement`
  ;[0.6997 1 0.5547 1 40] Save Detail Data
  (`parent.SaveAchievement`)
  (goto _label_2))

(event `self.FetchInventoryData`
  ;[1 0.3976 0.3178 1 40] Fetch Data
  (bind _playerref (`self.PlayerRef`)
    (:`then`
      (bind _iteminventory (`MainCharacterBase.ItemInventory` _playerref))
      (set `self.InventorySaveData` (make `InventorySaveData` (`ItemInventoryComponent.GetGenesiumAmount` _iteminventory) (`ItemInventoryComponent.GetFusionCellAmount` _iteminventory)))
      (`KismetSystemLibrary.PrintString` "InvSaved")
      (`BackStreetGameInstance.CacheGameData` (`/Game/UI/Global/BPFL_CommonWidget.GetGameInstanceRef`) (`self.ProgressSaveData`) (`self.AchievementSaveData`) (`self.InventorySaveData`) :!label _label_3))
    (:`else`)))

(event `self.LoadInventory`
  (bind (_genesiumcount _fusioncellcount) (break `InventorySaveData` (`self.InventorySaveData`)))
  ;[0.4257 0.7329 1 1 40] Load Detail Data
  (`parent.LoadInventory`)
  (bind _playerref (`self.PlayerRef`)
    (:`then`
      (bind _iteminventory (`MainCharacterBase.ItemInventory` _playerref))
      ;;[1 1 1 1 12] SetGenesium / FusionCell
      (`ItemInventoryComponent.AddItem` _iteminventory (`ItemInventoryComponent.GenesiumID` _iteminventory) (`KismetMathLibrary.Conv_IntToByte` _genesiumcount))
      (`ItemInventoryComponent.AddItem` _iteminventory (`ItemInventoryComponent.FusionCellID` _iteminventory) (`KismetMathLibrary.Conv_IntToByte` _fusioncellcount)))
    (:`else`)))

(event `self.FetchProgressData`
  ;[1 0.3976 0.3178 1 40] Fetch Data
  (bind _chaptermanagerref (`self.ChapterManagerRef`)
    (:`then`
      (bind _playerref (`self.PlayerRef`)
        (:`then`
          (set `self.ProgressSaveData` (make `ProgressSaveData` true true (`NewChapterManagerBase.GetCurrentChapterInfo` _chaptermanagerref) (`StageManagerComponent.GetCurrentStageInfo` (`NewChapterManagerBase.StageManagerComponent` _chaptermanagerref)) (`CharacterBase.CharacterGameplayInfo` _playerref)))
          (`KismetSystemLibrary.PrintString` "ChapterSaved")
          (goto _label_3))
        (:`else`)))
    (:`else`
      (`KismetSystemLibrary.PrintString` "NotValid"))))

(event `self.LoadProgress`
  (bind (_bistutorialdone _bisingame _chapterinfo _stageinfo _characterinfo) (break `ProgressSaveData` (`self.ProgressSaveData`)))
  ;[0.4257 0.7329 1 1 40] Load Detail Data
  (`parent.LoadProgress`)
  (bind _chaptermanagerref (`self.ChapterManagerRef`)
    (:`then`
      (`StageManagerComponent.OverwriteStageInfo` (`NewChapterManagerBase.StageManagerComponent` _chaptermanagerref) _chapterinfo _stageinfo)
      (bind _playerref (`self.PlayerRef`)
        (:`then`
          (set `CharacterBase.CharacterGameplayInfo` _characterinfo _playerref)
          (`KismetSystemLibrary.PrintString` "LogSystem) BP_SaveManager :: LoadProgress - Load Done" false))
        (:`else`)))
    (:`else`
      (`KismetSystemLibrary.PrintString` "LogSystem) BP_SaveManager :: LoadProgress - ChapterManager is not valid" false))))

(event `self.LoadAchievement`
  ;[0.4257 0.7329 1 1 40] Load Detail Data
  (`parent.LoadAchievement`))

(event `self.FetchAchievementData`
  ;[1 0.3976 0.3178 1 40] Fetch Data
)

(fn `UserConstructionScript`)