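; BP_SaveSlotManager handles saving and loading of the game's progress, inventory, achievement and slot-info data through EasySaveGame.
; SaveGameData caches current state and starts a save via the game instance only for valid slots: named, tutorial done, in game or neutral zone.
; The component's callback chains the four variables through SaveOrLoadVariable and reports completion.
; It then sets the slot name, picking the first free index if needed; Tick prints debug state.
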(event `self.ReceiveTick`
  (params (DeltaSeconds :type "Float (single-precision)"))
  (bind ((`bIsInNeutralZone` _bisinneutralzone) (`bIsRequiredToMoveNeutralZone` _bisrequiredtomoveneutralzone)) (break `SaveSlotInfo` (`self.SaveSlotInfo`)))
  (`KismetSystemLibrary.PrintString` (`KismetStringLibrary.Concat_StrStr` "Core  Count : " (`KismetStringLibrary.Conv_IntToString` (`.TotalCoreCountInGame` (break `ProgressSaveData` (`self.ProgressSaveData`)))) ", " (`KismetStringLibrary.Conv_IntToString` (`.CoreCount` (break `InventorySaveData` (`self.InventorySaveData`)))) " /  bIsInNeutralZone : " (`KismetStringLibrary.Conv_BoolToString` _bisinneutralzone) " \n / bIsRequiredToMoveNeutralZone : " (`KismetStringLibrary.Conv_BoolToString` _bisrequiredtomoveneutralzone)) true true (struct :`G` 1.0 :`B` 0.297706 :`A` 1.0) (`GameplayStatics.GetWorldDeltaSeconds`)))

(event `self.BP_EasySaveGameComponent.LoadingOrSavingVariables`
  (params (OperationType :type "/Game/EasyGameUI/EasySaveGameUI/Datas/E_SaveGameOperationType Enum" :default "NewEnumerator0") (JsonObject :type "JsonObjectWrapper Structure"))
  (bind _returnvalue (`self.DefineSaveSlotName`))
  ;[1 0.9617 0 1 32] Handling EasySaveGame System
  (set `self.TempCount` 0)
  (bind _loadedvalue (`/Game/EasyGameUI/Core/BML_EasyMacroUtilities.SaveOrLoadVariable` OperationType JsonObject "ProgressSaveData" (`self.ProgressSaveData`))
    (:`Saved`
      (`/Engine/EditorBlueprintResources/StandardMacros.IncrementInt` (`self.TempCount`)
        (:`  `
          (bind _loadedvalue_2 (`/Game/EasyGameUI/Core/BML_EasyMacroUtilities.SaveOrLoadVariable` OperationType JsonObject "InventorySaveData" (`self.InventorySaveData`) :!label _label)
            (:`Saved`
              (`/Engine/EditorBlueprintResources/StandardMacros.IncrementInt` (`self.TempCount`)
                (:`  `
                  (bind _loadedvalue_3 (`/Game/EasyGameUI/Core/BML_EasyMacroUtilities.SaveOrLoadVariable` OperationType JsonObject "AchievementSaveData" (`self.AchievementSaveData`) :!label _label_2)
                    (:`Saved`
                      (`/Engine/EditorBlueprintResources/StandardMacros.IncrementInt` (`self.TempCount`)
                        (:`  `
                          (bind _loadedvalue_4 (`/Game/EasyGameUI/Core/BML_EasyMacroUtilities.SaveOrLoadVariable` OperationType JsonObject "SaveSlotInfo" (`self.SaveSlotInfo`) :!label _label_3)
                            (:`Saved`
                              (`/Engine/EditorBlueprintResources/StandardMacros.IncrementInt` (`self.TempCount`)
                                (:`  `
                                  (if (== (`self.TempCount`) 4)
                                    (`self.OnSaveDone` true)
                                    (`KismetSystemLibrary.Delay` 2.0 :!label _label_4)
                                    (`KismetSystemLibrary.PrintString` (`KismetStringLibrary.Concat_StrStr` "LogSaveSystem) BP_SaveSlotManager : New save slot name is --> " _returnvalue) true true (struct :`R` 1.0 :`G` 0.887542 :`A` 1.0) :!label _label_5)
                                    (`self.SetSaveSlotName` _returnvalue)
                                    (else
                                      (`KismetSystemLibrary.PrintString` "LogSaveSystem) BP_SaveSlotManager : Failed" false :!label _label_6)
                                      (`self.OnLoadDone` false))))))
                            (:`Loaded`
                              (bind (_saveslotname _bisinitialized _bestchaptercleartimelist _bistutorialdone _bisingame) (break `SaveSlotInfo` _loadedvalue_4))
                              (`KismetSystemLibrary.PrintString` (`KismetStringLibrary.Concat_StrStr` "Slot Name : " _saveslotname " / is init ? : " (`KismetStringLibrary.Conv_BoolToString` _bisinitialized) " / Is tuto done ? : " (`KismetStringLibrary.Conv_BoolToString` _bistutorialdone) " / Is in game ? : " (`KismetStringLibrary.Conv_BoolToString` _bisingame) "@@@@@@@@@@@@@@@@@@@@@@@@@@@@@@@@@@@@"))
                              (set `self.SaveSlotInfo` _loadedvalue_4)
                              (`self.OnLoadDone` true)
                              (goto _label_4))
                            (:`FailedToLoad`
                              (goto _label_6))))))
                    (:`Loaded`
                      (set `self.AchievementSaveData` _loadedvalue_3)
                      (goto _label_3))
                    (:`FailedToLoad`
                      (goto _label_6))))))
            (:`Loaded`
              (set `self.InventorySaveData` _loadedvalue_2)
              (goto _label_2))
            (:`FailedToLoad`
              (goto _label_6))))))
    (:`Loaded`
      (set `self.ProgressSaveData` _loadedvalue)
      (goto _label))
    (:`FailedToLoad`
      (goto _label_6))))

(event `self.InitializeSaveSlotName`
  ;[1 0.9617 0 1 32] Handling EasySaveGame System
  (bind _returnvalue (`GameplayStatics.GetCurrentLevelName` true))
  (if (not (`KismetStringLibrary.Contains` _returnvalue "MainMenu"))
    (goto _label_5)))

(event `self.SaveGameData`
  (bind _asback_street_game_instance (`/Game/UI/Global/BPFL_CommonWidget.GetGameInstanceRef`))
  (bind ((`SaveSlotName` _saveslotname) (`BestChapterClearTimeList` _bestchaptercleartimelist) (`bIsTutorialDone` _bistutorialdone) (`bIsInGame` _bisingame) (`bIsInNeutralZone` _bisinneutralzone)) (break `SaveSlotInfo` (`self.SaveSlotInfo`)))
  ;[1 0.9617 0 1 32] Handling EasySaveGame System
  ;;[1 0.3574 0.515] 세이브 슬롯에 저장한다
  (`parent.SaveGameData`)
  (if (and (`KismetStringLibrary.Contains` _saveslotname (`self.Main Save Type`)) _bistutorialdone (or _bisingame _bisinneutralzone))
    (`self.FetchGameData`)
    (`self.CacheCurrentGameState`)
    (message `/Game/EasyGameUI/EasySaveGameUI/Core/BPI_EasySaveGameInterface.StartSaveGameOperation` _asback_street_game_instance (make `/Game/EasyGameUI/EasySaveGameUI/Datas/S_SaveOperationInfos` (`.SaveSlotName` (break `SaveSlotInfo` (`BackStreetGameInstance.SaveSlotInfo` _asback_street_game_instance)))) false)
    (else
      (`KismetSystemLibrary.PrintString` "BP_SaveSlotManager -> SaveGameData : Invalid SaveSlot" false))))

(fn `DefineSaveSlotName`
  (returns (ReturnValue :type String))
  (bind ((`SaveSlotName` _saveslotname)) (break `SaveSlotInfo` (`self.SaveSlotInfo`)))
  (if (not (`KismetStringLibrary.Contains` _saveslotname (`self.Main Save Type`)))
    (bind _foundslots (`/Game/EasyGameUI/EasySaveGameUI/Core/BFL_EasySaveGameFunctions.GetAllSaveSlots` (`self.Main Save Type`)))
    (for _index (range (+ (`KismetArrayLibrary.Array_Length` _foundslots) 1))
      (bind _returnvalue (`KismetStringLibrary.Concat_StrStr` (`self.Main Save Type`) " " (`KismetStringLibrary.Conv_IntToString` _index)))
      (if (not (`KismetArrayLibrary.Array_Contains` _foundslots _returnvalue))
        (return _returnvalue)))
    (else
      (return _saveslotname))))

(fn `PrintCurrentSaveSlotName`
  (bind _asgi_egui_main_game_instance (cast `/Game/EasyGameUI/Core/GI_EGUI_MainGameInstance` (`/Game/UI/Global/BPFL_CommonWidget.GetGameInstanceRef`)))
  (if true
    (`KismetSystemLibrary.PrintString` (`KismetStringLibrary.Concat_StrStr` (`BackStreetGameInstance.GetCurrentSaveSlotName` _asgi_egui_main_game_instance) " / " (`/Game/EasyGameUI/EasySaveGameUI/Core/BP_EasySaveGameOperationsManager.CurrentSaveSlot` (`/Game/EasyGameUI/Core/GI_EGUI_MainGameInstance.SaveGameOperationsManager` _asgi_egui_main_game_instance))) true false (struct :`R` 1.0 :`B` 0.823312 :`A` 1.0))))

(fn `UserConstructionScript`)