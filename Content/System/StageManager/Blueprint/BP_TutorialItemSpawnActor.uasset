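; BP_TutorialItemSpawnActor is a tutorial helper actor that supplies the player with a melee-only item box.
; SpawnWeaponBox spawns a BP_ItemBox_MeleeOnly only when none tagged "Tuto" exists, then tags the new box to prevent duplicates.
; The box appears at the player character's location plus a fixed-seed random unit vector, so the tiny offset is always identical.
; The event graph is empty, so this file never calls the function itself.
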(event `self.ReceiveActorBeginOverlap`
  (params (OtherActor :type "Actor Object Reference")))

(fn `SpawnWeaponBox`
  (bind _returnvalue_location (`KismetMathLibrary.BreakTransform` (`self.GetTransform` (`GameplayStatics.GetPlayerCharacter` 0))))
  (bind _outactors (`GameplayStatics.GetAllActorsOfClassWithTag` "/Game/Item/Blueprint/ItemBox/BP_ItemBox_MeleeOnly.BP_ItemBox_MeleeOnly_C" "Tuto"))
  (if (`KismetArrayLibrary.Array_IsEmpty` _outactors)
    (bind _returnvalue (`|SpawnActorFromClass` "/Game/Item/Blueprint/ItemBox/BP_ItemBox_MeleeOnly.BP_ItemBox_MeleeOnly_C" (`KismetMathLibrary.MakeTransform` (+ _returnvalue_location (`KismetMathLibrary.RandomUnitVectorFromStream` (`KismetMathLibrary.MakeRandomStream` 50)))) "Undefined" "OverrideRootScale" null null))
    (`KismetArrayLibrary.Array_Add` (`Actor.Tags` _returnvalue) "Tuto")))

(fn `UserConstructionScript`)