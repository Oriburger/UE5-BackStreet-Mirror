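; BP_ChapterManager_ shows the end-of-chapter and game result screens.
; CreateGameResultWidget spawns the result widget with IsGameOver set to the inverse of ChapterClear, while CreateChapterCleartWidget spawns the chapter clear widget.
; Both events slow global time dilation, wait briefly, safely create the widget on the viewport, store its reference, and pass it as an activatable base to HandleInputMappingContext.
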(event `self.CreateGameResultWidget`
  (params (bChapterClear :type Boolean))
  ;[1 1 1] 게임 결과창
  (`GameplayStatics.SetGlobalTimeDilation` 0.2)
  (`KismetSystemLibrary.Delay` 0.2)
  (bind _widgetref (`/Game/EasyGameUI/Core/BFL_EasyFunctionUtilities.SafeCreateWidget` "/Game/UI/InGame/Blueprint/CombatUI/Area/WB_Area_GameResult.WB_Area_GameResult_C"))
  (bind _aswb_area_game_result (cast `/Game/UI/InGame/Blueprint/CombatUI/Area/WB_Area_GameResult` _widgetref))
  (set `/Game/UI/InGame/Blueprint/CombatUI/Area/WB_Area_GameResult.bIsGameOver` (not bChapterClear) _aswb_area_game_result)
  (bind _output_get (set `self.GameResultWidgetRef` _aswb_area_game_result))
  (bind _aswb_cui_activatable_base (cast `/Game/UI/Global/WB_CUI_ActivatableBase` _output_get))
  (`/Game/UI/Global/BPFL_CommonWidget.Handle Input Mapping Context` _aswb_cui_activatable_base))

(event `self.CreateChapterCleartWidget`
  ;[1 1 1] 게임 결과창
  (`GameplayStatics.SetGlobalTimeDilation` 0.2)
  (`KismetSystemLibrary.Delay` 0.2)
  (bind _widgetref (`/Game/EasyGameUI/Core/BFL_EasyFunctionUtilities.SafeCreateWidget` "/Game/UI/InGame/Blueprint/CombatUI/Area/WB_Area_ChapterClear.WB_Area_ChapterClear_C"))
  (bind _output_get (set `self.ChapterClearWidgetRef` _widgetref))
  (bind _aswb_cui_activatable_base (cast `/Game/UI/Global/WB_CUI_ActivatableBase` _output_get))
  (`/Game/UI/Global/BPFL_CommonWidget.Handle Input Mapping Context` _aswb_cui_activatable_base))

(fn `UserConstructionScript`)