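; Stage gate actor that previews a stage through an icon and info widget.
; InitGate fills both from StageInfo, using the first reward for most combat stages and masking heal pack sizes behind a generic name.
; After a delay, a timeline drives dynamic-material opacity to reveal the gate, then enables overlap, arrow, icon and direction indicator.
; Interaction availability toggles a key-guide child actor and plays the info animation forward or reverse.
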(event `self.InitGate`
  (params (NewDirection :type "Vector2D Structure") (StageInfo :type "StageInfo Structure"))
  (bind (_stagetype _stageicon _coordinate _mainlevelasset _outerlevelasset _enemycompositioninfo _rewardinfolist) (break `StageInfo` (`self.Stage Info`)))
  (bind ((`ItemName` _itemname) (`ItemNameText` _itemnametext) (`ItemDescriptionText` _itemdescriptiontext)) (break `ItemInfoDataStruct` (`|GetArrayItem` _rewardinfolist)))
  (bind _returnvalue (`KismetStringLibrary.Contains` (`KismetStringLibrary.Conv_NameToString` _itemname) "힐팩"))
  ;[1 1 1] 코멘트
  (`parent.InitGate` NewDirection StageInfo)
  (bind _output_get (set `self.Stage Info` StageInfo))
  (bind (_stagetype_2 _stageicon_2) (break `StageInfo` _output_get))
  (bind _output_get_2 (set `self.Stage Type` _stagetype_2))
  (bind _aswb_comp_info_map_stage_icon (cast `/Game/UI/InGame/Blueprint/Legacy/WB_Comp_InfoMap_StageIcon` (`WidgetComponent.GetWidget` (`self.Icon`))))
  (`/Game/UI/InGame/Blueprint/Legacy/WB_Comp_InfoMap_StageIcon.Initialize` _aswb_comp_info_map_stage_icon _output_get_2 true _stageicon_2)
  (bind _aswb_stage_info (cast `/Game/Item/UI/WB_StageInfo` (`WidgetComponent.GetWidget` (`self.InfoWidget`)))
    (:`then`
      (switch `EStageCategoryInfo` _stagetype
        (:`E_None`
          (`KismetSystemLibrary.PrintString` "BP_Gate : Invalid Stage Info" :!label _label))
        (:`E_Lobby`
          (goto _label))
        (:`E_Entry`
          (`/Game/Item/UI/WB_StageInfo.Initialize` _aswb_stage_info 0 (select `bool` _returnvalue :`false` _itemnametext :`true` "Name_HealPack") _stageicon (select `bool` _returnvalue :`false` _itemdescriptiontext :`true` "Desc_HealPack") :!label _label_2))
        (:`E_Exterminate`
          (goto _label_2))
        (:`E_EliteExterminate`
          (goto _label_2))
        (:`E_TimeAttack`
          (goto _label_2))
        (:`E_EliteTimeAttack`
          (goto _label_2))
        (:`E_Escort`
          (goto _label_2))
        (:`E_EliteEscort`
          (goto _label_2))
        (:`E_Boss`
          (`/Game/Item/UI/WB_StageInfo.Initialize` _aswb_stage_info 0 "Name_BossStage" _stageicon "Desc_BossStage"))
        (:`E_Craft`
          (`/Game/Item/UI/WB_StageInfo.Initialize` _aswb_stage_info 0 "Name_CraftStage" _stageicon "Desc_CraftStage"))
        (:`E_MiniGame`
          (goto _label))
        (:`E_Gatcha`
          (goto _label))))
    (:`CastFailed`
      _))
  ;[0.484 0.6318 1] Appearance
  (`KismetSystemLibrary.Delay` 2.0)
  (`ActorComponent.Activate` (`self.GateSoundComponent`) true)
  (`SceneComponent.SetVisibility` (`self.RootComponent`) true true)
  (for (_array_element _array_index) (`self.MainMeshMaterialList`)
    (bind _returnvalue_2 (`PrimitiveComponent.CreateDynamicMaterialInstance` (`self.Mesh`) _array_index _array_element "None"))
    (`KismetArrayLibrary.Array_Add` (`self.MainMeshDynamicMaterialList`) _returnvalue_2))
  (bind (_direction `_새_트랙_0`) (`Timeline|UpdateAppearance` :!via `PlayFromStart`)
    (:`Update`
      (for _array_element_2 (`self.MainMeshDynamicMaterialList`)
        (`/Engine/EditorBlueprintResources/StandardMacros.IsValid` _array_element_2
          (:`Is Valid`
            (`MaterialInstanceDynamic.SetScalarParameterValue` _array_element_2 "OpacityProgress" `_새_트랙_0`)))))
    (:`Finished`
      (`SceneComponent.SetHiddenInGame` (`self.GuideArrow`) false true)
      (`SceneComponent.SetHiddenInGame` (`self.Icon`) false true)
      (set `PrimitiveComponent.bGenerateOverlapEvents` true (`self.OverlapVolume`))
      (`/Game/Map/Blueprint/Component/BPA_DirectionIndicatorComponent.CreateDirectionIndicator` (`self.BPA_DirectionIndicatorComponent`)))))

(event `self.ReceiveBeginPlay`
  ;[1 1 1] 코멘트
  (`SceneComponent.SetVisibility` (`self.RootComponent`) false true)
  (`GameplayStatics.PlaySoundAtLocation` "/Game/Sound/SW_Login_interaction/SW_Login_interaction_Portal_Object.SW_Login_interaction_Portal_Object" (`self.K2_GetActorLocation`) (struct) 1.0 1.0 0.0 null null null null))

(event `self.ReceiveEndPlay`
  (params (EndPlayReason :type "EEndPlayReason Enum" :default "Destroyed"))
  (bind _directionindicatorwidget (`self.DirectionIndicatorWidget`))
  ;[1 1 1] 코멘트
  (`/Engine/EditorBlueprintResources/StandardMacros.IsValid` _directionindicatorwidget
    (:`Is Valid`
      (`Widget.RemoveFromParent` _directionindicatorwidget))))

(event `self.OverlapVolume.OnInteractionAvailableStateUpdate`
  (params (bNewState :type Boolean))
  (bind _childactor (`ChildActorComponent.ChildActor` (`self.ChildActor`)))
  ;[1 1 1] Key guide
  (if bNewState
    (`self.SetActorHiddenInGame` _childactor false)
    (`self.PlayInfoWidgetAnimation` "Forward")
    (else
      (`self.SetActorHiddenInGame` _childactor true)
      (`self.PlayInfoWidgetAnimation` "Reverse"))))

(fn `PlayInfoWidgetAnimation`
  (params (PlayMode :type "EUMGSequencePlayMode Enum" :default "Forward"))
  (bind _aswb_stage_info (cast `/Game/Item/UI/WB_StageInfo` (`WidgetComponent.GetWidget` (`self.InfoWidget`))))
  (`UserWidget.PlayAnimation` _aswb_stage_info (`/Game/Item/UI/WB_StageInfo.Appear` _aswb_stage_info) 0.0 1 PlayMode 1.0 false))

(fn `UserConstructionScript`)