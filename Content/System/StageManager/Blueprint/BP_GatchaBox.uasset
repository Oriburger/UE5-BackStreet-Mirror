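; BP_GatchaBox is a gacha box that trades a player's ticket for a random ability of the matching tier.
; BeginPlay caches the player and sorts ability IDs from D_AbilityInfoTable into tier lists.
; PlayGatcha removes the ticket, rolls via GetRandomAbility, which retries with a cap against active abilities, and broadcasts the result.
; AddAbility grants the stored ID; the interaction event is empty and widget-opening code is disconnected.
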(event `self.ReceiveBeginPlay`
  (bind _returnvalue (`GameplayStatics.GetPlayerCharacter` 0))
  (`|ExecutionSequence`
    (:`then_0`
      (`/Engine/EditorBlueprintResources/StandardMacros.IsValid` _returnvalue
        (:`Is Valid`
          (bind _asmain_character_base (cast `MainCharacterBase` _returnvalue))
          (set `self.PlayerRef` _asmain_character_base))))
    (:`then_1`
      (for _index (range 23)
        (bind _returnvalue_2 (`|GetDataTableRow` "/Game/Character/MainCharacter/Data/D_AbilityInfoTable.D_AbilityInfoTable" (`KismetStringLibrary.Conv_StringToName` (`KismetStringLibrary.Conv_IntToString` _index)))
          (:`then`
            (bind ((`AbilityId` _abilityid) (`TargetStatMap` _targetstatmap) (`AbilityTier` _abilitytier)) (break `AbilityInfoStruct` _returnvalue_2))
            (switch `EAbilityTierType` _abilitytier
              (:`E_Common`
                (`KismetArrayLibrary.Array_AddUnique` (`self.CommonIDList`) _abilityid))
              (:`E_Rare`
                (`KismetArrayLibrary.Array_AddUnique` (`self.RareIDList`) _abilityid))
              (:`E_Legendary`
                (`KismetArrayLibrary.Array_AddUnique` (`self.LegendaryIDList`) _abilityid))
              (:`E_Mythic`
                (`KismetArrayLibrary.Array_AddUnique` (`self.MythicIDList`) _abilityid)))))))))

(event `self.InteractiveCollision.OnInteractionBegin`)

(event `PlayGatcha`
  (params (TicketID :type Integer))
  (bind _playerref (`self.PlayerRef`))
  (bind (_resultid _resultdata) (`self.GetRandomAbility` (select `int` (- TicketID 5) :`0` "E_Common" :`1` "E_Rare" :`2` "E_Legendary" :`3` "E_Mythic" :!type "EAbilityTierType Enum")))
  (`/Engine/EditorBlueprintResources/StandardMacros.IsValid` _playerref
    (:`Is Valid`
      (`ItemInventoryComponent.RemoveItem` (`MainCharacterBase.ItemInventory` _playerref) TicketID 1)
      (set `self.ResultAbilityID` _resultid)
      (bind _output_get (set `self.Result Data` _resultdata))
      (`self.OnGatchaEnded` _output_get)
      (set `self.Is Finished` true))))

(event `AddAbility`
  (bind _playerref (`self.PlayerRef`))
  (`/Engine/EditorBlueprintResources/StandardMacros.IsValid` _playerref
    (:`Is Valid`
      (`MainCharacterBase.TryAddNewAbility` _playerref (`self.ResultAbilityID`)))))

(fn `GetRandomAbility`
  (params (TierType :type "EAbilityTierType Enum" :default "E_None"))
  (returns (ResultID :type Integer) (ResultData :type "AbilityInfoStruct Structure"))
  (locals (TargetIDList :type "Array of Integer") (TryCount :type Integer) (Result :type Integer))
  (bind _outitem (`KismetArrayLibrary.Array_Random` (`local.TargetIDList`)))
  (`/Engine/EditorBlueprintResources/StandardMacros.IsValid` (`self.PlayerRef`)
    (:`Is Valid`
      (bind _output_get (set `local.TargetIDList` (select `EAbilityTierType` TierType :`E_Common` (`self.CommonIDList`) :`E_Rare` (`self.RareIDList`) :`E_Legendary` (`self.LegendaryIDList`) :`E_Mythic` (`self.MythicIDList`))))
      (if (`KismetArrayLibrary.Array_IsNotEmpty` _output_get)
        (bind _output_get_2 (set `local.Result` _outitem :!label _label))
        (if (and (`MainCharacterBase.GetIsAbilityActive` (`self.PlayerRef`) _outitem) (< (`local.TryCount`) 500))
          (`/Engine/EditorBlueprintResources/StandardMacros.IncrementInt` (`local.TryCount`)
            (:`  `
              (goto _label)))
          (else
            (bind _returnvalue (`|GetDataTableRow` "/Game/Character/MainCharacter/Data/D_AbilityInfoTable.D_AbilityInfoTable" (`KismetStringLibrary.Conv_StringToName` (`KismetStringLibrary.Conv_IntToString` _output_get_2)))
              (:`then`
                (return _output_get_2 _returnvalue)))))
        (else
          (return 0))))))

(fn `GetTicketDataMap`
  (returns (result :type "Map of Integer to ItemInfoDataStruct Structure"))
  (locals (resultMap :type "Map of Integer to ItemInfoDataStruct Structure"))
  (bind _playerref (`self.PlayerRef`))
  (`/Engine/EditorBlueprintResources/StandardMacros.IsValid` _playerref
    (:`Is Valid`
      (for _index (range 5 9)
        (`BlueprintMapLibrary.Map_Add` (`local.resultMap`) _index (`ItemInventoryComponent.GetItemData` (`MainCharacterBase.ItemInventory` _playerref) _index)))
      (return (`local.resultMap`)))))

(fn `UserConstructionScript`)