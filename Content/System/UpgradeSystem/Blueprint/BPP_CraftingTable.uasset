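; Crafting table prop that opens the booster chip upgrade UI when the player interacts with it.
; Its InteractiveCollision component triggers creation of WB_UI_UpgradeBoosterchip on the viewport, then hands the widget to HandleInputMappingContext as an activatable base widget.
; The same component's availability updates show or hide the InputPromptKeyGuide child actor as a key prompt.
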(event `self.ReceiveBeginPlay`
  (`parent.ReceiveBeginPlay`))

(event `self.InteractiveCollision.OnInteractionBegin`
  ;[1 1 1] 인터렉션 시작
  (bind _widgetref (`/Game/EasyGameUI/Core/BFL_EasyFunctionUtilities.SafeCreateWidget` "/Game/UI/InGame/Blueprint/UpgradeBoosterchip/WB_UI_UpgradeBoosterchip.WB_UI_UpgradeBoosterchip_C"))
  (bind _aswb_cui_activatable_base (cast `/Game/UI/Global/WB_CUI_ActivatableBase` _widgetref))
  (`/Game/UI/Global/BPFL_CommonWidget.Handle Input Mapping Context` _aswb_cui_activatable_base))

(event `self.InteractiveCollision.OnInteractionAvailableStateUpdate`
  (params (bNewState :type Boolean))
  (bind _childactor (`ChildActorComponent.ChildActor` (`self.InputPrompt_KeyGuide`)))
  ;[1 1 1] 키가이드 표시
  (if bNewState
    (`self.SetActorHiddenInGame` _childactor false)
    (else
      (`self.SetActorHiddenInGame` _childactor true))))

(fn `UserConstructionScript`)