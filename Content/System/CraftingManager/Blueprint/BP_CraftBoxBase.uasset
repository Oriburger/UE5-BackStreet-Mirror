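; BP_CraftBoxBase is a base crafting box actor that shows a Press F prompt on overlap and opens a crafting UI for the player.
; EnterUI creates a single crafting widget, slows global time to near zero, switches to game-and-UI input, and initializes the widget with the box.
; The box exposes its crafting recipe through a getter, clears the widget reference on WidgetClosed, and hides its Widget component unless tagged Tutorial.
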(event `self.ReceiveBeginPlay`
  (`parent.ReceiveBeginPlay`)
  (if (not (`self.ActorHasTag` "Tutorial"))
    (`SceneComponent.SetVisibility` (`self.Widget`) false false)))

(event `self.OverlapVolume.OnComponentBeginOverlap`
  (params (OverlappedComponent :type "PrimitiveComponent Object Reference") (OtherActor :type "Actor Object Reference") (OtherComp :type "PrimitiveComponent Object Reference") (OtherBodyIndex :type Integer) (bFromSweep :type Boolean) (SweepResult :type "HitResult Structure (by ref)"))
  ;[1 1 1] Press F 팝업 문구 호출
  (`self.VisibleGuideTextRender` OtherActor))

(event `self.OverlapVolume.OnComponentEndOverlap`
  (params (OverlappedComponent :type "PrimitiveComponent Object Reference") (OtherActor :type "Actor Object Reference") (OtherComp :type "PrimitiveComponent Object Reference") (OtherBodyIndex :type Integer))
  ;[1 1 1] Press F 팝업 문구 제거
  (`self.InVisibleGuideTextRender` OtherActor))

(event `self.EnterUI`
  (params (Causer :type "Actor Object Reference"))
  ;[1 1 1] Press F 팝업 문구 제거
  (`/Engine/EditorBlueprintResources/StandardMacros.IsValid` (`self.CraftingUI_2`)
    (:`Is Not Valid`
      (if (`self.ActorHasTag` Causer "Player")
        (bind _returnvalue (`|CreateWidget` "/Game/UI/InGame/Blueprint/Component/Crafting/WB_CraftingUI_.WB_CraftingUI__C" (`GameplayStatics.GetPlayerController` 0)))
        (bind _output_get (set `self.CraftingUI_2` _returnvalue))
        (`GameplayStatics.SetGlobalTimeDilation` 0.001)
        (`WidgetBlueprintLibrary.SetInputMode_GameAndUIEx` (`GameplayStatics.GetPlayerController` 0) null "DoNotLock" false)
        (`UserWidget.AddToViewport` _output_get 0)
        (`/Game/UI/InGame/Blueprint/Component/Crafting/WB_CraftingUI_.Initialize` _output_get self)))))

(event `WidgetClosed`
  ;[1 1 1] Press F 팝업 문구 제거
  (set `self.CraftingUI_2` null))

(fn `GetCraftingRecipe`
  (returns (NewParam :type "Array of /Game/Weapon/Data/CraftingRecipe/F_CraftingRecipe Structure"))
  (return (`self.CraftingRecipe`)))

(fn `UserConstructionScript`
  (`SceneComponent.SetVisibility` (`self.TextRenderComp`) true false))