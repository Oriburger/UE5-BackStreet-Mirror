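; BP_CraftBox is an interactable crafting box that opens the skill craft menu.
; BeginPlay creates WB_SkillCraftMenu off-screen, initializes it with the crafting manager component and binds its craft-confirmed event.
; The first interaction sets up the manager with the main character, resets craft candidates and re-initializes the menu; each interaction adds the menu to the viewport if absent.
; Interaction availability shows or hides the key guide child actor.
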(event `self.ReceiveBeginPlay`
  (`parent.ReceiveBeginPlay`)
  (bind _widgetref (`/Game/EasyGameUI/Core/BFL_EasyFunctionUtilities.SafeCreateWidget` "/Game/UI/InGame/Blueprint/Crafting/WB_SkillCraftMenu.WB_SkillCraftMenu_C" 0 false))
  (bind _aswb_skill_craft_menu (cast `/Game/UI/InGame/Blueprint/Crafting/WB_SkillCraftMenu` _widgetref))
  (`/Game/UI/InGame/Blueprint/Crafting/WB_SkillCraftMenu.Initialize` _aswb_skill_craft_menu (`self.BPA_CraftingManagerComponent`))
  (bind _output_get (set `self.SkillCraftMenuRef` _aswb_skill_craft_menu))
  (add `/Game/UI/InGame/Blueprint/Crafting/WB_SkillCraftMenu.OnCraftConfirmed` _output_get (`|CreateDelegate` (`self.BPA_CraftingManagerComponent`) :!event `OnCraftConfirmed`)))

(event `self.InteractiveCollision.OnInteractionBegin`
  (bind _bpa_craftingmanagercomponent (`self.BPA_CraftingManagerComponent`))
  (bind _skillcraftmenuref (`self.SkillCraftMenuRef`))
  ;[1 1 1] 인터렉션 시작
  (`|ExecutionSequence`
    (:`then_0`
      (`/Engine/EditorBlueprintResources/StandardMacros.DoOnce` false
        (:`Completed`
          (`CraftingManagerComponent.InitCraftingManager` _bpa_craftingmanagercomponent (`/Game/UI/Global/BPFL_CommonWidget.GetMainCharacterRef`))
          (`/Game/System/CraftingManager/Blueprint/BPA_CraftingManagerComponent.ResetCraftCandidateIDList` _bpa_craftingmanagercomponent)
          (`/Game/UI/InGame/Blueprint/Crafting/WB_SkillCraftMenu.Initialize` (`self.SkillCraftMenuRef`) _bpa_craftingmanagercomponent))))
    (:`then_1`
      (`/Engine/EditorBlueprintResources/StandardMacros.IsValid` _skillcraftmenuref
        (:`Is Valid`
          (if (not (`Widget.IsInViewport` _skillcraftmenuref))
            (`UserWidget.AddToViewport` _skillcraftmenuref 0)))))))

(event `self.InteractiveCollision.OnInteractionAvailableStateUpdate`
  (params (bNewState :type Boolean))
  (bind _childactor (`ChildActorComponent.ChildActor` (`self.InputPrompt_KeyGuide`)))
  ;[1 1 1] 키가이드 표시
  (if bNewState
    (`self.SetActorHiddenInGame` _childactor false)
    (else
      (`self.SetActorHiddenInGame` _childactor true))))

(fn `UserConstructionScript`)