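; Crafting manager component that lets the main character craft skills from material items.
; Resetting refills the candidate ID list with random craftable skills, up to the maximum slot count.
; On craft confirmation with a valid skill ID and enough material in the inventory, it removes that candidate, consumes the material and asks the skill manager to add the skill.
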(event `ResetCraftCandidateIDList`
  (set `self.CraftCandidateIDList` (`self.GetRandomCraftableSkillIdx` (`self.MaxCraftSlotCount`))))

(event `self.OnCraftConfirmed`
  (params (SkillInfo :type "SkillInfo Structure"))
  (bind (_skillid _skillname _iconimage _skilldescription _skillsubdescription _skillanimation _bcontainprevaction _prevactionclass _bislifespanwithcauser _bisplayerskill _materialid _materialcount) (break `SkillInfo` SkillInfo))
  (bind _returnvalue__ (`/Game/UI/Global/BPFL_CommonWidget.GetMainCharacterRef`))
  (bind _iteminventory (`MainCharacterBase.ItemInventory` _returnvalue__))
  ;[1 1 1] 크래프팅 이후, 아이템을 제거하고 스킬을 추가한다.
  (if (!= _skillid 0)
    (if (>= (`ItemInventoryComponent.GetItemAmount` _iteminventory _materialid) _materialcount)
      (`KismetArrayLibrary.Array_RemoveItem` (`self.CraftCandidateIDList`) _skillid)
      (`ItemInventoryComponent.RemoveItem` _iteminventory _materialid (`KismetMathLibrary.Conv_IntToByte` _materialcount))
      (`SkillManagerComponentBase.TryAddSkill` (`/Game/UI/Global/BPFL_CommonWidget.GetSkillManagerRef` _returnvalue__) (`.SkillID` (break `SkillInfo` SkillInfo))))))