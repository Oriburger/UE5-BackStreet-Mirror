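; Base crafting box actor that opens a crafting UI for the player and exposes its crafting recipe through a getter.
; Overlapping its volume toggles an interaction prompt (Press F), and its Widget component is hidden unless the actor is tagged Tutorial.
; EnterUI creates WB_CraftingTMP with itself as source, switches input to Game and UI, and nearly freezes time through global time dilation.
; A DoOnce gate blocks re-entry until WidgetClosed resets it.
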(event `self.ReceiveBeginPlay`
  (`parent.ReceiveBeginPlay`)
  (if (not (`self.ActorHasTag` "Tutorial"))
    (`SceneComponent.SetVisibility` (`self.Widget`) false false)))

(event `self.OverlapVolume.OnComponentBeginOverlap`
  (params (OverlappedComponent :type "PrimitiveComponent Object Reference") (OtherActor :type "Actor Object Reference") (OtherComp :type "PrimitiveComponent Object Reference") (OtherBodyIndex :type Integer) (bFromSweep :type Boolean) (SweepResult :type "HitResult Structure (by ref)"))
  ;[1 1 1] Press F 팝업 문구 호출
  (`self.VisibleGuideTextRender` OtherActor))

(event `self.OverlapVolume.OnComponentEndOverlap`
  (params (OverlappedComponent :type "PrimitiveComponent Object Reference") (OtherActor :type "Actor Object Reference") (OtherComp :type "PrimitiveComponent Object Reference") (OtherBodyIndex :type Integer))
  ;[1 1 1] Press F 팝업 문구 제거
  (`self.InVisibleGuideTextRender` OtherActor))

(event `self.EnterUI`
  (params (Causer :type "Actor Object Reference"))
  ;[1 1 1] Press F 팝업 문구 제거
  (`/Engine/EditorBlueprintResources/StandardMacros.DoOnce` false :!label _label
    (:`Completed`
      (`/Engine/EditorBlueprintResources/StandardMacros.IsValid` null
        (:`Is Not Valid`
          (if (`self.ActorHasTag` Causer "Player")
            (bind _returnvalue (`|CreateWidget` "/Game/UI/InGame/Blueprint/Component/Crafting/WB_CraftingTMP.WB_CraftingTMP_C" (`GameplayStatics.GetPlayerController` 0)))
            (bind _output_get (set `self.CraftingWidget` _returnvalue))
            (`/Game/UI/InGame/Blueprint/Component/Crafting/WB_CraftingTMP.Initialize` _output_get self)
            (`GameplayStatics.SetGlobalTimeDilation` 0.001)
            (`WidgetBlueprintLibrary.SetInputMode_GameAndUIEx` (`GameplayStatics.GetPlayerController` 0) _output_get "DoNotLock" false)
            (`UserWidget.AddToViewport` _output_get 0)))))))

(event `WidgetClosed`
  ;[1 1 1] Press F 팝업 문구 제거
  (set `self.CraftingWidget` (`self.CraftingWidget`))
  (goto _label :!via `Reset`))

(fn `GetCraftingRecipe`
  (returns (NewParam :type "Array of /Game/Weapon/Data/CraftingRecipe/F_CraftingRecipe Structure"))
  (return (`self.CraftingRecipe`)))

(fn `UserConstructionScript`
  (`SceneComponent.SetVisibility` (`self.TextRenderComp`) true false))