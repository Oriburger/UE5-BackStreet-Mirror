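; Game mode for BackStreet that starts in-game sessions, spawns the chapter manager, and drives combat, minimap and chapter-end UI.
; StartGame builds the combat UI and minimap, while FinishChapter slows time before showing game-over or clear widgets.
; A tutorial checklist combines per-tick input polling with character, inventory and tagged reward-box delegates.
; When every mission is done, TutoClear activates the gate, hides the mission UI and unbinds those delegates.
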(event `self.ReceiveTick`
  (params (DeltaSeconds :type "Float (single-precision)"))
  (if (`self.IsTutorial`)
    (`self.CheckTuto`)))

(event `self.FinishChapter`
  (params (bGameIsOver :type Boolean))
  (bind _returnvalue (`GameplayStatics.GetPlayerController` 0))
  ;[1 0.7981 0.2486] BP_ ImplementableEvent
  ;;[1 1 1] 챕터 종료 로직
  (`GameplayStatics.SetGlobalTimeDilation` 0.25)
  (`KismetSystemLibrary.Delay` 0.5)
  (if bGameIsOver
    (bind _returnvalue_2 (`|CreateWidget` "/Game/UI/InGame/Blueprint/WB_GameOver.WB_GameOver_C" _returnvalue))
    (`UserWidget.AddToViewport` _returnvalue_2 0)
    (else
      (bind _returnvalue_3 (`|CreateWidget` "/Game/UI/InGame/Blueprint/WB_GameClear.WB_GameClear_C" _returnvalue))
      (`UserWidget.AddToViewport` _returnvalue_3 0))))

(event `self.FadeOut`
  ;[1 0.7981 0.2486] BP_ ImplementableEvent
  ;;[1 1 1] UI
  (`/Game/UI/InGame/Blueprint/WB_CombatUI.PlayFadeOutAnimation` (`self.CombatUI`)))

(event `self.PopUpClearUI`
  ;[1 0.7981 0.2486] BP_ ImplementableEvent
  ;;[1 1 1] UI
  (`/Game/UI/InGame/Blueprint/WB_CombatUI.PlayPopUpAnimation` (`self.CombatUI`)))

(event `self.SetMiniMapUI`
  ;[1 0.7981 0.2486] BP_ ImplementableEvent
  ;;[1 1 1] UI
  (bind _returnvalue (`self.GetChapterManagerRef`))
  (`/Game/UI/InGame/Blueprint/Component/WB_MiniMap.Set Stage Map` (`self.MiniMapUI`) _returnvalue))

(event `self.UpdateMiniMapUI`
  ;[1 0.7981 0.2486] BP_ ImplementableEvent
  ;;[1 1 1] UI
  (bind _returnvalue (`self.GetChapterManagerRef`))
  (bind _returnvalue_2 (`ChapterManagerBase.GetCurrentStage` _returnvalue))
  (`/Game/UI/InGame/Blueprint/Component/WB_MiniMap.UpdateCurTile` (`self.MiniMapUI`) _returnvalue_2))

(event `self.CreateChapterManager`
  ;[1 0.7981 0.2486] BP_ ImplementableEvent
  (bind _returnvalue (`|SpawnActorFromClass` "/Game/System/StageManager/Blueprint/BP_ChapterManager.BP_ChapterManager_C" (`KismetMathLibrary.MakeTransform` (0.0 0.0 0.0)) "AlwaysSpawn" "OverrideRootScale" self null))
  (bind _output_get (set `self.ChapterManager` _returnvalue))
  (`ChapterManagerBase.CreateChapterManager` _output_get))

(event `RemoveMissionUI`
  (bind _wb_tutomission (`/Game/UI/InGame/Blueprint/WB_CombatUI.WB_TutoMission` (`self.CombatUI`)))
  ;[1 0.7981 0.2486] BP_ ImplementableEvent
  (`|PlayAnimation` _wb_tutomission (`/Game/UI/InGame/Blueprint/Component/Tutorial/WB_TutoMission.ClearRemove` _wb_tutomission)
    (:`Finished`
      (`Widget.SetVisibility` _wb_tutomission "Hidden"))))

(event `AchieveTutoAttack`
  ;[1 0.7981 0.2486] BP_ ImplementableEvent
  (`self.TutoClear` 5))

(event `AchieveTutoAbility`
  ;[1 0.7981 0.2486] BP_ ImplementableEvent
  (`self.TutoClear` 3))

(event `AchieveTutoWeapon`
  ;[1 0.7981 0.2486] BP_ ImplementableEvent
  (`self.TutoClear` 4))

(event `AchieveTutoWeaponSwap`
  ;[1 0.7981 0.2486] BP_ ImplementableEvent
  (`self.TutoClear` 6))

(event `AchieveTutoWeaponDrop`
  ;[1 0.7981 0.2486] BP_ ImplementableEvent
  (`self.TutoClear` 7))

(fn `BindTutoDelegate`
  (bind _asbp_main_character (cast `/Game/Character/MainCharacter/BP_MainCharacter` (`GameplayStatics.GetPlayerCharacter` 0)))
  (add `MainCharacterBase.OnAttack` _asbp_main_character (`|CreateDelegate` :!event `AchieveTutoAttack`))
  (bind _returnvalue (`CharacterBase.GetInventoryRef` _asbp_main_character))
  (add `WeaponInventoryBase.OnAddWeapon` _returnvalue (`|CreateDelegate` :!event `AchieveTutoWeapon`))
  (add `WeaponInventoryBase.OnDropWeapon` _returnvalue (`|CreateDelegate` :!event `AchieveTutoWeaponDrop`))
  (add `WeaponInventoryBase.OnSwapWeapon` _returnvalue (`|CreateDelegate` :!event `AchieveTutoWeaponSwap`))
  (bind _outactors (`GameplayStatics.GetAllActorsOfClassWithTag` "/Game/Item/Blueprint/RewardBox/BP_RewardBox.BP_RewardBox_C" "Tuto"))
  (for _array_element _outactors
    (add `RewardBoxBase.OnAddAbility` _array_element (`|CreateDelegate` :!event `AchieveTutoAbility`))))

(fn `CheckTuto`
  (bind _returnvalue (`GameplayStatics.GetPlayerController` 0))
  (`|ExecutionSequence`
    (:`then_0`
      (if (or (`PlayerController.WasInputKeyJustPressed` _returnvalue "W") (`PlayerController.WasInputKeyJustPressed` _returnvalue "A") (`PlayerController.WasInputKeyJustPressed` _returnvalue "S") (`PlayerController.WasInputKeyJustPressed` _returnvalue "D"))
        (`self.TutoClear` 0)))
    (:`then_1`
      (if (`PlayerController.WasInputKeyJustPressed` (`GameplayStatics.GetPlayerController` 0) "MouseWheelAxis")
        (`self.TutoClear` 1)))
    (:`then_2`
      (if (`PlayerController.WasInputKeyJustPressed` (`GameplayStatics.GetPlayerController` 0) "LeftShift")
        (`self.TutoClear` 2)))))

(fn `GateOn`
  (bind _returnvalue (`GameplayStatics.GetActorOfClass` "/Game/System/StageManager/Blueprint/BP_Gate.BP_Gate_C"))
  (if (`self.ActorHasTag` _returnvalue "Off")
    (`KismetArrayLibrary.Array_RemoveItem` (`Actor.Tags` _returnvalue) "Off")
    (`GateBase.ActivateNormalGate` _returnvalue)))

(fn `StartGame`
  (if (`self.bIsInGame`)
    (`GameplayStatics.PlaySound2D` "/Game/Map/MainMenu/Sound/SQ_InGame.SQ_InGame" 1.0 1.0 0.0 null null)
    (bind _returnvalue (`|CreateWidget` "/Game/UI/InGame/Blueprint/WB_CombatUI.WB_CombatUI_C" (`GameplayStatics.GetPlayerController` 0)))
    (set `self.CombatUI` _returnvalue)
    (bind _output_get (set `self.MiniMapUI` (`/Game/UI/InGame/Blueprint/WB_CombatUI.GetMiniMapWidgetRef` _returnvalue)))
    (`self.InitializeGame`)
    (bind _returnvalue_2 (`self.GetChapterManagerRef`))
    (`/Game/UI/InGame/Blueprint/Component/WB_MiniMap.SetChapterManager` _output_get _returnvalue_2)
    (`/Game/UI/InGame/Blueprint/Component/WB_MiniMap.SetAnimMap` _output_get)
    (`self.SetMiniMapUI`)
    (`self.UpdateMiniMapUI`)
    (`/Game/UI/InGame/Blueprint/WB_CombatUI.Initialize` _returnvalue self)
    (`self.BindTutoDelegate`)
    (`UserWidget.AddToViewport` _returnvalue 0)))

(fn `TutoClear`
  (params (Num :type Integer))
  (`/Game/UI/InGame/Blueprint/Component/Tutorial/WB_TutoMission.Update Image` (`/Game/UI/InGame/Blueprint/WB_CombatUI.WB_TutoMission` (`self.CombatUI`)) Num)
  (set `self.IsTutoClear` true)
  (for _array_element (`/Game/UI/InGame/Blueprint/Component/Tutorial/WB_TutoMission.List` (`/Game/UI/InGame/Blueprint/WB_CombatUI.WB_TutoMission` (`self.CombatUI`)))
    (if (not _array_element)
      (set `self.IsTutoClear` false)
      (break)))
  (if (`self.IsTutoClear`)
    (`KismetSystemLibrary.PrintString` "Clear")
    (set `self.IsTutorial` false)
    (`self.GateOn`)
    (`self.RemoveMissionUI`)
    (`self.UnBindTutoDelegate`)))

(fn `UnBindTutoDelegate`
  (bind _asbp_main_character (cast `/Game/Character/MainCharacter/BP_MainCharacter` (`GameplayStatics.GetPlayerCharacter` 0)))
  (clear `MainCharacterBase.OnAttack` _asbp_main_character)
  (bind _returnvalue (`CharacterBase.GetInventoryRef` _asbp_main_character))
  (clear `WeaponInventoryBase.OnAddWeapon` _returnvalue)
  (clear `WeaponInventoryBase.OnSwapWeapon` _returnvalue)
  (clear `WeaponInventoryBase.OnDropWeapon` _returnvalue)
  (bind _outactors (`GameplayStatics.GetAllActorsOfClassWithTag` "/Game/Item/Blueprint/RewardBox/BP_RewardBox.BP_RewardBox_C" "Tuto"))
  (for _array_element _outactors
    (clear `RewardBoxBase.OnAddAbility` _array_element)))

(fn `UserConstructionScript`)