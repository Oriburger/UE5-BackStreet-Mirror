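; Base ability item that, when picked, offers the player a choice of random abilities through a reward selection UI.
; Pickup requests three random abilities of its AbilityType from the main character's AbilityManagerComponent, passes them to WB_UI_RewardSelect, then destroys the item without calling the parent logic.
; Items spawned with a valid owner pick themselves automatically after a short delay.
; The construction script writes ItemIDOverride into the item info.
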(event `self.ReceiveBeginPlay`
  (`parent.ReceiveBeginPlay`)
  (`KismetSystemLibrary.DelayUntilNextTick`)
  (`/Engine/EditorBlueprintResources/StandardMacros.IsValid` (`self.GetOwner`)
    (:`Is Valid`
      ;[1 1 1] Force Pick Item
      (`KismetSystemLibrary.Delay` 1.5)
      (`self.OnItemPicked`))))

(event `self.OnItemPicked`
  ;[1 1 1] On ItemPicked / 부모 호출하지 않음
  (bind _output_get (set `self.RandomAbilityInfoList` (`AbilityManagerComponent.GetRandomAbilityInfoList` (`MainCharacterBase.AbilityManagerComponent` (`/Game/UI/Global/BPFL_CommonWidget.GetMainCharacterRef`)) 3 (`|MakeArray` (`self.AbilityType`)))))
  (if (`KismetArrayLibrary.Array_IsNotEmpty` _output_get)
    (bind _widgetref (`/Game/EasyGameUI/Core/BFL_EasyFunctionUtilities.SafeCreateWidget` "/Game/UI/InGame/Blueprint/RewardUI/WB_UI_RewardSelect.WB_UI_RewardSelect_C"))
    (bind _aswb_ui_reward_select (cast `/Game/UI/InGame/Blueprint/RewardUI/WB_UI_RewardSelect` _widgetref)
      (:`then`
        (`/Game/UI/InGame/Blueprint/RewardUI/WB_UI_RewardSelect.Initialize` _aswb_ui_reward_select (`self.RandomAbilityInfoList`)))
      (:`CastFailed`
        _)))
  (`self.K2_DestroyActor`))

(fn `UserConstructionScript`
  (setmembers `ItemInfoDataStruct` :`StructRef` (`self.ItemInfo`) :`ItemID` (`self.Item ID Override`))
  (`parent.UserConstructionScript`))