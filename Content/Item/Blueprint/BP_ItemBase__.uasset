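; Base item Blueprint that initializes itself from an item data table and presents itself when activated.
; BeginPlay waits briefly, then passes a hardcoded ItemDataInfoTable row to InitItem; LoadMesh async-loads the main mesh asset onto the mesh component.
; ActivateItem enables physics on the root collision after a delay, then runs a scale timeline that triggers the particle effect once.
; A mesh rotation timeline exists but is disconnected.
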(event `self.ActivateItem`
  ;[1 0.6249 0.4631 1 36] BP_Implementable
  (`|ExecutionSequence`
    (:`then_0`
      (`KismetSystemLibrary.Delay` 0.25)
      (`PrimitiveComponent.SetSimulatePhysics` (`self.RootCollisionVolume`) true))
    (:`then_1`
      (`KismetSystemLibrary.Delay` 0.5)
      (bind (_direction _scale) (`Timeline|타임라인_0`)
        (:`Update`
          (`self.SetActorScale3D` (`KismetMathLibrary.Conv_DoubleToVector` _scale))
          (`/Engine/EditorBlueprintResources/StandardMacros.DoOnce` false
            (:`Completed`
              (`ActorComponent.Activate` (`self.ParticleComponent`) false))))))))

(event `self.ReceiveBeginPlay`
  (`parent.ReceiveBeginPlay`)
  (`KismetSystemLibrary.Delay` 3.0)
  (bind _returnvalue (`|GetDataTableRow` (`self.ItemDataInfoTable`) "31100")
    (:`then`
      (`self.InitItem` _returnvalue))))

(event `LoadMesh`
  (bind _object (`|LoadAsset` (`self.MainMeshAsset`))
    (:`Completed`
      (bind `_as스태틱_메시` (cast `StaticMesh` _object))
      (bind _returnvalue (`StaticMeshComponent.SetStaticMesh` (`self.MeshComponent`) `_as스태틱_메시`))
      (if _returnvalue
        (`KismetSystemLibrary.PrintString` "Load Done!")))))

(fn `UserConstructionScript`)