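; Base Blueprint for projectile pickup items that give a player ammo for a weapon, or the weapon itself if it is a throwable.
; On pickup, a macro validates the player-tagged causer and its inventory, then ammo is added if the weapon is held.
; Unowned throwables are picked up as weapons; other types show a "pick up the matching weapon first" message.
; Success plays effect and sound, then destroys the actor; DoOnce guards reset on failure.
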(event `self.OnItemPicked`
  (params (Causer :type "Actor Object Reference"))
  (bind _itemid (`self.ItemID`))
  (bind _asbp_back_street_game_mode (cast `/Game/BP_BackStreetGameMode` (`GameplayStatics.GetGameMode`) :!pure true))
  ;[1 0.2846 0.4761 1 35] BP_ImplementableEvent
  (`/Engine/EditorBlueprintResources/StandardMacros.IsValid` Causer
    (:`Is Valid`
      (if (`self.ActorHasTag` Causer "Player")
        (bind _asmain_character_base (cast `MainCharacterBase` Causer))
        (bind _returnvalue (`CharacterBase.GetInventoryRef` _asmain_character_base))
        (`/Engine/EditorBlueprintResources/StandardMacros.IsValid` _returnvalue
          (:`Is Valid`
            (bind _returnvalue_2 (`WeaponInventoryBase.GetWeaponIsContained` _returnvalue _itemid))
            (if _returnvalue_2
              (`/Engine/EditorBlueprintResources/StandardMacros.DoOnce` false :!label _label
                (:`Completed`
                  (bind _returnvalue_3 (`WeaponInventoryBase.TryAddAmmoToWeapon` _returnvalue _itemid (`self.AmmoCount`)))
                  (if _returnvalue_3
                    (`NiagaraFunctionLibrary.SpawnSystemAtLocation` (`self.EndEffect`) (`self.K2_GetActorLocation`) (struct :`Yaw` 90.0) :!label _label_2)
                    (`GameplayStatics.PlaySound2D` (`self.PickSound`) 1.0 1.0 0.0 null null)
                    (`self.K2_DestroyActor`)
                    (else
                      (goto _label :!via `Reset`)))))
              (elif (`|EnumEquality` (`.WeaponType` (break `WeaponStatStruct` (`BackStreetGameModeBase.GetWeaponStatInfoWithID` _asbp_back_street_game_mode _itemid))) "E_Throw")
                (`/Engine/EditorBlueprintResources/StandardMacros.DoOnce` false :!label _label_3
                  (:`Completed`
                    (bind _returnvalue_4 (`CharacterBase.PickWeapon` _asmain_character_base _itemid))
                    (if _returnvalue_4
                      (goto _label_2)
                      (else
                        (goto _label_3 :!via `Reset`)))))
                (else
                  (`BackStreetGameModeBase.PrintSystemMessageDelegate` _asbp_back_street_game_mode "탄환에 맞는 무기를 먼저 주워주세요" (make `Color` 255 255 255 255)))))))))))

(fn `UserConstructionScript`
  (`parent.UserConstructionScript`))