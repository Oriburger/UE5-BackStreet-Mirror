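; Heal pack pickup that heals the main character when picked up, or on player overlap if AutoActivate is set, then destroys itself.
; Base heal comes from HealAmountOverride or a grade keyword match on the item name.
; GetAbilityValueUsingProbability supplies a multiplier, re-called separately for the debug print, heal and effect choice.
; Heal size selects a small, medium or large Niagara effect, played with a sound.
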(event `self.ReceiveBeginPlay`
  (bind _previewicon (`self.PreviewIcon`))
  ;[1 1 1] Re-Init icon to preview icon
  (`self.SetComponentIcon` (`self.IconWidgetComponent`) _previewicon)
  (`self.SetComponentIcon` (`self.Icon Widget Component _ back`) _previewicon))

(event `self.OnItemPicked`
  (bind _returnvalue__ (`/Game/UI/Global/BPFL_CommonWidget.GetMainCharacterRef`))
  (bind _returnvalue (* (`self.GetHealAmount`) (`KismetMathLibrary.SelectFloat` (`CharacterBase.GetStatTotalValue` _returnvalue__ "E_HealItemPerformance") 1.0 (>= (`CharacterBase.GetStatProbabilityValue` _returnvalue__ "E_HealItemPerformance") (`KismetMathLibrary.RandomFloatInRange` 0.0 1.0)))))
  ;[1 1 1] Apply Item Effect
  (`/Engine/EditorBlueprintResources/StandardMacros.IsValid` _returnvalue__
    (:`Is Valid`
      (`KismetSystemLibrary.PrintString` (`KismetStringLibrary.Conv_DoubleToString` _returnvalue))
      (`CharacterBase.TakeHeal` _returnvalue__ _returnvalue false 0)
      (`NiagaraFunctionLibrary.SpawnSystemAttached` (`self.GetHealNiagaraSystem` _returnvalue) (`Actor.RootComponent` _returnvalue__) "None" (0.0 0.0 -50.0) (struct) "KeepRelativeOffset" true)
      (`GameplayStatics.PlaySoundAtLocation` (`self.ActivateSound`) (`self.K2_GetActorLocation` _returnvalue__) (struct) 1.0 1.0 0.0 "/Game/System/Sound/SA_Common.SA_Common" null _returnvalue__ null)
      (`self.K2_DestroyActor`))))

(event `self.ItemTriggerVolume.OnComponentBeginOverlap`
  (params (OverlappedComponent :type "PrimitiveComponent Object Reference") (OtherActor :type "Actor Object Reference") (OtherComp :type "PrimitiveComponent Object Reference") (OtherBodyIndex :type Integer) (bFromSweep :type Boolean) (SweepResult :type "HitResult Structure (by ref)"))
  ;[1 1 1] Set Player Ref
  (`/Engine/EditorBlueprintResources/StandardMacros.IsValid` OtherActor
    (:`Is Valid`
      (if (`self.ActorHasTag` OtherActor "Player")
        (if (`self.bAutoActivate`)
          (`self.OnItemPicked`))))))

(fn `GetHealAmount`
  (returns (Result :type "Float (double-precision)"))
  (bind _healamountoverride (`self.HealAmountOverride`))
  (bind _healvaluelistpergrade (`self.HealValueListPerGrade`))
  (bind _returnvalue (`KismetStringLibrary.Conv_NameToString` (`.ItemName` (break `ItemInfoDataStruct` (`self.ItemInfo`)))))
  ;[1 1 1] Override
  (if (<= _healamountoverride 0.0)
    (`KismetSystemLibrary.PrintString` _returnvalue)
    ;[1 1 1] 검사
    (for (_array_element _array_index) (`self.HealItemGradeKeywordList`)
      (if (`KismetStringLibrary.Contains` _returnvalue _array_element)
        (if (`KismetArrayLibrary.Array_IsValidIndex` _healvaluelistpergrade _array_index)
          (return (`|GetArrayItem` _healvaluelistpergrade _array_index)))))
    (return 0.1)
    (else
      (return _healamountoverride))))

(fn `GetHealNiagaraSystem`
  (params (HealAmount :type "Float (double-precision)"))
  (returns (ActivateEffect :type "NiagaraSystem Object Reference"))
  (if (<= HealAmount 25.0)
    (return "/Game/VFX/FX/Character/Item/NS_Healing_Small.NS_Healing_Small")
    (elif (<= HealAmount 55.0)
      (return "/Game/VFX/FX/Character/Item/NS_Healing_Medium.NS_Healing_Medium")
      (else
        (return "/Game/VFX/FX/Character/Item/NS_Healing_Large.NS_Healing_Large")))))

(fn `UserConstructionScript`
  (`parent.UserConstructionScript`))