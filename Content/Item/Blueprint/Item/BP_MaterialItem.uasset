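; BP_MaterialItem is a child item Blueprint for a material pickup the player collects by touching it.
; Overlap of its trigger volume by a Player-tagged actor attaches a pickup Niagara effect to the overlapping component, plays an obtain sound and calls OnItemPicked.
; OnItemPicked runs once, waiting briefly before handing off to the parent's pickup logic.
; A homing-projectile fly-to-player sequence remains in the graph but is disconnected and never runs.
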(event `self.OnItemPicked`
  (`/Engine/EditorBlueprintResources/StandardMacros.DoOnce` false
    (:`Completed`
      (`KismetSystemLibrary.Delay` 0.2)
      (`parent.OnItemPicked`))))

(event `self.ItemTriggerVolume.OnComponentBeginOverlap`
  (params (OverlappedComponent :type "PrimitiveComponent Object Reference") (OtherActor :type "Actor Object Reference") (OtherComp :type "PrimitiveComponent Object Reference") (OtherBodyIndex :type Integer) (bFromSweep :type Boolean) (SweepResult :type "HitResult Structure (by ref)"))
  (`/Engine/EditorBlueprintResources/StandardMacros.IsValid` OtherActor
    (:`Is Valid`
      (if (`self.ActorHasTag` OtherActor "Player")
        (`NiagaraFunctionLibrary.SpawnSystemAttached` "/Game/VFX/FX/Character/Item/NS_Pick_Up_End.NS_Pick_Up_End" OtherComp "None" (0.0 0.0 20.0) (struct) "KeepRelativeOffset" true)
        (`GameplayStatics.PlaySoundAtLocation` "/Game/Sound/SW_Login_interaction/SW_Login_interaction_Craft_Obtain.SW_Login_interaction_Craft_Obtain" (`self.K2_GetActorLocation`) (struct) 1.0 1.0 0.0 null null null null)
        (`self.OnItemPicked`)))))

(fn `UserConstructionScript`
  (`parent.UserConstructionScript`))