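; BP_ItemBox_WeaponOnly is an item box variant, named as weapon-only, that adds tutorial highlighting on top of its parent's behavior.
; On BeginPlay it hides its widget unless the actor has the "Tuto" tag.
; For tagged boxes, a Player-tagged actor entering the overlap volume starts the WB_WorldActorTuto widget's endlessly looping Blink animation, and leaving stops it.
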(event `self.ReceiveBeginPlay`
  (`parent.ReceiveBeginPlay`)
  (if (not (`self.ActorHasTag` "Tuto"))
    (`SceneComponent.SetVisibility` (`self.Widget`) false false)))

(event `self.OverlapVolume.OnComponentBeginOverlap`
  (params (OverlappedComponent :type "PrimitiveComponent Object Reference") (OtherActor :type "Actor Object Reference") (OtherComp :type "PrimitiveComponent Object Reference") (OtherBodyIndex :type Integer) (bFromSweep :type Boolean) (SweepResult :type "HitResult Structure (by ref)"))
  (bind _returnvalue (`WidgetComponent.GetWidget` (`self.Widget`)))
  (if (`self.ActorHasTag` "Tuto")
    (`/Engine/EditorBlueprintResources/StandardMacros.IsValid` OtherActor
      (:`Is Valid`
        (if (`self.ActorHasTag` OtherActor "Player")
          (bind _aswb_world_actor_tuto (cast `/Game/UI/InGame/Blueprint/Component/Tutorial/WB_WorldActorTuto` _returnvalue))
          (`UserWidget.PlayAnimation` _returnvalue (`/Game/UI/InGame/Blueprint/Component/Tutorial/WB_WorldActorTuto.Blink` _aswb_world_actor_tuto) 0.0 0 "Forward" 1.0 false))))))

(event `self.OverlapVolume.OnComponentEndOverlap`
  (params (OverlappedComponent :type "PrimitiveComponent Object Reference") (OtherActor :type "Actor Object Reference") (OtherComp :type "PrimitiveComponent Object Reference") (OtherBodyIndex :type Integer))
  (if (`self.ActorHasTag` "Tuto")
    (`/Engine/EditorBlueprintResources/StandardMacros.IsValid` OtherActor
      (:`Is Valid`
        (if (`self.ActorHasTag` OtherActor "Player")
          (bind _aswb_world_actor_tuto (cast `/Game/UI/InGame/Blueprint/Component/Tutorial/WB_WorldActorTuto` (`WidgetComponent.GetWidget` (`self.Widget`))))
          (`UserWidget.StopAnimation` _aswb_world_actor_tuto (`/Game/UI/InGame/Blueprint/Component/Tutorial/WB_WorldActorTuto.Blink` _aswb_world_actor_tuto)))))))

(fn `UserConstructionScript`
  (`parent.UserConstructionScript`))