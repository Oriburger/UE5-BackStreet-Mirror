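; Base pickup item Blueprint that displays an item in the world and adds it to the main character's inventory when picked up.
; Construction initializes from ItemID and shows front and back preview icon widgets when no mesh is set.
; On activation, timelines animate scale and tilted yaw on meshed items with particles, or rotate the icon display otherwise.
; Sub-weapons grant a quarter of their data-table max ammo; other items grant one.
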(event `self.ReceiveBeginPlay`
  (`parent.ReceiveBeginPlay`))

(event `self.ActivateItem`
  (bind _meshcomponent (`self.MeshComponent`))
  ;[1 0.6249 0.4631 1 36] BP_Implementable
  (`|ExecutionSequence`
    (:`then_0`
      (`/Engine/EditorBlueprintResources/StandardMacros.IsValid` _meshcomponent
        (:`Is Valid`
          (`/Engine/EditorBlueprintResources/StandardMacros.IsValid` (`StaticMeshComponent.StaticMesh` _meshcomponent)
            (:`Is Valid`
              ;;[1 1 1] StaticMesh
              (`|ExecutionSequence`
                (:`then_0`
                  (`KismetSystemLibrary.Delay` 0.5)
                  (bind (_direction _scale) (`Timeline|타임라인_0`)
                    (:`Update`
                      (`self.SetActorScale3D` (`KismetMathLibrary.Conv_DoubleToVector` _scale))
                      (`/Engine/EditorBlueprintResources/StandardMacros.DoOnce` false
                        (:`Completed`
                          (`ActorComponent.Activate` (`self.ParticleComponent`) false))))))
                (:`then_1`
                  (`SceneComponent.K2_SetWorldRotation` (`self.MeshComponent`) (struct :`Pitch` 45.0 :`Yaw` 45.0) false false)
                  (bind (_direction_2 `_새_트랙_0`) (`Timeline|타임라인_1`)
                    (:`Update`
                      (`SceneComponent.K2_SetWorldRotation` (`self.MeshComponent`) (`KismetMathLibrary.MakeRotator` 0.0 45.0 `_새_트랙_0`) false false))))
                (:`then_2`
                  (`SceneComponent.SetHiddenInGame` (`self.IconWidgetComponent`) true false)
                  (`SceneComponent.SetHiddenInGame` (`self.Icon Widget Component _ back`) true false))))
            (:`Is Not Valid`
              ;;[1 1 1] Icon
              (`SceneComponent.SetHiddenInGame` (`self.IconWidgetComponent`) false false :!label _label)
              (`SceneComponent.SetHiddenInGame` (`self.Icon Widget Component _ back`) false false)
              (bind (_direction_3 `_새_트랙_0_2`) (`Timeline|타임라인`)
                (:`Update`
                  (`SceneComponent.K2_SetWorldRotation` (`self.MeshComponent`) (`KismetMathLibrary.MakeRotator` 0.0 0.0 `_새_트랙_0_2`) false false))))))
        (:`Is Not Valid`
          (goto _label))))
    (:`then_1`
      (`NiagaraComponent.ResetSystem` (`self.ParticleComponent`)))))

(event `self.OnItemPicked`
  (bind _returnvalue__ (`/Game/UI/Global/BPFL_CommonWidget.GetMainCharacterRef`))
  (bind ((`ItemID` _itemid) (`ItemType` _itemtype)) (break `ItemInfoDataStruct` (`self.ItemInfo`)))
  (`/Engine/EditorBlueprintResources/StandardMacros.IsValid` _returnvalue__
    (:`Is Valid`
      (`ItemInventoryComponent.AddItem` (`MainCharacterBase.ItemInventory` _returnvalue__) _itemid (select `bool` (`|EnumEquality` _itemtype "E_SubWeapon") :`false` 1 :`true` (`KismetMathLibrary.Conv_IntToByte` (`self.GetDefaultAmmoCount` _itemid)))))
    (:`Is Not Valid`
      _))
  (`parent.OnItemPicked`))

(fn `GetDefaultAmmoCount`
  (params (ItemID :type Integer))
  (returns (`Max Ammo Per Magazine` :type Integer))
  (bind _returnvalue (`|GetDataTableRow` "/Game/Weapon/Data/D_WeaponStatTable.D_WeaponStatTable" (`KismetStringLibrary.Conv_StringToName` (`KismetStringLibrary.Conv_IntToString` (- ItemID 20000))))
    (:`then`
      (return (`KismetMathLibrary.Round` (* (`KismetMathLibrary.Conv_IntToDouble` (`.MaxTotalAmmo` (break `RangedWeaponStatStruct` (`.RangedWeaponStat` (break `WeaponStatStruct` _returnvalue))))) 0.25))))
    (:`RowNotFound`
      (return 0))))

(fn `SetComponentIcon`
  (params (WidgetComponent :type "WidgetComponent Object Reference") (Texture :type "Texture2D Object Reference"))
  (bind _returnvalue (`WidgetComponent.GetWidget` WidgetComponent))
  (`/Engine/EditorBlueprintResources/StandardMacros.IsValid` _returnvalue
    (:`Is Valid`
      (bind _aswb_item_icon (cast `/Game/Item/Widget/WB_ItemIcon` _returnvalue))
      (`/Game/Item/Widget/WB_ItemIcon.InitIcon` _aswb_item_icon Texture))))

(fn `UserConstructionScript`
  (bind _previewicon (`self.PreviewIcon`))
  (bind (_itemid _itemname _itemlifetype _itemtype _bisactoritem _itemclass _itemmesh) (break `ItemInfoDataStruct` (`self.ItemInfo`)))
  (bind _returnvalue (`KismetSystemLibrary.IsValidSoftObjectReference` _itemmesh))
  (`self.InitItem` _itemid (struct :`ItemLifeType` "E_None" :`ItemType` "E_None" :`InitialLocation` (0.0 0.0 0.0) :`InitialRotation` (struct) :`InitialScale` (0.0 0.0 0.0)))
  (`SceneComponent.SetVisibility` (`self.IconWidgetComponent`) (not _returnvalue) false)
  (`SceneComponent.SetVisibility` (`self.Icon Widget Component _ back`) (not _returnvalue) false)
  ;[1 1 1] Preview
  (if (not _returnvalue)
    (`self.SetComponentIcon` (`self.IconWidgetComponent`) _previewicon)
    (`self.SetComponentIcon` (`self.Icon Widget Component _ back`) _previewicon)))