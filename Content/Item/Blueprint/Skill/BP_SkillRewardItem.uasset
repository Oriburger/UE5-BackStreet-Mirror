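; Skill reward pickup that grants the player a skill derived from the last two digits of its item ID.
; On BeginPlay it sets its preview icons, rerolls a "00" ID into a random player skill from the craftable list, then adjusts its height.
; Pickup destroys it if the skill is owned or successfully added via SkillManagerComponent.
; With three or more skills owned, it instead shows a one-time warning banner whose Continue re-runs pickup.
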(event `self.ReceiveBeginPlay`
  (bind _previewicon (`self.PreviewIcon`))
  (bind _skillmanagercomponent (`CharacterBase.SkillManagerComponent` (`/Game/UI/Global/BPFL_CommonWidget.GetMainCharacterRef`)))
  (bind _returnvalue (`SkillManagerComponentBase.GetPlayerSkillIDList` _skillmanagercomponent))
  ;[1 1 1] Re-Init icon to preview icon
  (`parent.ReceiveBeginPlay`)
  (bind _output_get (set `self.PlayerControllerRef` (`GameplayStatics.GetPlayerController` 0)))
  (set `self.ControllerComponent` (`self.GetComponentByClass` _output_get "/Game/EasyGameUI/Core/BP_EGUI_ControllerComponent.BP_EGUI_ControllerComponent_C"))
  (`self.SetComponentIcon` (`self.IconWidgetComponent`) _previewicon)
  (`self.SetComponentIcon` (`self.Icon Widget Component _ back`) _previewicon)
  (`KismetSystemLibrary.Delay` 0.2)
  (if (== (mod (`.ItemID` (break `ItemInfoDataStruct` (`self.ItemInfo`))) 100) 0)
    (if (`KismetArrayLibrary.Array_IsNotEmpty` _returnvalue)
      (bind _output_get_2 (set `self.SkillIDListCopy` _returnvalue))
      (`KismetArrayLibrary.Array_Shuffle` _output_get_2)
      (for _array_element (`self.SkillIDListCopy`)
        (if (`KismetArrayLibrary.Array_Contains` (`SkillManagerComponentBase.GetCraftableIDList` _skillmanagercomponent) _array_element)
          (`self.InitItem` (+ _array_element 10000) (struct :`ItemLifeType` "E_None" :`ItemType` "E_None" :`InitialLocation` (0.0 0.0 0.0) :`InitialRotation` (struct) :`InitialScale` (0.0 0.0 0.0) :`EffectInitialLocation` (0.0 0.0 0.0) :`EffectInitialRotation` (struct)))
          (break)))
      (`self.AdjustItemZLocation`))))

(event `self.OnItemPicked`
  (bind _returnvalue__ (`/Game/UI/Global/BPFL_CommonWidget.GetMainCharacterRef`))
  (bind _skillmanagercomponent (`CharacterBase.SkillManagerComponent` _returnvalue__))
  (bind _returnvalue (`SkillManagerComponentBase.GetOwnedSkillIDList` _skillmanagercomponent))
  (bind _returnvalue_2 (mod (`.ItemID` (break `ItemInfoDataStruct` (`self.ItemInfo`))) 100))
  ;[1 1 1] Apply Item Effect
  (`/Engine/EditorBlueprintResources/StandardMacros.IsValid` _returnvalue__
    (:`Is Valid`
      (if (`KismetArrayLibrary.Array_Contains` _returnvalue _returnvalue_2)
        (`self.K2_DestroyActor` :!label _label)
        (elif (>= (`KismetArrayLibrary.Array_Length` _returnvalue) 3)
          (`/Engine/EditorBlueprintResources/StandardMacros.DoOnce` false
            (:`Completed`
              (`self.ActivateErrorBanner`)))
          (else
            (bind (_bisininventory _returnvalue_3) (`SkillManagerComponentBase.TryAddSkill` _skillmanagercomponent _returnvalue_2))
            (if _returnvalue_3
              (goto _label))))))))

(event `ActivateErrorBanner`
  ;[1 0.5173 0.5272] 슬롯이 꽉 찼다면?
  (bind _bannerwidget (`/Game/EasyGameUI/Core/BP_EGUI_ControllerComponent.SetupAlertBanner` (`self.ControllerComponent`) (`/Game/UI/Global/BPFL_CommonWidget.Get Main HUD Ref`) "Warning" (`|MakeArray` "Button_Continue" "Button_Cancel" :!type "Text") "Automatic" 0 0 "/Game/UI/InGame/Blueprint/Crafting/Component/WB_EGUI_CraftWarningAlertBanner.WB_EGUI_CraftWarningAlertBanner_C"))
  (add `/Game/EasyGameUI/Core/CommonWidgets/WBP_EGUI_CommonAlertBanner.ActionRequested` _bannerwidget (delegate `DeactivateErrorBanner`))
  (`/Game/UI/Global/BPFL_CommonWidget.SetInputModeAndCursorVisibility` _bannerwidget false true))

(event `DeactivateErrorBanner`
  (params (ButtonIndex :type Integer))
  ;[1 0.5173 0.5272] 슬롯이 꽉 찼다면?
  (switch `int` ButtonIndex
    (:`0`
      (`self.OnItemPicked`))
    (:`1`
      _))
  (`/Game/EasyGameUI/Core/BP_EGUI_ControllerComponent.ResetFocusFromAlertBanner` (`self.ControllerComponent`) (stale `ActivateErrorBanner` _bannerwidget) null)
  (`/Game/UI/Global/BPFL_CommonWidget.SetInputModeAndCursorVisibility` (`/Game/UI/Global/BPFL_CommonWidget.Get Main HUD Ref`) true false true))

(fn `ActivateCraftErrorBanner`)

(fn `UserConstructionScript`
  (`parent.UserConstructionScript`))