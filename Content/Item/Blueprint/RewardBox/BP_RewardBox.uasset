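; BP_RewardBox is a reward box that offers an ability and shows it through an info widget.
; Outside the tutorial, it hides its tutorial widget, selects a random ability index on BeginPlay and plays a spawn sound through the global asset manager.
; Widget events initialize the info widget with the ability ID and play its appear animation from the deactivate flag.
; Boxes tagged Tutorial also start or stop a blinking marker.
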(event `self.ReceiveBeginPlay`
  ;[1 1 1] Begin Play
  (`parent.ReceiveBeginPlay`)
  (if (not (`self.ActorHasTag` "Tutorial"))
    (`SceneComponent.SetVisibility` (`self.Widget`) false false)
    (`self.SelectRandomAbilityIdx`)
    (`KismetSystemLibrary.DelayUntilNextTick`)
    (bind _asback_street_game_mode_base (cast `BackStreetGameModeBase` (`GameplayStatics.GetGameMode`)))
    (bind _returnvalue (`BackStreetGameModeBase.GetGlobalAssetManagerBaseRef` _asback_street_game_mode_base))
    (`/Engine/EditorBlueprintResources/StandardMacros.IsValid` _returnvalue
      (:`Is Valid`
        (`AssetManagerBase.PlaySingleSound` _returnvalue self "E_System" 3000 "SpawnAbilityBox" 1.0 1.0 0.0)))))

(event `self.InitializeWidgetComponent`
  ;[1 1 1 1 40] BP_Implementable
  ;;[0.6997 1 0.6008] 위젯 초기화
  (bind _aswb_reward_box_info (cast `/Game/Item/Blueprint/RewardBox/Widget/WB_RewardBoxInfo` (`WidgetComponent.GetWidget` (`self.InfoWidgetComponent`))))
  (`/Game/Item/Blueprint/RewardBox/Widget/WB_RewardBoxInfo.Initialize` _aswb_reward_box_info (`self.AbilityID`)))

(event `self.ActivateWidgetComponent`
  (params (bDeactivateFlag :type Boolean))
  (bind _returnvalue (`WidgetComponent.GetWidget` (`self.Widget`)))
  ;[1 1 1 1 40] BP_Implementable
  ;;[1 0.9395 0.6452] 위젯 활성화
  (if (`self.ActorHasTag` "Tutorial")
    (if bDeactivateFlag
      (bind _aswb_world_actor_tuto (cast `/Game/UI/InGame/Blueprint/Legacy/Component/Tutorial/WB_WorldActorTuto` _returnvalue))
      (`UserWidget.StopAnimation` _aswb_world_actor_tuto (`/Game/UI/InGame/Blueprint/Legacy/Component/Tutorial/WB_WorldActorTuto.Blink` _aswb_world_actor_tuto))
      (else
        (bind _aswb_world_actor_tuto_2 (cast `/Game/UI/InGame/Blueprint/Legacy/Component/Tutorial/WB_WorldActorTuto` _returnvalue))
        (`UserWidget.PlayAnimation` _aswb_world_actor_tuto_2 (`/Game/UI/InGame/Blueprint/Legacy/Component/Tutorial/WB_WorldActorTuto.Blink` _aswb_world_actor_tuto_2) 0.0 0 "Forward" 1.0 false))))
  (bind _aswb_reward_box_info (cast `/Game/Item/Blueprint/RewardBox/Widget/WB_RewardBoxInfo` (`WidgetComponent.GetWidget` (`self.InfoWidgetComponent`))))
  (bind _playlength (`/Game/Item/Blueprint/RewardBox/Widget/WB_RewardBoxInfo.PlayAppearAnimation` _aswb_reward_box_info bDeactivateFlag))
  (`KismetSystemLibrary.Delay` (+ _playlength 0.1)))

(fn `UserConstructionScript`)