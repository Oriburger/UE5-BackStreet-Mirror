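; BP_WeaponItemBase is the base Blueprint for weapon items that the player can pick up.
; When OnItemPicked receives a valid Player-tagged causer, it casts to MainCharacterBase and passes its ItemID to PickWeapon.
; On success it spawns an end effect, plays a 2D pickup sound and destroys itself.
; A DoOnce blocks repeat pickups and resets if the character fails to take the weapon.
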(event `self.OnItemPicked`
  (params (Causer :type "Actor Object Reference"))
  ;[1 0.9696 0.5955 1 36] BP_Implementable
  (`/Engine/EditorBlueprintResources/StandardMacros.IsValid` Causer
    (:`Is Valid`
      (if (`self.ActorHasTag` Causer "Player")
        (bind _asmain_character_base (cast `MainCharacterBase` Causer))
        (`/Engine/EditorBlueprintResources/StandardMacros.DoOnce` false :!label _label
          (:`Completed`
            (bind _returnvalue (`CharacterBase.PickWeapon` _asmain_character_base (`self.ItemID`)))
            (if _returnvalue
              (`NiagaraFunctionLibrary.SpawnSystemAtLocation` (`self.EndEffect`) (`self.K2_GetActorLocation`) (struct :`Yaw` 90.0))
              (`GameplayStatics.PlaySound2D` (`self.PickSound`) 1.0 1.0 0.0 null null)
              (`self.K2_DestroyActor`)
              (else
                (goto _label :!via `Reset`)))))))))

(fn `UserConstructionScript`)