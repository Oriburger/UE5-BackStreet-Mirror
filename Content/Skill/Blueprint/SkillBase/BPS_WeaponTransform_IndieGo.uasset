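; Weapon-transform skill actor (IndieGo) that upgrades the caster's current weapon and damages enemies it touches.
; StartSkill attaches it to the Causer's root and, only for one specific weapon ID, swaps that weapon in the inventory for its transformed version, plays an impact effect, then detaches and hides.
; Box overlaps damage Enemy-tagged characters using the current weapon's melee damage, damage rate and the caster's attack multiplier.
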(event `self.StartSkill`
  (bind _causer (`self.Causer`))
  (bind _ascharacter_base (cast `CharacterBase` _causer))
  (bind _returnvalue (`CharacterBase.GetCurrentWeaponRef` _ascharacter_base))
  (`/Engine/EditorBlueprintResources/StandardMacros.IsValid` _returnvalue
    (:`Is Valid`
      (`self.K2_AttachToActor` _causer "root" "SnapToTarget" "KeepRelative" "KeepRelative")
      (bind _weaponid (`WeaponBase.WeaponID` _returnvalue))
      (if (== _weaponid 12130)
        (bind _returnvalue_2 (`CharacterBase.GetInventoryRef` _ascharacter_base))
        (`WeaponInventoryBase.RemoveWeapon` _returnvalue_2 _weaponid)
        (`WeaponInventoryBase.AddWeapon` _returnvalue_2 12131)
        (bind _ascharacter_base_2 (cast `CharacterBase` (`self.Causer`)))
        (bind _returnvalue_3 (`CharacterBase.GetCurrentWeaponRef` _ascharacter_base_2))
        (`GameplayStatics.SpawnEmitterAtLocation` "/Game/Asset/VFX/RPGEffects/Particles/P_Warrior_HeavyImpact.P_Warrior_HeavyImpact" (`self.K2_GetActorLocation` _returnvalue_3) (`self.K2_GetActorRotation` _returnvalue_3) (`self.GetActorScale3D` _returnvalue_3))
        (`self.K2_DetachFromActor` "KeepRelative")
        (`self.HideSkill`)))))

(event `self.Box.OnComponentBeginOverlap`
  (params (OverlappedComponent :type "PrimitiveComponent Object Reference") (OtherActor :type "Actor Object Reference") (OtherComp :type "PrimitiveComponent Object Reference") (OtherBodyIndex :type Integer) (bFromSweep :type Boolean) (SweepResult :type "HitResult Structure (by ref)"))
  (`/Engine/EditorBlueprintResources/StandardMacros.IsValid` OtherActor
    (:`Is Valid`
      (if (`self.ActorHasTag` OtherActor "Enemy")
        (bind _asenemy_character_base (cast `EnemyCharacterBase` OtherActor))
        (bind _ascharacter_base (cast `CharacterBase` (`self.Causer`)))
        (bind ((`WeaponDamageRate` _weapondamagerate) (`MeleeWeaponStat` _meleeweaponstat)) (break `WeaponStatStruct` (`WeaponBase.GetWeaponStat` (`CharacterBase.GetCurrentWeaponRef` _ascharacter_base))))
        (`GameplayStatics.ApplyDamage` _asenemy_character_base (* (`.WeaponMeleeDamage` (break `MeleeWeaponStatStruct` _meleeweaponstat)) _weapondamagerate (`.CharacterAtkMultiplier` (break `CharacterStatStruct` (`CharacterBase.CharacterStat` _ascharacter_base)))) (`Pawn.GetController` _ascharacter_base) _ascharacter_base)))))

(fn `UserConstructionScript`)