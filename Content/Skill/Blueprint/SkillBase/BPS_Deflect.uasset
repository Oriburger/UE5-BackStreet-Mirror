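; Deflect skill actor that redirects incoming projectiles and hands their ownership to the skill's caster.
; On start it snaps to the caster's root socket, stays for the grade-defined "Deflect Duration", then detaches and hides.
; When its box overlaps a "Projectile"-tagged actor, it sets the caster as owner and relaunches the projectile at its own speed along the actor-to-SkillMesh direction, rather than mirroring its incoming path.
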(event `self.StartSkill`
  (bind _causer (`self.Causer`))
  (bind (_value _returnvalue) (`BlueprintMapLibrary.Map_Find` (`self.SkillGradeVariableMap`) "Deflect Duration"))
  (`/Engine/EditorBlueprintResources/StandardMacros.IsValid` _causer
    (:`Is Valid`
      (`self.K2_AttachToActor` _causer "root" "SnapToTarget" "KeepRelative" "KeepRelative")
      (if _returnvalue
        (`KismetSystemLibrary.Delay` _value)
        (`self.K2_DetachFromActor` "KeepRelative")
        (`self.HideSkill`)))))

(event `self.Box.OnComponentBeginOverlap`
  (params (OverlappedComponent :type "PrimitiveComponent Object Reference") (OtherActor :type "Actor Object Reference") (OtherComp :type "PrimitiveComponent Object Reference") (OtherBodyIndex :type Integer) (bFromSweep :type Boolean) (SweepResult :type "HitResult Structure (by ref)"))
  (bind _skillmesh (`self.SkillMesh`))
  (`/Engine/EditorBlueprintResources/StandardMacros.IsValid` OtherActor
    (:`Is Valid`
      (if (`self.ActorHasTag` OtherActor "Projectile")
        (`/Engine/EditorBlueprintResources/StandardMacros.IsValid` _skillmesh
          (:`Is Valid`
            (bind _asprojectile_base (cast `ProjectileBase` OtherActor))
            (bind _ascharacter_base (cast `CharacterBase` (`self.Causer`)))
            (`ProjectileBase.SetOwnerCharacter` _asprojectile_base _ascharacter_base)
            (set `MovementComponent.Velocity` (* (`KismetMathLibrary.Normal` (- (`SceneComponent.K2_GetComponentLocation` _skillmesh) (`self.K2_GetActorLocation`) (0.0 0.0 1.0)) 1.0) (`.ProjectileSpeed` (break `ProjectileStatStruct` (`ProjectileBase.ProjectileStat` _asprojectile_base)))) (`ProjectileBase.ProjectileMovement` _asprojectile_base))))))))

(fn `UserConstructionScript`)