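; Skill Blueprint that transforms the causer's current weapon into another one by swapping inventory entries.
; StartSkill casts Causer to CharacterBase and continues only if its current weapon is valid and matches one hardcoded WeaponID.
; It then removes that weapon, adds the replacement by a fixed ID and calls HideSkill.
; The swap is one-way, and HideSkill runs only when it happens.
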(event `self.StartSkill`
  (bind _ascharacter_base (cast `CharacterBase` (`self.Causer`)))
  (bind _returnvalue (`CharacterBase.GetCurrentWeaponRef` _ascharacter_base))
  (`/Engine/EditorBlueprintResources/StandardMacros.IsValid` _returnvalue
    (:`Is Valid`
      (bind _weaponid (`WeaponBase.WeaponID` _returnvalue))
      (if (== _weaponid 12130)
        (bind _returnvalue_2 (`CharacterBase.GetInventoryRef` _ascharacter_base))
        (`WeaponInventoryBase.RemoveWeapon` _returnvalue_2 _weaponid)
        (`WeaponInventoryBase.AddWeapon` _returnvalue_2 12131)
        (`self.HideSkill`)))))

(fn `UserConstructionScript`)