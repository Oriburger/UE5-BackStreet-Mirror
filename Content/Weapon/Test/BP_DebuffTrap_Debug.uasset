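; BP_DebuffTrap_Debug is a debug trap that heals or debuffs characters entering its box.
; On overlap by an actor tagged "Character", it casts to CharacterBase and, based on the Heal flag, applies a fixed heal or a debuff built from its variables, printing the debuff result.
; A DoOnce with a delayed reset gives the whole trap a five-second cooldown shared by all characters.
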(event `self.Box.OnComponentBeginOverlap`
  (params (OverlappedComponent :type "PrimitiveComponent Object Reference") (OtherActor :type "Actor Object Reference") (OtherComp :type "PrimitiveComponent Object Reference") (OtherBodyIndex :type Integer) (bFromSweep :type Boolean) (SweepResult :type "HitResult Structure (by ref)"))
  (`/Engine/EditorBlueprintResources/StandardMacros.IsValid` OtherActor
    (:`Is Valid`
      (if (`self.ActorHasTag` OtherActor "Character")
        (`/Engine/EditorBlueprintResources/StandardMacros.DoOnce` false :!label _label
          (:`Completed`
            (bind _ascharacter_base (cast `CharacterBase` OtherActor))
            (if (`self.bHeal`)
              (`CharacterBase.TakeHeal` _ascharacter_base 10.0 false 0)
              (else
                (bind _returnvalue (`CharacterBase.TryAddNewDebuff` _ascharacter_base (make `DebuffInfoStruct` (`self.Debuff Type`) (`self.Total Time`) (`self.Variable`) (`self.Is Percentage`)) self))
                (`KismetSystemLibrary.PrintString` (`KismetStringLibrary.Conv_BoolToString` _returnvalue) true true (struct :`R` 1.0 :`G` 0.303001 :`B` 0.193211 :`A` 1.0))))
            (`KismetSystemLibrary.Delay` 5.0)
            (goto _label :!via `Reset`)))))))

(fn `UserConstructionScript`)