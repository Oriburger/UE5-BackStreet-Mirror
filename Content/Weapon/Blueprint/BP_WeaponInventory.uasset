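; BP_WeaponInventory is a weapon inventory Blueprint whose graphs hold only debug scaffolding, with no active logic.
; Its events and construction script are empty, including PrintDebugMessage.
; A disconnected debug chain would print capacity, weapon count and current index, then loop over the inventory array.
; That chain shows each weapon's ID, name and type, plus ammo for throw weapons or durability for others, using frame-length print durations.
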(event `self.PrintDebugMessage`)

(fn `UserConstructionScript`)