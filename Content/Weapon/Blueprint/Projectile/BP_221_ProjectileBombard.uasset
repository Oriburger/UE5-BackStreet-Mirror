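; Bombard weapon projectile that explodes with area damage when it leaves play.
; The construction script copies speed and gravity scale from ProjectileStat into the ProjectileMovement component.
; EndPlay, rather than a hit event, applies radial damage at a multiple of the projectile's base damage, credited to the owning character and its controller.
; The explosion is skipped when the owner character is invalid.
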(event `self.ReceiveEndPlay`
  (params (EndPlayReason :type "EEndPlayReason Enum" :default "Destroyed"))
  (bind _returnvalue (`self.GetOwnerCharacterRef`))
  ;[1 1 1] 봄바드 폭발 이벤트
  (`/Engine/EditorBlueprintResources/StandardMacros.IsValid` _returnvalue
    (:`Is Valid`
      (`GameplayStatics.ApplyRadialDamage` :`BaseDamage` (* (`.ProjectileDamage` (break `ProjectileStatStruct` (`self.ProjectileStat`))) 2.5) :`Origin` (`self.K2_GetActorLocation`) :`DamageRadius` (`self.Damage Radius`) :`DamageCauser` _returnvalue :`InstigatedByController` (`Pawn.GetController` _returnvalue)))))

(fn `UserConstructionScript`
  (bind _projectilemovement (`self.ProjectileMovement`))
  (bind (_projectilename _description _bisexplosive _projectilespeed _projectiledamage _gravityscale) (break `ProjectileStatStruct` (`self.ProjectileStat`)))
  (set `ProjectileMovementComponent.InitialSpeed` _projectilespeed _projectilemovement)
  (set `ProjectileMovementComponent.MaxSpeed` _projectilespeed _projectilemovement)
  (set `ProjectileMovementComponent.ProjectileGravityScale` _gravityscale _projectilemovement))