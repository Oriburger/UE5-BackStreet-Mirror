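; BP_300_ProjectileSwordAura is a sword aura weapon projectile.
; Its construction script copies speed and gravity scale from ProjectileStat into ProjectileMovement, using the same speed as both initial and maximum.
; On BeginPlay, a timeline drives the mesh's world yaw from a float track, holding pitch and roll at zero regardless of the actor's orientation.
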(event `self.ReceiveBeginPlay`
  (bind (_direction `_새_트랙_0`) (`Timeline|타임라인_0`)
    (:`Update`
      (`SceneComponent.K2_SetWorldRotation` (`self.Mesh`) (`KismetMathLibrary.MakeRotator` 0.0 0.0 `_새_트랙_0`) false false))))

(fn `UserConstructionScript`
  (bind _projectilemovement (`self.ProjectileMovement`))
  (bind (_projectilename _description _bisexplosive _projectilespeed _projectiledamage _gravityscale) (break `ProjectileStatStruct` (`self.ProjectileStat`)))
  (set `ProjectileMovementComponent.InitialSpeed` _projectilespeed _projectilemovement)
  (set `ProjectileMovementComponent.MaxSpeed` _projectilespeed _projectilemovement)
  (set `ProjectileMovementComponent.ProjectileGravityScale` _gravityscale _projectilemovement))