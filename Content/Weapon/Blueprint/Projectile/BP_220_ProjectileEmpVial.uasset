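; EMP vial projectile that stuns nearby characters when it ends play.
; The construction script copies speed and gravity scale from ProjectileStat into the projectile movement component.
; On EndPlay, with a valid owner character, it sphere-overlaps pawns except the owner and gives CharacterBase hits a fixed-duration stun debuff credited to the owner.
; The stat-driven debuff type and damage nodes are left unconnected.
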(event `self.ReceiveEndPlay`
  (params (EndPlayReason :type "EEndPlayReason Enum" :default "Destroyed"))
  (bind _returnvalue (`self.GetOwnerCharacterRef`))
  ;[1 1 1] EMP 효과 반영 이벤트
  (`/Engine/EditorBlueprintResources/StandardMacros.IsValid` _returnvalue
    (:`Is Valid`
      (bind _outactors (`KismetSystemLibrary.SphereOverlapActors` (`self.K2_GetActorLocation`) (`self.Sphere Radius`) (`|MakeArray` "ObjectTypeQuery3" :!type "EObjectTypeQuery Enum") null (`|MakeArray` _returnvalue :!type "Actor Object Reference")))
      (for _array_element _outactors
        (`/Engine/EditorBlueprintResources/StandardMacros.IsValid` _array_element
          (:`Is Valid`
            (bind _ascharacter_base (cast `CharacterBase` _array_element))
            (`CharacterBase.TryAddNewDebuff` _ascharacter_base "E_Stun" _returnvalue 10.0 0.0)))))))

(fn `UserConstructionScript`
  (bind _projectilemovement (`self.ProjectileMovement`))
  (bind (_projectilename _description _bisexplosive _projectilespeed _projectiledamage _gravityscale) (break `ProjectileStatStruct` (`self.ProjectileStat`)))
  (set `ProjectileMovementComponent.InitialSpeed` _projectilespeed _projectilemovement)
  (set `ProjectileMovementComponent.MaxSpeed` _projectilespeed _projectilemovement)
  (set `ProjectileMovementComponent.ProjectileGravityScale` _gravityscale _projectilemovement))